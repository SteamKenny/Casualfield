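; Base actor for interactive devices that show a HUD widget and can be locked to one player at a time.
; Cosmetic clients register it with the UI manager, which now owns show/hide logic; ShowHide fills one widget slot per Z-order, behind the HUD.
; Update refreshes interactability and a pending token through overridable checks.
; Lock requests route through the player's UI manager message object to authority-only functions, which call empty lock/unlock action hooks.
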(event Custom|OnSelfDestroyed
  (params (DestroyedActor :type Actor%20Object%20Reference))
  (bind (_uimanager _isvalid) (CallFunction|GetUIManager))
  (if _isvalid
    (Default|UnregisterDevice _uimanager self))
  (Utilities|IsValid (Variables|Logic|GetUIWidget)
    (:Is%20Valid
      (Logic|ShowHide false))))

(event Custom|CancelInteract)

(event Custom|Update
  (params (DeltaSeconds :type Float%20%28single-precision%29))
  (Networking|CanExecuteCosmeticEvents
    (:True
      (Logic|UpdateCanInteract))))

(event Custom|OnUserWidgetDestroyed_Internal
  (Utilities|IsValid (Variables|Logic|GetUIWidget)
    (:Is%20Valid
      (Logic|ShowHide false))))

(event EventBeginPlay
  (Networking|CanExecuteCosmeticEvents
    (:True
      (Game|BindEventtoOnDestroyed self (delegate Custom|OnSelfDestroyed))
      (EventDispatchers|BindEventtoOnUserWidgetDestroyed (delegate Custom|OnUserWidgetDestroyed_Internal))
      (Utilities|WaitforPlayerController
        (:Out
          (Default|RegisterDevice (.UIManager (CallFunction|GetUIManager)) self))))))

(event Collision|EventActorBeginOverlap
  (params (OtherActor :type Actor%20Object%20Reference)))

(fn ConstructionScript)

(fn IsObservable
  (params (TargetActor :type Actor%20Object%20Reference) (RotationTollerance :type Float%20%28single-precision%29) (DistanceTollerance :type Float%20%28single-precision%29))
  (bind _returnvalue (Game|GetPlayerController 0))
  (bind _returnvalue_2 (Game|GetPlayerCameraManager 0))
  (bind _returnvalue_3 (Transformation|GetActorLocation TargetActor))
  (bind _returnvalue_4 (Pawn|GetControlRotation _returnvalue :!class /Script/Engine.Controller))
  (bind _transformcomponent (Variables|/Script/Engine.PlayerCameraManager|GetTransformComponent _returnvalue_2))
  (bind _returnvalue_5 (Transformation|GetWorldLocation _transformcomponent))
  (bind _returnvalue_6 (Math|Vector|GetForwardVector _returnvalue_4))
  (bind _returnvalue_7 (Math|Vector|Distance(Vector) _returnvalue_3 _returnvalue_5))
  (bind _returnvalue_8 (Math|Rotator|FindLookatRotation _returnvalue_3 _returnvalue_5))
  (bind _returnvalue_9 (Math|Vector|GetForwardVector _returnvalue_8))
  (bind _returnvalue_10 (Math|Vector|DotProduct _returnvalue_9 _returnvalue_6))
  (bind _returnvalue_11 (* _returnvalue_10 -1.0))
  (Utilities|IsValid (Game|Player|GetPlayerPawn 0)
    (:Is%20Valid
      (if (Rendering|IsVisible (Variables|/Script/Engine.Actor|GetRootComponent TargetActor))
        (if (and (<= _returnvalue_7 DistanceTollerance) (or (>= _returnvalue_11 RotationTollerance) (== RotationTollerance 0.0)))
          (bind _returnvalue_12 (Collision|LineTraceByChannel _returnvalue_5 _returnvalue_3 "TraceTypeQuery3" false 0 "None"))
          (return (not _returnvalue_12) _returnvalue_11 _returnvalue_7)
          (else
            (return false 0.0 0.0)))))))

(fn UserWidgetCreated
  (params (Widget :type Widget%20Object%20Reference))
  (bind _aswbp_interactive_device (Utilities|Casting|CastToWBP_Interactive_Device Widget))
  (Default|AssignOwner _aswbp_interactive_device self)
  (Development|PrintString "UI Created")
  (Default|CallOnUserWidgetCreated))

(fn UserWidgetDestroyed
  (Logic-Locking|ServerUnlockforPlayer)
  (Development|PrintString "UI Destroyed")
  (Default|CallOnUserWidgetDestroyed))

(fn LockforPlayer
  (params (PlayerId :type Integer) (Action :type String) (Controller :type Controller%20Object%20Reference) (Token :type Actor%20Object%20Reference) (PlayerState :type Player%20State%20Object%20Reference))
  (Networking|SwitchHasAuthority
    (:Authority
      (if (== (Variables|Logic-Locking|GetLockedPlayer) 0)
        (bind _output_get (Variables|Logic-Locking|SetLockedPlayer PlayerId))
        (bind _output_get_2 (Variables|Logic-Locking|SetLockedController Controller))
        (bind _output_get_3 (Variables|Logic-Locking|SetLockedToken Token))
        (Variables|Logic-Locking|SetLockedPlayerState PlayerState)
        (Logic-Locking|ExecuteLockAction Action _output_get_2 _output_get_3)
        (CallFunction|PrintInt "Locked" _output_get "(R=0.000000,G=0.658824,B=1.000000,A=1.000000)")))))

(fn UnlockforPlayer
  (params (PlayerId :type Integer))
  (Networking|SwitchHasAuthority
    (:Authority
      (if (== (Variables|Logic-Locking|GetLockedPlayer) PlayerId)
        (CallFunction|PrintInt "Unlocked" (Variables|Logic-Locking|GetLockedPlayer) "(R=0.000000,G=0.658824,B=1.000000,A=1.000000)")
        (Variables|Logic-Locking|SetLockedPlayer 0)
        (Variables|Logic-Locking|SetLockedController 0)
        (Variables|Logic-Locking|SetLockedToken 0)
        (Variables|Logic-Locking|SetLockedAction "")
        (Variables|Logic-Locking|SetLockedPlayerState 0)
        (Logic-Locking|ExecuteUnlockAction)))))

(fn ServerLockforPlayer
  (params (Action :type String))
  (bind _playercontroller (CallFunction|GetClientPlayerController))
  (bind _playerstate (Variables|/Script/Engine.Controller|GetPlayerState _playercontroller))
  (bind _uimanager (Class|IFControllerCQB|GetUIManager(Message) _playercontroller))
  (Utilities|IsValid _uimanager
    (:Is%20Valid
      (Default|ServerLockforPlayer _uimanager self (Variables|/Script/Engine.PlayerState|GetPlayerId _playerstate) Action (Variables|Logic|GetPendingToken) _playerstate))))

(fn ServerUnlockforPlayer
  (bind _playercontroller (CallFunction|GetClientPlayerController))
  (bind _uimanager (Class|IFControllerCQB|GetUIManager(Message) _playercontroller))
  (Utilities|IsValid _uimanager
    (:Is%20Valid
      (Default|ServerUnlockforPlayer _uimanager self (Variables|/Script/Engine.PlayerState|GetPlayerId (Variables|/Script/Engine.Controller|GetPlayerState _playercontroller))))))

(fn IsShowingUI
  (return (Utilities|IsValid (Variables|Logic|GetUIWidget))))

(fn ExecuteLockAction
  (params (Action :type String) (Controller :type Controller%20Object%20Reference) (Token :type Actor%20Object%20Reference)))

(fn ExecuteUnlockAction)

(fn AddWidgetto
  (params (Widget :type Widget%20Object%20Reference))
  (bind _returnvalue (Widget|Panel|AddChild (Widget|GetParent (Variables|/HDCore/UI/HUD/WBP_HUD.WBP_HUD_C|GetCaptureStatus (Variables|/HDCore/Core/BP_HDHUDBase.BP_HDHUDBase_C|GetHUDContainerUW (CallFunction|GetHDHUDBP)))) Widget))
  (bind _ascanvas_panel_slot (Utilities|Casting|CastToCanvasPanelSlot _returnvalue))
  ;[1 1 1] Set our child widget to full screen within the HUD, but behind the rest of the HUD
  (Class|CanvasPanelSlot|SetAnchors _ascanvas_panel_slot (Utilities|Struct|MakeAnchors "(X=0.000000,Y=0.000000)" "(X=1.000000,Y=1.000000)"))
  (Class|CanvasPanelSlot|SetAlignment _ascanvas_panel_slot)
  (Class|CanvasPanelSlot|SetZOrder _ascanvas_panel_slot -1)
  (Class|CanvasPanelSlot|SetOffsets _ascanvas_panel_slot (Utilities|Struct|MakeMargin 0.0 0.0 0.0 0.0)))

(fn ShowHide
  (params (State :type Boolean))
  (bind _uimanager (CallFunction|GetUIManager))
  (bind (_uimanager_2 _isvalid) (CallFunction|GetUIManager))
  (bind _zorder (Variables|Logic|GetZorder))
  (bind _widget (Default|GetWidget _uimanager_2 _zorder))
  (if _isvalid
    (if State
      (Utilities|IsValid _widget
        (:Is%20Not%20Valid
          (bind _widgetclass (Logic|GetUIWidgetClass))
          (bind _returnvalue (UserInterface|CreateWidget _widgetclass (Game|GetPlayerController 0)))
          (Default|SetWidget _uimanager (Variables|Logic|GetZorder) _returnvalue)
          (bind _output_get (Variables|Logic|SetUIWidget _returnvalue))
          (Logic|UserWidgetCreated _output_get)
          (Logic|AddWidgetto _output_get)))
      (elif (Math|Boolean|ANDBoolean (Utilities|IsValid _widget) (== _widget (Variables|Logic|GetUIWidget)) (Utilities|IsValid (Variables|Logic|GetUIWidget)))
        (Widget|RemovefromParent _widget)
        (Default|SetWidget _uimanager (Variables|Logic|GetZorder))
        (Variables|Logic|SetUIWidget 0)
        (Variables|Logic|SetInteracted false)))))

(fn GetUIWidgetClass
  (return (Variables|Logic|GetUIWidgetClass)))

(fn ShowHideLogic
  (bind _hdplayerchar (CallFunction|GetHDPlayerCharacterBP))
  (if (Utilities|IsValid _hdplayerchar)
    (if (Class|DFBaseCharacter|IsAlive _hdplayerchar)
      (if (Logic|GetIsRelevantto (Game|GetPlayerController 0))
        (if (!= (Variables|Logic|GetZorder) -1)
          (bind _result (Logic|IsObservable self (Variables|Logic|GetRotationTollerance) (Variables|Logic|GetDistanceTollerance)))
          (Logic|ShowHide _result))
        (else
          (Logic|ShowHide false :!label _label)))
      (else
        (goto _label)))
    (else
      (goto _label))))

(fn UpdateCanInteract
  (bind (_caninteract _token) (Logic|GetCanInteract))
  (Networking|CanExecuteCosmeticEvents
    (:True
      (bind _output_get (LocalVariables|SetCanInteractInitial (Variables|Logic|GetCanInteract)))
      (bind _output_get_2 (Variables|Logic|SetCanInteract (and (Logic|GetIsRelevantto (Game|GetPlayerController 0)) _caninteract)))
      (if _output_get_2
        (Variables|Logic|SetPendingToken _token)
        (else
          (Variables|Logic|SetPendingToken 0)
          (if (Math|Boolean|NotEqual(Boolean) _output_get_2 _output_get)
            (CallFunction|CancelInteract)))))))

(fn GetCanInteract
  (return true 0))

(fn GetIsRelevantto
  (params (Controller :type Controller%20Object%20Reference))
  (return true))