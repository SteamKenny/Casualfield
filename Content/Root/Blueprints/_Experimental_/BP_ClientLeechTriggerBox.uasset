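; An experimental trigger box that resizes and moves itself at BeginPlay to cover the level's playable area.
; It reads the minimap boundary length and midpoint from TBWorldSettings, setting its horizontal box extent to half that length and centering itself there at Z zero.
; The vertical half-extent is the absolute world KillZ, so the box reaches down to the kill height and equally far above.
; The Blueprint contains no overlap handling of its own.
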(event EventBeginPlay
  (bind _returnvalue (Class|DFBlueprintFunctions|GetWorldSettings))
  (|CallParentFunction)
  (bind _astbworld_settings (Utilities|Casting|CastToTBWorldSettings _returnvalue))
  (bind _asbox_collision (Utilities|Casting|CastToBoxComponent (Variables|Default|GetCollisionComponent)))
  (Components|Box|SetBoxExtent _asbox_collision (Math|Vector|MakeVector (* (.PlayableBoundaryLength (Utilities|Struct|BreakMinimapGenerationSettings (Variables|/Script/Tinkerbox.TBWorldSettings|GetMinimapSettings _astbworld_settings))) 0.5) (* (.PlayableBoundaryLength (Utilities|Struct|BreakMinimapGenerationSettings (Variables|/Script/Tinkerbox.TBWorldSettings|GetMinimapSettings _astbworld_settings))) 0.5) (Math|Float|Absolute(Float) (Variables|/Script/Engine.WorldSettings|GetKillZ _returnvalue))) true)
  (Transformation|SetActorLocation (Math|Vector|MakeVector (.X (Math|Vector|BreakVector (.BoundaryMidPointLoc (Utilities|Struct|BreakMinimapGenerationSettings (Variables|/Script/Tinkerbox.TBWorldSettings|GetMinimapSettings _astbworld_settings))))) (.Y (Math|Vector|BreakVector (.BoundaryMidPointLoc (Utilities|Struct|BreakMinimapGenerationSettings (Variables|/Script/Tinkerbox.TBWorldSettings|GetMinimapSettings _astbworld_settings))))) 0.0) false false))

(event EventTick
  (params (DeltaSeconds :type Float%20%28single-precision%29)))

(fn ConstructionScript)