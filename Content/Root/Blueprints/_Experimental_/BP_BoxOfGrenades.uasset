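; Experimental grenade box actor that, when used, releases a burst of M67 grenade projectiles.
; The Used event plays a beep, waits a short delay, then loops to spawn grenades above the static mesh with the invoking pawn as instigator.
; Each grenade gets a random yaw and steep upward pitch, and its projectile movement initial speed is set to a low value after spawning.
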(event EventBeginPlay)

(event Collision|EventActorBeginOverlap
  (params (OtherActor :type Actor%20Object%20Reference)))

(event EventTick
  (params (DeltaSeconds :type Float%20%28single-precision%29)))

(event EventUsed
  (params (Invoker :type Actor%20Object%20Reference))
  (bind _staticmesh (Variables|Default|GetStaticMesh))
  (bind _returnvalue (Transformation|GetWorldTransform _staticmesh))
  (bind (_location _rotation _scale) (Math|Transform|BreakTransform _returnvalue))
  (Audio|PlaySound2D "/Detonation/Root/Audio/beep-23.beep-23" 1.0 1.0 0.0 0 0)
  (Utilities|FlowControl|Delay 3.0)
  (bind _aspawn (Utilities|Casting|CastToPawn Invoker))
  (for _index (range 0 5)
    (bind _returnvalue_2 (Game|SpawnActorfromClass "/HDAssets/Items/Weapons/Grenades/M67_P/BP_HDProj_M67_P_Grenade.BP_HDProj_M67_P_Grenade_C" (Math|Transform|MakeTransform (+ _location "0, 0,150.000000") (Math|Rotator|MakeRotator 0.0 (Math|Random|RandomFloatinRange 6e+01 9e+01) (Math|Random|RandomFloatinRange 0.0 3.6e+02)) _scale) "AlwaysSpawn" 0 _aspawn))
    (Variables|/Script/Engine.ProjectileMovementComponent|SetInitialSpeed (Variables|/Script/DonkehFramework.DFBaseProjectile|GetProjectileMovement _returnvalue_2) 5.0)))

(fn ConstructionScript)