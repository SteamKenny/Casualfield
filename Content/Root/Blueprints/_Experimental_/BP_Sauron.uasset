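; BP_Sauron is an experimental free-moving observer pawn that hides the HUD, shows WBP_Sauron and switches player tags to Sauron mode.
; Mouse wheel sets fly speed, PageUp/PageDown step scale, and right click toggles camera-trace selection that outline-highlights a player.
; OnPawnSpawn reselects that player by PlayerId.
; A looping timer saves server name, player roster and selection to the SauronOut slot when STEAMSERVERNAME is set.
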(event Custom|CreateSauronOut
  (Logic|WriteSauronOut))

(event Custom|OnPawnSpawn
  (params (Pawn :type Pawn%20Object%20Reference))
  (bind _playerstate (Variables|/Script/Engine.Pawn|GetPlayerState Pawn))
  (bind _playerid (Variables|/Script/Engine.PlayerState|GetPlayerId _playerstate))
  (Utilities|IsValid _playerstate
    (:Is%20Valid
      (if (== _playerid (Variables|Logic|GetSelectedPlayerId))
        (Logic|SetTargetActor Pawn _playerid (PlayerState|GetPlayerName _playerstate))))))

(event EventDestroyed
  (|CallParentFunction)
  (Networking|CanExecuteCosmeticEvents
    (:True
      (Widget|SetRenderOpacity (Variables|/HDCore/Core/BP_HDHUDBase.BP_HDHUDBase_C|GetHUDContainerUW (CallFunction|GetHDHUDBP)) 1.0)
      (bind _outactors (Actor|GetAllActorsOfClass "/CasualCQB/Root/Core/BP_HDPlayerCharacter_CQB.BP_HDPlayerCharacter_CQB_C"))
      (for _array_element _outactors
        (Default|SauronOff (Variables|/CasualCQB/Root/Core/BP_HDPlayerCharacter_CQB.BP_HDPlayerCharacter_CQB_C|GetCP_Character_WC_PlayerTag _array_element)))
      (Widget|RemovefromParent (Variables|Logic|GetSauronUI))
      (Variables|Logic|SetSauronUI 0))))

(event Collision|EventActorBeginOverlap
  (params (OtherActor :type Actor%20Object%20Reference)))

(event EventTick
  (params (DeltaSeconds :type Float%20%28single-precision%29))
  (|CallParentFunction DeltaSeconds)
  (if (Variables|Logic|GetSelectModeActive)
    (bind _asplayer_controller (Utilities|Casting|CastToPlayerController (Pawn|GetController)))
    (bind _outhit (Collision|LineTraceByChannel (Transformation|GetWorldLocation (Variables|/Script/Engine.PlayerCameraManager|GetTransformComponent (Variables|/Script/Engine.PlayerController|GetPlayerCameraManager _asplayer_controller))) (+ (* (Math|Vector|GetForwardVector (Transformation|GetWorldRotation (Variables|/Script/Engine.PlayerCameraManager|GetTransformComponent (Variables|/Script/Engine.PlayerController|GetPlayerCameraManager _asplayer_controller)))) (Variables|Logic-Config|GetRayCastLength)) (Transformation|GetWorldLocation (Variables|/Script/Engine.PlayerCameraManager|GetTransformComponent (Variables|/Script/Engine.PlayerController|GetPlayerCameraManager _asplayer_controller)))) "TraceTypeQuery2" false 0 "None"))
    (bind _ascharacter (Utilities|Casting|CastToCharacter (.HitActor (Collision|BreakHitResult _outhit))))
    (Utilities|IsValid (Variables|/Script/Engine.Pawn|GetPlayerState _ascharacter)
      (:Is%20Valid
        (Logic|SetTargetActor _ascharacter (Variables|/Script/Engine.PlayerState|GetPlayerId (Variables|/Script/Engine.Pawn|GetPlayerState _ascharacter)) (PlayerState|GetPlayerName (Variables|/Script/Engine.Pawn|GetPlayerState _ascharacter)))))))

(event EventPossessed
  (params (NewController :type Controller%20Object%20Reference))
  (|CallParentFunction NewController))

(event EventBeginPlay
  (|CallParentFunction)
  (Networking|CanExecuteCosmeticEvents
    (:True
      (Widget|SetRenderOpacity (Variables|/HDCore/Core/BP_HDHUDBase.BP_HDHUDBase_C|GetHUDContainerUW (CallFunction|GetHDHUDBP)) 0.0)
      (bind _outactors (Actor|GetAllActorsOfClass "/CasualCQB/Root/Core/BP_HDPlayerCharacter_CQB.BP_HDPlayerCharacter_CQB_C"))
      (for _array_element _outactors
        (Default|Sauronon (Variables|/CasualCQB/Root/Core/BP_HDPlayerCharacter_CQB.BP_HDPlayerCharacter_CQB_C|GetCP_Character_WC_PlayerTag _array_element))
        (Utilities|IsValid (Actor|GetComponentbyClass _array_element "/CasualCQB/Root/Blueprints/Components/CP_Actor_Basic_Cosmetics.CP_Actor_Basic_Cosmetics_C")
          (:Is%20Valid
            (Default|SetHighlightState (Actor|GetComponentbyClass _array_element "/CasualCQB/Root/Blueprints/Components/CP_Actor_Basic_Cosmetics.CP_Actor_Basic_Cosmetics_C") false))))
      (bind _asplayer_controller (Utilities|Casting|CastToPlayerController (Components|GetOwner)))
      (bind _returnvalue (UserInterface|CreateWidget "/CasualCQB/Root/UI/HUD/WBP_Sauron.WBP_Sauron_C" _asplayer_controller))
      (Default|Initialise _returnvalue self)
      (UserInterface|Viewport|AddtoViewport _returnvalue 1)
      (Variables|Logic|SetSauronUI _returnvalue)
      (Utilities|Time|SetTimerbyEvent (delegate Custom|CreateSauronOut) (Variables|Logic-Config|GetDataOutputFreq) true)
      (Default|Initialise (Variables|Default|GetCP_Actor_Basic_Cosmetics) (Variables|Default|GetCamera) "/CasualCQB/Root/Materials/M_Outline_Only_Inst_Sauron.M_Outline_Only_Inst_Sauron")
      (bind _asplayer_controller_2 (Utilities|Casting|CastToPlayerController (Pawn|GetController)))
      (Input|EnableInput _asplayer_controller_2))))

(event Input|MouseEvents|MouseWheelAxis
  (params (AxisValue :type Float%20%28single-precision%29))
  (bind _movementcomponent (Variables|Default|GetMovementComponent))
  (bind _asfloating_pawn_movement (Utilities|Casting|CastToFloatingPawnMovement _movementcomponent))
  (Variables|/Script/Engine.FloatingPawnMovement|SetMaxSpeed _asfloating_pawn_movement (Math|Float|Clamp(Float) (+ (Class|MovementComponent|GetMaxSpeed _movementcomponent) (* AxisValue (Variables|Logic-Config|GetSpeedAxisDelta))) (Variables|Logic-Config|GetMinSpeed) (Variables|Logic-Config|GetMaxSpeed))))

(event Input|KeyboardEvents|PageUp
  (params (Key :type Key%20Structure :default "None"))
  (:Pressed
    (Logic|AlterScale 1)))

(event Input|KeyboardEvents|PageDown
  (params (Key :type Key%20Structure :default "None"))
  (:Pressed
    (Logic|AlterScale -1)))

(event Input|MouseEvents|RightMouseButton
  (params (Key :type Key%20Structure :default "None"))
  (:Pressed
    (bind _output_get (Variables|Logic|SetSelectModeActive (not (Variables|Logic|GetSelectModeActive))))
    (Default|CallOnSelectModeChange _output_get)))

(event Input|MouseEvents|MiddleMouseButton
  (params (Key :type Key%20Structure :default "None"))
  (:Pressed
    (Default|CallOnToggleHUD)))

(fn ConstructionScript)

(fn AlterScale
  (params (Delta :type Integer))
  (bind _scaleset (Variables|Logic-Config|GetScaleSet))
  (LocalVariables|SetOldScaleIndex (Variables|Logic|GetScaleIndex))
  (bind _output_get (Variables|Logic|SetScaleIndex (Math|Integer|Clamp(Integer) (+ (Variables|Logic|GetScaleIndex) Delta) 0 (- (Utilities|Array|Length _scaleset) 1))))
  (Variables|Logic|SetScale (Utilities|Array|Get(acopy) _scaleset _output_get))
  (if (!= (LocalVariables|GetOldScaleIndex) (Variables|Logic|GetScaleIndex))
    (Default|CallOnScaleChange)))

(fn WriteSauronOut
  (bind _value (Default|GetServerCommandLineOption (CallFunction|GetGameStateCQB) "STEAMSERVERNAME"))
  (if (not (Class|DFBlueprintFunctions|IsEmptyorWhitespace _value))
    (LocalVariables|SetServerName _value)
    (bind _returnvalue (SaveGame|CreateSaveGameObject "/CasualCQB/Root/Core/SauronOut.SauronOut_C"))
    (Utilities|FlowControl|Sequence
      (:then_0
        (for _array_element (Variables|/Script/Engine.GameStateBase|GetPlayerArray (CallFunction|GetGameStateCQB))
          (Utilities|IsValid _array_element
            (:Is%20Valid
              (Utilities|Map|Add (LocalVariables|GetPlayerMapping) (Variables|/Script/Engine.PlayerState|GetPlayerId _array_element) (PlayerState|GetPlayerName _array_element)))))
        (Variables|/CasualCQB/Root/Core/SauronOut.SauronOut_C|SetPlayerMapping _returnvalue (LocalVariables|GetPlayerMapping)))
      (:then_1
        (Variables|/CasualCQB/Root/Core/SauronOut.SauronOut_C|SetTimeStamp _returnvalue (Math|DateTime|UTCNow))
        (Variables|/CasualCQB/Root/Core/SauronOut.SauronOut_C|SetServerName _returnvalue (LocalVariables|GetServerName))
        (Variables|/CasualCQB/Root/Core/SauronOut.SauronOut_C|SetSelectedPlayerId _returnvalue (Variables|Logic|GetSelectedPlayerId))
        (Variables|/CasualCQB/Root/Core/SauronOut.SauronOut_C|SetSelectedPlayerAt _returnvalue (Variables|Logic|GetSelectedPlayerAt))
        (SaveGame|SaveGametoSlot _returnvalue "SauronOut")))))

(fn SetTargetActor
  (params (Actor :type Actor%20Object%20Reference) (PlayerId :type Integer) (PlayerName :type String))
  (bind _returnvalue (Actor|GetComponentbyClass Actor "/CasualCQB/Root/Blueprints/Components/CP_Actor_Basic_Cosmetics.CP_Actor_Basic_Cosmetics_C"))
  (Utilities|FlowControl|Sequence
    (:then_0
      (LocalVariables|SetPreviousSelectedPlayerId (Variables|Logic|GetSelectedPlayerId))
      (Utilities|IsValid (Variables|Logic|GetBasicCosmeticsTarget)
        (:Is%20Valid
          (Default|SetHighlightState (Variables|Logic|GetBasicCosmeticsTarget) false)
          (Variables|Logic|SetBasicCosmeticsTarget 0)
          (Variables|Logic|SetSelectedPlayerId 0)
          (Variables|Logic|SetSelectedPlayerAt ""))))
    (:then_1
      (Utilities|IsValid Actor
        (:Is%20Valid
          (Utilities|IsValid _returnvalue
            (:Is%20Valid
              (bind _output_get (Variables|Logic|SetBasicCosmeticsTarget _returnvalue))
              (Default|SetHighlightState _output_get true)
              (bind _output_get_2 (Variables|Logic|SetSelectedPlayerId PlayerId))
              (if (!= _output_get_2 (LocalVariables|GetPreviousSelectedPlayerId))
                (Default|CallOnSelectedPlayerChange _output_get_2 PlayerName)
                (Variables|Logic|SetSelectedPlayerAt (Math|DateTime|UTCNow))))))))))