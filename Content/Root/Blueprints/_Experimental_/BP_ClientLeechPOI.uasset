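; BP_ClientLeechPOI is an experimental point-of-interest actor, by its name for a leech, that follows an owning actor.
; On BeginPlay, if the owning actor is valid, it derives its team from that actor's instigator and snap-attaches itself to the actor.
; It binds to the owner's destroyed event and destroys itself when the owner is destroyed.
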(event Custom|OnOwningActorDestroyed
  (params (DestroyedActor :type Actor%20Object%20Reference))
  (Actor|DestroyActor))

(event EventBeginPlay
  (bind _owningactor (Variables|Logic|GetOwningActor))
  (|CallParentFunction)
  (Utilities|IsValid _owningactor
    (:Is%20Valid
      (Variables|Logic|SetOwningTeam (Utilities|Enum|ByteToEnumEHDTeam (Class|DFBlueprintFunctions|GetTeamNum (Game|GetInstigator _owningactor))))
      (Game|BindEventtoOnDestroyed _owningactor (delegate Custom|OnOwningActorDestroyed))
      (Transformation|AttachActorToActor _owningactor "None" "SnapToTarget" "SnapToTarget" "SnapToTarget" true))))

(event Collision|EventActorBeginOverlap
  (params (OtherActor :type Actor%20Object%20Reference)))

(fn ConstructionScript)