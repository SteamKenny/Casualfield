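; Experimental controller utility that detects mapped actors on the client and spawns BP_ClientLeechPOI markers for them.
; On BeginPlay, where cosmetic events can execute, it spawns a BP_ClientLeechTriggerBox and binds to its overlap event.
; Overlapping actors' class paths key into the Clientleech_mapping data table; matches spawn a typed POI owning that actor and log its class.
; An earlier hard-coded name-substring lookup remains as unreachable code.
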(event Custom|OnActorBeginOverlap
  (params (OverlappedActor :type Actor%20Object%20Reference) (OtherActor :type Actor%20Object%20Reference))
  (bind (_success _type) (Logic|GetTypefromActor OtherActor))
  (if _success
    (Game|SpawnActorfromClass "/CasualCQB/Root/Blueprints/_Experimental_/BP_ClientLeechPOI.BP_ClientLeechPOI_C" (Math|Transform|MakeTransform "0, 0, 0") "Undefined" 0 OtherActor _type 0)
    (CallFunction|AddLogTextRaw (Utilities|ToString(SoftClassReference) (Utilities|ResolveSoftReference (Utilities|GetClass OtherActor))) true)))

(event EventBeginPlay
  (|CallParentFunction)
  (Networking|CanExecuteCosmeticEvents
    (:True
      (bind _returnvalue (Game|SpawnActorfromClass "/CasualCQB/Root/Blueprints/_Experimental_/BP_ClientLeechTriggerBox.BP_ClientLeechTriggerBox_C" (Math|Transform|MakeTransform "0, 0, 0") "Undefined" 0 0))
      (Collision|BindEventtoOnActorBeginOverlap _returnvalue (delegate Custom|OnActorBeginOverlap)))))

(event EventTick
  (params (DeltaSeconds :type Float%20%28single-precision%29)))

(fn GetTypefromActor
  (params (Actor :type Actor%20Object%20Reference))
  (bind _returnvalue (Utilities|GetDataTableRow "/CasualCQB/Root/Data/clientleech_mapping.clientleech_mapping" (Utilities|String|StringToName (CallFunction|GetActorClassPath Actor)))
    (:then
      (return true (Utilities|Struct|BreakSTR_Client_Leech_Mapping _returnvalue)))
    (:RowNotFound
      (return false "NewEnumerator0"))))