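; Actor component that registers its owning actor as a point of interest (POI) on the player's minimap.
; On BeginPlay, where cosmetic events can execute, it gets the minimap widget from player controller 0 and adds a POI unless one already exists.
; If the controller or widget is invalid, it logs the failure and retries every 0.2 seconds, with no attempt limit.
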(event Custom|Retry
  ;[1 1 1] Will retry AddPOI until successful
  (Variables|Logic|SetPlayerController (CallFunction|GetHDPlayerControllerBP))
  (bind _playercontroller (Variables|Logic|GetPlayerController)
    (:then
      (Variables|Logic|SetMinimap (Default|GetMinimapWidget _playercontroller))
      (bind _minimap (Variables|Logic|GetMinimap)
        (:then
          (bind _returnvalue (Class|DFMinimap|FindPOIbyActor _minimap (Components|GetOwner)))
          (if _returnvalue
            (Class|DFBlueprintFunctions|PrintStringtoLog "POI already exist" "Warning")
            (else
              (Class|DFMinimap|AddNewPOI _minimap (Components|GetOwner)))))
        (:else
          (Class|DFBlueprintFunctions|PrintStringtoLog "Failed to add POI for CP, Minimap reference is not valid!" "Warning")
          (Utilities|FlowControl|Delay 0.2 :!label _label)
          (CallFunction|Retry))))
    (:else
      (Class|DFBlueprintFunctions|PrintStringtoLog "Failed to add POI for CP, Player Controller is not valid!" "Warning")
      (goto _label))))

(event EventBeginPlay
  ;[1 1 1] Will retry AddPOI until successful
  (|CallParentFunction)
  (Networking|CanExecuteCosmeticEvents
    (:True
      (Variables|Logic|SetPlayerController (CallFunction|GetHDPlayerControllerBP))
      (bind _playercontroller (Variables|Logic|GetPlayerController)
        (:then
          (Variables|Logic|SetMinimap (Default|GetMinimapWidget _playercontroller))
          (bind _minimap (Variables|Logic|GetMinimap)
            (:then
              (bind _returnvalue (Class|DFMinimap|FindPOIbyActor _minimap (Components|GetOwner)))
              (if _returnvalue
                (Class|DFBlueprintFunctions|PrintStringtoLog "POI already exist" "Warning")
                (else
                  (Class|DFMinimap|AddNewPOI _minimap (Components|GetOwner)))))
            (:else
              (Class|DFBlueprintFunctions|PrintStringtoLog "Failed to add POI for CP, Minimap reference is not valid!" "Warning")
              (Utilities|FlowControl|Delay 0.2 :!label _label)
              (CallFunction|Retry))))
        (:else
          (Class|DFBlueprintFunctions|PrintStringtoLog "Failed to add POI for CP, Player Controller is not valid!" "Warning")
          (goto _label))))))

(event EventTick
  (params (DeltaSeconds :type Float%20%28single-precision%29)))