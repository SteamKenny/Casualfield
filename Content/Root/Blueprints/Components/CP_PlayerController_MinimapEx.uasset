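; Player controller component that creates the deploy menu with a custom spawn minimap widget in place of the stock one.
; InitialiseExVersionOfMinimap repeats the parent LoadDeployMenu logic, creating WBP_DeployMenu if none is valid, then removing its minimap and adding a DeployMenuSpawnMinimapClass instance to the same parent.
; It auto-sizes the new canvas slot and rebinds preload and spawn point selection dispatchers before preloading menu content.
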(event Custom|InitialiseExVersionOfMinimap
  (bind _playercontroller (Logic|GetOwningPlayerController))
  ;[1 1 1] Copied code from the parent LoadDeployMenu Function
  (Utilities|IsValid (Variables|Logic|GetDeployMenu)
    (:Is%20Not%20Valid
      (bind _returnvalue (UserInterface|CreateWidget "/HDCore/UI/DeployMenu/WBP_DeployMenu.WBP_DeployMenu_C" _playercontroller 0 0))
      (bind _output_get (Variables|Logic|SetDeployMenu _returnvalue)) ; Store widget reference
      (EventDispatchers|BindEventtoOnPreloadFinished _output_get (EventDispatchers|CreateEvent _playercontroller :!event OnDeployMenuPreloadFinished))
      ;[1 1 1] Swap out SpawnMinimap Widget
      (bind _output_get_2 (Variables|Logic|SetMinimapParent (Widget|GetParent (Variables|/HDCore/UI/DeployMenu/SpawnMap/WBP_DeployMenu_SpawnMapView.WBP_DeployMenu_SpawnMapView_C|GetMinimap (Variables|/HDCore/UI/DeployMenu/WBP_DeployMenu.WBP_DeployMenu_C|GetSpawnMapView (Variables|Logic|GetDeployMenu)))))) ; Save the ref to the Minimap parent for later
      (Development|PrintString (Utilities|String|Append "MinimapParent : " (Utilities|GetDisplayName _output_get_2)))
      (Widget|RemovefromParent (Variables|/HDCore/UI/DeployMenu/SpawnMap/WBP_DeployMenu_SpawnMapView.WBP_DeployMenu_SpawnMapView_C|GetMinimap (Variables|/HDCore/UI/DeployMenu/WBP_DeployMenu.WBP_DeployMenu_C|GetSpawnMapView (Variables|Logic|GetDeployMenu)))) ; Removing the Current minimap
      (bind _returnvalue_2 (UserInterface|CreateWidget (Variables|Logic|GetDeployMenuSpawnMinimapClass) _playercontroller))
      (bind _output_get_3 (Variables|/HDCore/UI/DeployMenu/SpawnMap/WBP_DeployMenu_SpawnMapView.WBP_DeployMenu_SpawnMapView_C|SetMinimap (Variables|/HDCore/UI/DeployMenu/WBP_DeployMenu.WBP_DeployMenu_C|GetSpawnMapView (Variables|Logic|GetDeployMenu)) (.AsWBP%20Deploy%20Menu%20Spawn%20Minimap (Utilities|Casting|CastToWBP_DeployMenu_SpawnMinimap _returnvalue_2)))) ; Replace the minimap with our custom one
      (bind _returnvalue_3 (Widget|Panel|AddChild _output_get_2 _output_get_3))
      ;;[1 1 1] fix layout bug
      (bind _ascanvas_panel_slot (Utilities|Casting|CastToCanvasPanelSlot _returnvalue_3))
      (Class|CanvasPanelSlot|SetAutoSize _ascanvas_panel_slot true)
      ;[1 1 1] Fix Event dispatcher on SpawnMapView
      (EventDispatchers|BindEventtoOnPreloadFinished _output_get_3 (EventDispatchers|CreateEvent (Variables|/HDCore/UI/DeployMenu/WBP_DeployMenu.WBP_DeployMenu_C|GetSpawnMapView (Variables|Logic|GetDeployMenu)) :!event BndEvtMinimapK2NodeComponentBoundEvent1onPreloadFinishedDelegateSignature))
      (EventDispatchers|BindEventtoOnSpawnPointSelected _output_get_3 (EventDispatchers|CreateEvent (Variables|/HDCore/UI/DeployMenu/WBP_DeployMenu.WBP_DeployMenu_C|GetSpawnMapView (Variables|Logic|GetDeployMenu)) :!event BndEvtMinimapK2NodeComponentBoundEvent0onSpawnPointSelectedDelegateSignature))
      (EventDispatchers|BindEventtoOnSpawnPointDeselected _output_get_3 (EventDispatchers|CreateEvent (Variables|/HDCore/UI/DeployMenu/WBP_DeployMenu.WBP_DeployMenu_C|GetSpawnMapView (Variables|Logic|GetDeployMenu)) :!event BndEvtMinimapK2NodeComponentBoundEvent2onSpawnPointDeselectedDelegateSignature))
      ;[1 1 1] Copied code from the parent LoadDeployMenu Function
      (Default|PreloadContent (Variables|Logic|GetDeployMenu)))))

(event EventBeginPlay)

(event EventTick
  (params (DeltaSeconds :type Float%20%28single-precision%29)))

(fn GetOwningPlayerController
  (return (.AsBP%20HDPlayer%20Controller (Utilities|Casting|CastToBP_HDPlayerController (Components|GetOwner)))))