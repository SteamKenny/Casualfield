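; Character component that takes over damage and health for player and bot characters, keeping an authoritative RealHealth.
; Server-bound point, radial and environmental/generic damage events feed ApplyDamage, which applies multipliers, protection checks and downed-for-revive or headshot rules.
; InterceptHealthChanged allows healing but reverts unmanaged health drops.
; Recent projectile hits are recorded to flag radial damage reduction, though ApplyDamage ignores that flag; recovered health resets the owner's health effect.
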(event Custom|OnHitActorDestroyed
  (params (DestroyedActor :type Actor%20Object%20Reference))
  (Utilities|Map|Remove (Variables|Logic|GetHitRecord) DestroyedActor))

(event Custom|OnPointDamage
  (params (DamagedActor :type Actor%20Object%20Reference) (Damage :type Float%20%28single-precision%29) (InstigatedBy :type Controller%20Object%20Reference) (HitLocation :type Vector) (FHitComponent :type Primitive%20Component%20Object%20Reference) (BoneName :type Name) (ShotFromDirection :type Vector) (DamageType :type Damage%20Type%20Object%20Reference) (DamageCauser :type Actor%20Object%20Reference))
  ;[1 1 1] Point damage handling
  (Logic|ApplyDamage DamagedActor Damage "NewEnumerator0" false InstigatedBy DamageCauser (Logic|IsBoneHeadShot BoneName)))

(event Custom|OnServerChange
  ;[1 1 1] Config change handling
  (Variables|Logic-Config|SetRadialDamageMultipler (Variables|/CasualCQB/Root/Blueprints/Components/CP_GameState_Config.CP_GameState_Config_C|GetRadialDamageMultiplier (CallFunction|GetServerConfig))))

(event Custom|OnTakeRadialDamage
  (params (DamagedActor :type Actor%20Object%20Reference) (Damage :type Float%20%28single-precision%29) (DamageType :type Damage%20Type%20Object%20Reference) (Origin :type Vector) (HitInfo :type Hit%20Result%20Structure) (InstigatedBy :type Controller%20Object%20Reference) (DamageCauser :type Actor%20Object%20Reference))
  (bind _hitrecord (Variables|Logic|GetHitRecord))
  (bind (_value _returnvalue) (Utilities|Map|Find _hitrecord DamageCauser))
  ;[1 1 1] Radial damage handling
  (Logic|ApplyDamage DamagedActor Damage "NewEnumerator1" (not (and _returnvalue (<= (- (Utilities|Time|GetGameTimeinSeconds) _value) (Variables|Logic-Config|GetRecentTolleranceSeconds)))) InstigatedBy DamageCauser false))

(event Custom|OnInitialise
  (Utilities|SwitchHasAuthority
    (:Authority
      (Collision|BindEventtoOnComponentHit (Variables|Logic|GetMesh) (delegate Custom|OnMeshHit)))))

(event Custom|PostInterceptHeath
  (params (NewHealthTotal :type Float%20%28single-precision%29) (Delta :type Float%20%28single-precision%29))
  (bind _owner (Variables|Logic|GetOwner))
  (if (> Delta 0.0) ; Reset health effect on heal
    (if (>= (Logic|GetHealthPercentageFraction) (Variables|Logic-Config|GetHealthOKThreashold))
      (if (not (Audio|Components|Audio|IsPlaying (Variables|/HDCore/Core/BP_HDPlayerCharacterBase.BP_HDPlayerCharacterBase_C|GetLerpTimeline _owner))) ; Don't call if we are already playing as this will just reset the effect
        (Default|EventResetHealthEffect _owner)))))

(event Custom|OnDelayAfterHit
  (bind _owner (Variables|Logic|GetOwner))
  (if (>= (Logic|GetHealthPercentageFraction) (Variables|Logic-Config|GetHealthOKThreashold))
    (if (not (Audio|Components|Audio|IsPlaying (Variables|/HDCore/Core/BP_HDPlayerCharacterBase.BP_HDPlayerCharacterBase_C|GetLerpTimeline _owner))) ; Don't call if we are already playing as this will just reset the effect
      (Default|EventResetHealthEffect _owner))))

(event Custom|OnHitDamage
  (Utilities|Time|ClearandInvalidateTimerbyHandle (Variables|Logic|GetHitTimer))
  (bind _returnvalue (Utilities|Time|SetTimerbyEvent (delegate Custom|OnDelayAfterHit) (Variables|Logic-Config|GetAfterHitHealthCheckTime)))
  (Variables|Logic|SetHitTimer _returnvalue))

(event Custom|OnMeshHit
  (params (HitComponent :type Primitive%20Component%20Object%20Reference) (OtherActor :type Actor%20Object%20Reference) (OtherComp :type Primitive%20Component%20Object%20Reference) (NormalImpulse :type Vector) (Hit :type Hit%20Result%20Structure%20%28by%20ref%29))
  (Utilities|Casting|CastToBP_HDProj_BulletBase OtherActor ; Consider anything apart from bullets
    (:CastFailed
      (bind _ashdbase_projectile (Utilities|Casting|CastToHDBaseProjectile OtherActor)) ; Has to be a projectile
      (Logic|AddHitRecord _ashdbase_projectile) ; Record projectile hit
      (Logic|AddHitRecord (Components|GetOwner OtherActor)) ; Record projectile owner hit (weapon)
    )))

(event Custom|OnTakeAnyDamage
  (params (DamagedActor :type Actor%20Object%20Reference) (Damage :type Float%20%28single-precision%29) (DamageType :type Damage%20Type%20Object%20Reference) (InstigatedBy :type Controller%20Object%20Reference) (DamageCauser :type Actor%20Object%20Reference))
  (bind _returnvalue (Utilities|GetClass DamageType))
  ;[1 1 1] All damage handling
  (if (or (== _returnvalue "/Engine/EngineDamageTypes/DmgTypeBP_Environmental.DmgTypeBP_Environmental_C") (== _returnvalue "/CasualCQB/Root/Blueprints/BP_GenericDamageType.BP_GenericDamageType_C"))
    (Logic|ApplyDamage DamagedActor Damage "NewEnumerator2" false InstigatedBy DamageCauser false)))

(event EventBeginPlay
  (bind _config (CallFunction|GetServerConfig))
  (|CallParentFunction)
  (Utilities|SwitchHasAuthority
    (:Authority
      (bind _ascharacter (Utilities|Casting|CastToCharacter (Components|GetOwner)))
      (EventDispatchers|BindEventtoOnTakeRadialDamage _ascharacter (delegate Custom|OnTakeRadialDamage)) ; TODO: make sure these NEVER operate after dying
      (EventDispatchers|BindEventtoOnTakePointDamage _ascharacter (delegate Custom|OnPointDamage))
      ;[1 1 1] All damage handling
      (EventDispatchers|BindEventtoOnTakeAnyDamage _ascharacter (delegate Custom|OnTakeAnyDamage))
      ;[1 1 1] Config change handling
      (EventDispatchers|BindEventtoOnServerChange _config (delegate Custom|OnServerChange))
      (Variables|Logic-Config|SetRadialDamageMultipler (Variables|/CasualCQB/Root/Blueprints/Components/CP_GameState_Config.CP_GameState_Config_C|GetRadialDamageMultiplier _config)))))

(fn Initialise
  (params (Mesh :type Mesh%20Component%20Object%20Reference))
  (Variables|Logic|SetMesh Mesh)
  (bind _asbp_hdplayer_character_base (Utilities|Casting|CastToBP_HDPlayerCharacterBase (Components|GetOwner)))
  (Variables|Logic|SetOwner _asbp_hdplayer_character_base)
  (CallFunction|OnInitialise))

(fn AddHitRecord
  (params (Actor :type Actor%20Object%20Reference))
  (Utilities|Map|Add (Variables|Logic|GetHitRecord) Actor (Utilities|Time|GetGameTimeinSeconds)) ; Record actor hit and at what game time
  (Game|BindEventtoOnDestroyed Actor (EventDispatchers|CreateEvent :!event Custom|OnHitActorDestroyed)))

(fn TidyHitRecord
  (bind _keys (Utilities|Map|Keys (Variables|Logic|GetHitRecord)))
  (for _array_element _keys
    (if (not (Class|DFBlueprintFunctions|IsValidActor _array_element))
      (Utilities|Map|Remove (Variables|Logic|GetHitRecord) _array_element))))

(fn InterceptHealthChanged
  (params (NewHealthTotal :type Float%20%28single-precision%29) (PrevHealthTotal :type Float%20%28single-precision%29))
  (bind _output_get (LocalVariables|SetDelta (- NewHealthTotal PrevHealthTotal)))
  (if (> _output_get 0.0)
    (Variables|Logic|SetRealHealth NewHealthTotal) ; On health going up, simply allow it
    (CallFunction|PostInterceptHeath (Variables|Logic|GetRealHealth) (LocalVariables|GetDelta) :!label _label)
    (Default|CallOnHealthRefresh)
    (elif (< _output_get 0.0)
      (Variables|/Script/DonkehFramework.DFBaseCharacter|SetHealth (Variables|Logic|GetOwner) (Variables|Logic|GetRealHealth)) ; On health going down, block it - ignore all damage we don't manage
      (goto _label))))

(fn GetHealthPercentageFraction
  (bind _owner (Variables|Logic|GetOwner))
  (return (/ (Variables|/Script/DonkehFramework.DFBaseCharacter|GetHealth _owner) (Variables|/Script/DonkehFramework.DFBaseCharacter|GetMaxHealth _owner))))

(fn ApplyDamage
  (params (DamagedActor :type Actor%20Object%20Reference) (Damage :type Float%20%28single-precision%29) (Type :type DamageType%20Enum :default "NewEnumerator2") (ReduceDamage :type Boolean) (DamageInstigator :type Controller%20Object%20Reference) (DamageCauser :type Actor%20Object%20Reference) (HeadShot :type Boolean))
  (bind _config (CallFunction|GetServerConfig))
  (bind (_feedbackinitialdelay _playerrevivedhealth _airevivedhealth) (Utilities|GetClassDefaults "/CasualCQB/Root/Blueprints/BP_Resuscitator.BP_Resuscitator_C"))
  (bind _radialdamagemultipler (Variables|Logic-Config|GetRadialDamageMultipler))
  (bind _pointdamagemultipler (Variables|Logic-Config|GetPointDamageMultipler))
  (bind _returnvalue (Utilities|Select :Index Type :NewEnumerator2 1.0 :NewEnumerator0 _pointdamagemultipler :NewEnumerator1 _radialdamagemultipler))
  (bind _returnvalue_2 (* Damage _returnvalue))
  (bind _asdfbase_character (Utilities|Casting|CastToDFBaseCharacter DamagedActor))
  (if (and (Class|DFBaseCharacter|IsAlive _asdfbase_character) (not (Variables|Logic|GetbDisableDamage)))
    (bind (_inprotection _downedordead) (Class|IFDamage|OnApplyDamage(Message) (Variables|Logic|GetOwner)))
    (if (and (not _inprotection) (not _downedordead))
      (bind _output_get (LocalVariables|SetTmpHealth (Math|Float|Clamp(Float) (- (Variables|Logic|GetRealHealth) _returnvalue_2) 0.0 (Variables|/Script/DonkehFramework.DFBaseCharacter|GetMaxHealth (Variables|Logic|GetOwner)))))
      (if (<= _output_get 0.0)
        (LocalVariables|SetbHealthZero true)
        (Variables|Logic|SetbDisableDamage true)
        (LocalVariables|SetTmpHealth (Math|Float|SelectFloat (Math|Float|SelectFloat _playerrevivedhealth _airevivedhealth (not (Pawn|IsBotControlled (Variables|Logic|GetOwner)))) 0.0 (and (Variables|/CasualCQB/Root/Blueprints/Components/CP_GameState_Config.CP_GameState_Config_C|GetAllowRevive _config) (or (not (Variables|/CasualCQB/Root/Blueprints/Components/CP_GameState_Config.CP_GameState_Config_C|GetbNoReviveOnHeadshot _config)) (not HeadShot))))))
      (bind _output_get_2 (Variables|Logic|SetRealHealth (LocalVariables|GetTmpHealth)))
      (Default|CallOnDamage _returnvalue_2 _output_get_2 DamageInstigator DamageCauser HeadShot (LocalVariables|GetbHealthZero) (> (Variables|Logic|GetRealHealth) 0.0))
      (Default|CallOnHealthRefresh)
      (else
        (Default|CallOnDamageBlocked DamageInstigator DamageCauser)))))

(fn SetHealth
  (params (Health :type Float%20%28single-precision%29))
  (bind _output_get (Variables|Logic|SetRealHealth (Math|Float|Clamp(Float) Health 0.0 (Variables|/Script/DonkehFramework.DFBaseCharacter|GetMaxHealth (Variables|Logic|GetOwner)))))
  (Variables|/Script/DonkehFramework.DFBaseCharacter|SetHealth (Variables|Logic|GetOwner) _output_get) ; To force a normal health mutation
)

(fn AdjustHealth
  (params (Delta :type Float%20%28single-precision%29))
  (Logic|SetHealth (+ (Variables|Logic|GetRealHealth) Delta)))

(fn IsBoneHeadShot
  (params (Bone :type Name))
  (return (Utilities|Enum|Equal(Enum) (Utilities|String|ToString(Name) Bone) "head")))

(fn EnableDamage
  (params (State :type Boolean))
  (Variables|Logic|SetbDisableDamage (not State)))