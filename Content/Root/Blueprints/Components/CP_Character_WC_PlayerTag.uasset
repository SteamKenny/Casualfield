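; Widget component that shows a character's player tag and can swap it for a Sauron-mode variant.
; On BeginPlay, where cosmetic events can run, it initialises and caches the standard tag widget.
; If the client controller has Sauron active, it notifies any BP_Sauron actor of the spawned pawn and switches to the Sauron tag.
; SauronOn creates that replacement widget, and SauronOff removes it and restores the cached original.
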(event Custom|SauronOn
  (bind _aspawn (Utilities|Casting|CastToPawn (Components|GetOwner)))
  (bind _returnvalue (UserInterface|CreateWidget "/CasualCQB/Root/UI/HUD/WBP_Player_Tag_Sauron.WBP_Player_Tag_Sauron_C" 0 _aspawn))
  (UserInterface|SetWidget _returnvalue))

(event Custom|SauronOff
  (Widget|RemovefromParent (UserInterface|GetUserWidgetObject))
  (UserInterface|SetWidget (Variables|Logic|GetOriginalWidget)))

(event EventBeginPlay
  (|CallParentFunction)
  (Networking|CanExecuteCosmeticEvents
    (:True
      (bind _aswbp_player_tag (Utilities|Casting|CastToWBP_PlayerTag (UserInterface|GetUserWidgetObject)))
      (bind _aspawn (Utilities|Casting|CastToPawn (Components|GetOwner)))
      (Default|Initialise _aswbp_player_tag _aspawn self)
      (Variables|Logic|SetOriginalWidget _aswbp_player_tag)
      (bind _asbp_hdplayer_controller_cqb (Utilities|Casting|CastToBP_HDPlayerController_CQB (CallFunction|GetClientPlayerController)))
      (if (Variables|/CasualCQB/Root/Core/BP_HDPlayerController_CQB.BP_HDPlayerController_CQB_C|GetbSauronActive _asbp_hdplayer_controller_cqb)
        (bind _returnvalue (Actor|GetActorOfClass "/CasualCQB/Root/Blueprints/_Experimental_/BP_Sauron.BP_Sauron_C"))
        (Utilities|IsValid _returnvalue
          (:Is%20Valid
            (bind _aspawn_2 (Utilities|Casting|CastToPawn (Components|GetOwner)))
            (Default|OnPawnSpawn _returnvalue _aspawn_2))
          (:Is%20Not%20Valid
            _))
        (CallFunction|Sauronon)))))