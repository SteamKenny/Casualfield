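; CP_Game_Tickets is a component that records each team's starting ticket counts for a match.
; On BeginPlay it copies BLUFOR and OPFOR tickets from the HD game state and then flags the values as ready.
; A WaitFor function reports that readiness for the starting-tickets case and returns true otherwise, while GetTickets is an empty stub.
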(event EventBeginPlay
  (bind _hdgamestate (CallFunction|GetHDGameState))
  (|CallParentFunction)
  (Variables|Logic|SetBluForStartingTickets (Variables|/Script/HDMain.HDGameState|GetBluforTickets _hdgamestate))
  (Variables|Logic|SetOpForStartingTickets (Variables|/Script/HDMain.HDGameState|GetOpforTickets _hdgamestate))
  (Variables|Logic|SetStartingTicketsReady true))

(event EventTick
  (params (DeltaSeconds :type Float%20%28single-precision%29)))

(fn GetTickets
  (return 0))

(fn Waitfor
  (params (IsReady :type String))
  (switch string IsReady
    (:Default
      (return true))
    (:StartingTickets
      (return (Variables|Logic|GetStartingTicketsReady)))))