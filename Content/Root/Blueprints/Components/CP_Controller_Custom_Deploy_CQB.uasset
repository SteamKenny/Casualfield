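; Controller component that reworks an existing deploy menu for CQB at runtime.
; On Initialise it injects server, squad, scoreboard, minimap, background and info widgets into the menu's panels and replaces the deploy button.
; A squad toggle swaps squad selection with a mini scoreboard, which is rebuilt on state changes, keeping scroll positions.
; Death and reset manage a POI actor, minimap last-position marker and drone sound; alive state gates background and suicide button.
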(event Custom|OnScoreboardStateChanged
  (Utilities|IsValid (Variables|Logic|GetDeployMenu)
    (:Is%20Valid
      (Logic|CreateScoreboardWidget (stale Custom|RefreshScoreboardUI PlayerController)))))

(event Custom|RequestListUpdate
  (bind _miniscoreboardwidget (Variables|Logic|GetMiniScoreboardWidget))
  (Utilities|IsValid _miniscoreboardwidget
    (:Is%20Valid
      (Default|OnRequestListRefresh _miniscoreboardwidget))))

(event Custom|OnClassSelectionScroll
  (params (CurrentOffset :type Float%20%28single-precision%29))
  (Variables|Logic|SetUserClassSelectionScrollPos CurrentOffset))

(event Custom|OnReset
  (Utilities|IsValid (Variables|Logic|GetDeathPOIActor)
    (:Is%20Valid
      (Actor|DestroyActor (Variables|Logic|GetDeathPOIActor))
      (Variables|Logic|SetDeathPOIActor 0))
    (:Is%20Not%20Valid
      _))
  (Logic|ClearMinimapLastPosition)
  (Logic|StartStopBackgroundSFX false))

(event Custom|RefreshScoreboardUI
  (params (PlayerController :type Player%20Controller%20Object%20Reference))
  (Utilities|IsValid (Variables|Logic|GetDeployMenu)
    (:Is%20Valid
      (Logic|CreateScoreboardWidget PlayerController))))

(event Custom|SquadToggleEvent
  (bind _output_get (Variables|Logic|SetbScoreboardShown (Class|KismetMathLibrary|XORBoolean (Variables|Logic|GetbScoreboardShown) true)))
  (Variables|/CasualCQB/Root/UI/DeployMenu/WBP_ScoreboardSquad.WBP_ScoreboardSquad_C|SetbScoreboardShown (Variables|Logic|GetScoreboardSquadWidget) _output_get)
  (Logic|UpdateUI))

(event Custom|AutoSquadJoinToggle
  (params (IsChecked :type Boolean))
  (Default|CallOnAutoSquadJoinToggle IsChecked))

(event Custom|Initialise
  (params (DeployMenu :type WBP%20Deploy%20Menu%20Object%20Reference) (PlayerController :type Player%20Controller%20Object%20Reference))
  (Variables|Logic|SetDeployMenu DeployMenu)
  (Logic|RepositionSquadUI)
  (Logic|CreateServerWidget PlayerController)
  (Logic|CreateSquadWidget PlayerController)
  (Logic|CreateScoreboardWidget PlayerController)
  (Logic|CreateMinimapAddonUI PlayerController)
  (Logic|CreateMinimapAddonUILower PlayerController)
  (Logic|CreateDeployButtonWidget PlayerController)
  (Logic|CreateInformationWidget)
  (Logic|CreateBackgroundWidget)
  (Logic|CreateMapArtWidget)
  (Logic|GrabSuicideButton)
  (Logic|HookClassSelectionScroll)
  (EventDispatchers|BindEventtoOnSquadToggle (Variables|Logic|GetScoreboardSquadWidget) (delegate Custom|SquadToggleEvent))
  (EventDispatchers|BindEventtoOnAutoSquadJoinToggle (Variables|Logic|GetScoreboardSquadWidget) (delegate Custom|AutoSquadJoinToggle))
  (Logic|StartStopBackgroundSFX true)
  (Variables|Logic|SetbInitialised true))

(event Custom|OnDeployMenuClose
  (Default|CloseDialog (Variables|Logic|GetServerWidget)))

(event Custom|OnAllowSuicide
  (params (Allow :type Boolean))
  (bind _suicidebutton (Variables|Logic|GetSuicideButton))
  (Variables|Logic|SetbAllowSuicide Allow)
  (Utilities|IsValid _suicidebutton
    (:Is%20Valid
      (Widget|SetIsEnabled _suicidebutton (and Allow (Logic|IsPlayerAlive))))))

(event Custom|OnDeployMenuOpen
  (CallFunction|OnAllowSuicide (Variables|Logic|GetbAllowSuicide))
  (Logic|SetBackgroundVisibility)
  (Logic|SetClassSelectionScrollPos)
  (CallFunction|RequestListUpdate) ; XXX: this used to be done on show/hide controller tick - is this as good here?
)

(event Custom|OnDeath
  (params (LastTransform :type Transform))
  (bind _returnvalue (Game|SpawnActorfromClass "/CasualCQB/Root/Blueprints/BP_DeathPOI.BP_DeathPOI_C" LastTransform "AlwaysSpawn" 0 0))
  (Variables|Logic|SetDeathPOIActor _returnvalue)
  (Logic|SetMinimapLastPosition (.Location (Math|Transform|BreakTransform LastTransform)))
  (Logic|SetBackgroundVisibility)
  (Logic|StartStopBackgroundSFX true))

(event EventBeginPlay)

(fn RepositionSquadUI
  (bind _ascanvas_panel_slot (Utilities|Casting|CastToCanvasPanelSlot (Variables|/Script/UMG.Widget|GetSlot (Variables|/HDCore/UI/DeployMenu/WBP_DeployMenu.WBP_DeployMenu_C|GetSquadSelectionPanel (Variables|Logic|GetDeployMenu)))))
  (Class|CanvasPanelSlot|SetPosition _ascanvas_panel_slot (Math|Vector2D|MakeVector2D (.X (Math|Vector2D|BreakVector2D (Class|CanvasPanelSlot|GetPosition _ascanvas_panel_slot))) (+ (.Y (Math|Vector2D|BreakVector2D (Class|CanvasPanelSlot|GetPosition _ascanvas_panel_slot))) 64.0))))

(fn CreateMapArtWidget
  (params (PlayerController :type Player%20Controller%20Object%20Reference))
  (Utilities|FlowControl|Sequence
    (:then_0
      (bind _returnvalue (UserInterface|CreateWidget "/CasualCQB/Root/UI/DeployMenu/WBP_MapArt.WBP_MapArt_C" PlayerController))
      (bind _output_get (Variables|Logic|SetMapArtWidget _returnvalue))
      (bind _returnvalue_2 (Widget|Panel|AddChild (Widget|GetParent (Variables|/HDCore/UI/DeployMenu/WBP_DeployMenu.WBP_DeployMenu_C|GetClassSelectionPanel (Variables|Logic|GetDeployMenu))) _output_get))
      (bind _ascanvas_panel_slot (Utilities|Casting|CastToCanvasPanelSlot _returnvalue_2))
      (Class|CanvasPanelSlot|SetAlignment _ascanvas_panel_slot "(X=0.500000,Y=0.500000)")
      (Class|CanvasPanelSlot|SetAnchors _ascanvas_panel_slot (Utilities|Struct|MakeAnchors "(X=0.500000,Y=0.500000)" "(X=0.500000,Y=0.500000)"))
      (Class|CanvasPanelSlot|SetSize _ascanvas_panel_slot "(X=560.000000,Y=75.000000)")
      (Class|CanvasPanelSlot|SetPosition _ascanvas_panel_slot "(X=0.000000,Y=-370.000000)")
      (Class|CanvasPanelSlot|SetZOrder _ascanvas_panel_slot))
    (:then_1
      (Widget|SetVisibility (Variables|/HDCore/UI/DeployMenu/WBP_DeployMenu.WBP_DeployMenu_C|GetMapNameText (Variables|Logic|GetDeployMenu)) "Hidden"))))

(fn CreateBackgroundWidget
  (params (PlayerController :type Player%20Controller%20Object%20Reference))
  (Utilities|FlowControl|Sequence
    (:then_0
      (bind _returnvalue (UserInterface|CreateWidget "/CasualCQB/Root/UI/DeployMenu/WBP_Background.WBP_Background_C" PlayerController))
      (bind _output_get (Variables|Logic|SetBackgroundWidget _returnvalue))
      (bind _returnvalue_2 (Widget|Panel|AddChild (Widget|GetParent (Variables|/HDCore/UI/DeployMenu/WBP_DeployMenu.WBP_DeployMenu_C|GetClassSelectionPanel (Variables|Logic|GetDeployMenu))) _output_get))
      (bind _ascanvas_panel_slot (Utilities|Casting|CastToCanvasPanelSlot _returnvalue_2))
      (Class|CanvasPanelSlot|SetAlignment _ascanvas_panel_slot "(X=0.500000,Y=0.500000)")
      (Class|CanvasPanelSlot|SetAnchors _ascanvas_panel_slot (Utilities|Struct|MakeAnchors "(X=0.000000,Y=0.000000)" "(X=1.000000,Y=1.000000)"))
      (Class|CanvasPanelSlot|SetSize _ascanvas_panel_slot "(X=1920.000000,Y=1080.000000)")
      (Class|CanvasPanelSlot|SetPosition _ascanvas_panel_slot "(X=0.000000,Y=0.000000)")
      (Class|CanvasPanelSlot|SetZOrder _ascanvas_panel_slot -1)
      (Class|CanvasPanelSlot|SetOffsets _ascanvas_panel_slot (Utilities|Struct|MakeMargin 0.0 0.0 0.0 0.0)))
    (:then_1
      (Class|CanvasPanelSlot|SetZOrder (Class|WidgetLayoutLibrary|SlotasCanvasSlot (Widget|GetParent (Variables|/HDCore/UI/DeployMenu/WBP_DeployMenu.WBP_DeployMenu_C|GetBgImg (Variables|Logic|GetDeployMenu)))) -2))))

(fn CreateServerWidget
  (params (PlayerController :type Player%20Controller%20Object%20Reference))
  (bind _returnvalue (UserInterface|CreateWidget "/CasualCQB/Root/UI/DeployMenu/WBP_Server_Information.WBP_Server_Information_C" PlayerController))
  (bind _output_get (Variables|Logic|SetServerWidget _returnvalue))
  (bind _returnvalue_2 (Widget|Panel|AddChild (Widget|GetParent (Variables|/HDCore/UI/DeployMenu/WBP_DeployMenu.WBP_DeployMenu_C|GetClassSelectionPanel (Variables|Logic|GetDeployMenu))) _output_get))
  (bind _ascanvas_panel_slot (Utilities|Casting|CastToCanvasPanelSlot _returnvalue_2))
  (Class|CanvasPanelSlot|SetAlignment _ascanvas_panel_slot "(X=1.000000,Y=0.000000)")
  (Class|CanvasPanelSlot|SetAnchors _ascanvas_panel_slot (Utilities|Struct|MakeAnchors "(X=1.000000,Y=0.000000)" "(X=1.000000,Y=0.000000)"))
  (Class|CanvasPanelSlot|SetSize _ascanvas_panel_slot "(X=580.000000,Y=140.000000)")
  (Class|CanvasPanelSlot|SetPosition _ascanvas_panel_slot "(X=-64.000000,Y=64.000000)"))

(fn CreateScoreboardWidget
  (params (PlayerController :type Player%20Controller%20Object%20Reference))
  (bind _deploymenu (Variables|Logic|GetDeployMenu))
  (bind _squadselectionpanel (Variables|/HDCore/UI/DeployMenu/WBP_DeployMenu.WBP_DeployMenu_C|GetSquadSelectionPanel _deploymenu))
  (Utilities|IsValid (Variables|Logic|GetMiniScoreboardWidget)
    (:Is%20Valid
      (LocalVariables|SetPreviousBluForScrollPos (Variables|/CasualCQB/Root/UI/ScoreboardMenu/WBP_HDScoreboardMenu_Mini_CQB.WBP_HDScoreboardMenu_Mini_CQB_C|GetBluForScrollPosition (Variables|Logic|GetMiniScoreboardWidget)))
      (LocalVariables|SetPreviousOpForScrollPos (Variables|/CasualCQB/Root/UI/ScoreboardMenu/WBP_HDScoreboardMenu_Mini_CQB.WBP_HDScoreboardMenu_Mini_CQB_C|GetOpForScrollPosition (Variables|Logic|GetMiniScoreboardWidget)))
      (Widget|RemovefromParent (Variables|Logic|GetMiniScoreboardWidget)))
    (:Is%20Not%20Valid
      _))
  (Widget|SetVisibility _squadselectionpanel (select (Variables|Logic|GetbScoreboardShown) "Hidden" "Visible"))
  (bind _returnvalue (UserInterface|CreateWidget "/CasualCQB/Root/UI/ScoreboardMenu/WBP_HDScoreboardMenu_Mini_CQB.WBP_HDScoreboardMenu_Mini_CQB_C" PlayerController))
  (bind _output_get (Variables|Logic|SetMiniScoreboardWidget _returnvalue))
  (EventDispatchers|BindEventtoOnStateChanged _output_get (EventDispatchers|CreateEvent :!event Custom|OnScoreboardStateChanged))
  (bind _returnvalue_2 (Widget|Panel|AddChild (Widget|GetParent _squadselectionpanel) _output_get))
  (bind _ascanvas_panel_slot (Utilities|Casting|CastToCanvasPanelSlot _returnvalue_2))
  (bind _ascanvas_panel_slot_2 (Utilities|Casting|CastToCanvasPanelSlot (Variables|/Script/UMG.Widget|GetSlot _squadselectionpanel)))
  (Class|CanvasPanelSlot|SetPosition _ascanvas_panel_slot (Class|CanvasPanelSlot|GetPosition _ascanvas_panel_slot_2))
  (Class|CanvasPanelSlot|SetLayout _ascanvas_panel_slot (Class|CanvasPanelSlot|GetLayout _ascanvas_panel_slot_2))
  (Class|CanvasPanelSlot|SetSize _ascanvas_panel_slot (Class|CanvasPanelSlot|GetSize _ascanvas_panel_slot_2))
  (Widget|SetVisibility (Variables|Logic|GetMiniScoreboardWidget) (select (Variables|Logic|GetbScoreboardShown) "Visible" "Hidden"))
  (Default|SetScrollPositions (Variables|Logic|GetMiniScoreboardWidget) (LocalVariables|GetPreviousBluForScrollPos) (LocalVariables|GetPreviousOpForScrollPos)))

(fn CreateMinimapAddonUI
  (params (PlayerController :type Player%20Controller%20Object%20Reference))
  (bind _deploymenu (Variables|Logic|GetDeployMenu))
  (bind _deploymenu_2 (Variables|Logic|GetDeployMenu))
  (bind _suicidebtn (Variables|/HDCore/UI/DeployMenu/WBP_DeployMenu.WBP_DeployMenu_C|GetSuicideBtn _deploymenu_2))
  (bind _returnvalue (Widget|GetParent _suicidebtn))
  (bind _returnvalue_2 (Widget|GetParent _returnvalue))
  (bind _returnvalue_3 (UserInterface|CreateWidget "/CasualCQB/Root/UI/DeployMenu/WBP_Minimap_AddonUI.WBP_Minimap_AddonUI_C" PlayerController (Variables|/HDCore/UI/DeployMenu/WBP_DeployMenu.WBP_DeployMenu_C|GetSpawnMapView _deploymenu) _deploymenu))
  (bind _returnvalue_4 (Widget|Panel|AddChild _returnvalue_2 _returnvalue_3))
  (bind _ashorizontal_box (Utilities|Casting|CastToHorizontalBox _returnvalue_2))
  (bind _output_get (LocalVariables|SetTempWidget (Class|PanelWidget|GetChildat _ashorizontal_box 1)))
  (Class|PanelWidget|RemoveChildat _ashorizontal_box 1)
  (Widget|Panel|AddChild _ashorizontal_box _output_get)
  (bind _ashorizontal_box_slot (Utilities|Casting|CastToHorizontalBoxSlot _returnvalue_4))
  (Layout|GridSlot|SetHorizontalAlignment _ashorizontal_box_slot "HAlign_Fill")
  (Class|HorizontalBoxSlot|SetSize _ashorizontal_box_slot (Utilities|Struct|MakeSlateChildSize 1.0 "Fill"))
  (Layout|BorderSlot|SetPadding (Class|WidgetLayoutLibrary|SlotasHorizontalBoxSlot (Class|PanelWidget|GetChildat _ashorizontal_box)) (Utilities|Struct|MakeMargin) :!class /Script/UMG.HorizontalBoxSlot))

(fn CreateInformationWidget
  (params (PlayerController :type Player%20Controller%20Object%20Reference))
  (bind _returnvalue (UserInterface|CreateWidget "/CasualCQB/Root/UI/DeployMenu/WBP_Information.WBP_Information_C" PlayerController))
  (bind _output_get (Variables|Logic|SetInformationWidget _returnvalue))
  (bind _returnvalue_2 (Widget|Panel|AddChild (Widget|GetParent (Variables|/HDCore/UI/DeployMenu/WBP_DeployMenu.WBP_DeployMenu_C|GetClassSelectionPanel (Variables|Logic|GetDeployMenu))) _output_get))
  (bind _ascanvas_panel_slot (Utilities|Casting|CastToCanvasPanelSlot _returnvalue_2))
  (Class|CanvasPanelSlot|SetAlignment _ascanvas_panel_slot "(X=4.500000,Y=1.000000)")
  (Class|CanvasPanelSlot|SetAnchors _ascanvas_panel_slot (Utilities|Struct|MakeAnchors "(X=0.851062,Y=1.000000)" "(X=0.851062,Y=1.000000)"))
  (Class|CanvasPanelSlot|SetSize _ascanvas_panel_slot "(X=512.000000,Y=64.000000)")
  (Class|CanvasPanelSlot|SetPosition _ascanvas_panel_slot "(X=2000.000000,Y=-48.000000)"))

(fn CreateMinimapAddonUILower
  (params (PlayerController :type Player%20Controller%20Object%20Reference))
  (bind _returnvalue (UserInterface|CreateWidget "/CasualCQB/Root/UI/DeployMenu/WBP_Minimap_AddonUI_Lower.WBP_Minimap_AddonUI_Lower_C" PlayerController (Variables|Logic|GetDeployMenu)))
  (Widget|Panel|AddChild (Widget|GetParent (Variables|/HDCore/UI/DeployMenu/WBP_DeployMenu.WBP_DeployMenu_C|GetSpawnMapView (Variables|Logic|GetDeployMenu))) _returnvalue))

(fn CreateDeployButtonWidget
  (params (PlayerController :type Player%20Controller%20Object%20Reference))
  (LocalVariables|SetParentWidget (Widget|GetParent (Variables|/HDCore/UI/DeployMenu/WBP_DeployMenu.WBP_DeployMenu_C|GetDeployBtn (Variables|Logic|GetDeployMenu))))
  (Widget|RemovefromParent (Variables|/HDCore/UI/DeployMenu/WBP_DeployMenu.WBP_DeployMenu_C|GetDeployBtn (Variables|Logic|GetDeployMenu)))
  (bind _returnvalue (UserInterface|CreateWidget "/CasualCQB/Root/UI/DeployMenu/WBP_DeployMenu_DeployButton_CQB.WBP_DeployMenu_DeployButton_CQB_C" PlayerController (Variables|Logic|GetDeployMenu)))
  (bind _output_get (Variables|/HDCore/UI/DeployMenu/WBP_DeployMenu.WBP_DeployMenu_C|SetDeployBtn (Variables|Logic|GetDeployMenu) _returnvalue))
  (Widget|Panel|AddChild (LocalVariables|GetParentWidget) _output_get)
  (EventDispatchers|BindEventtoOnClicked _output_get (EventDispatchers|CreateEvent (Variables|Logic|GetDeployMenu) :!event BndEvtDeployBtnK2NodeComponentBoundEvent7onClickedDelegateSignature)))

(fn CreateSquadWidget
  (params (PlayerController :type Player%20Controller%20Object%20Reference))
  (bind _deploymenu (Variables|Logic|GetDeployMenu))
  (bind _squadselectionpanel (Variables|/HDCore/UI/DeployMenu/WBP_DeployMenu.WBP_DeployMenu_C|GetSquadSelectionPanel _deploymenu))
  (bind _returnvalue (UserInterface|CreateWidget "/CasualCQB/Root/UI/DeployMenu/WBP_ScoreboardSquad.WBP_ScoreboardSquad_C"))
  (bind _output_get (Variables|Logic|SetScoreboardSquadWidget _returnvalue))
  (bind _returnvalue_2 (Widget|Panel|AddChild (Widget|GetParent _squadselectionpanel) _output_get))
  (bind _ascanvas_panel_slot (Utilities|Casting|CastToCanvasPanelSlot _returnvalue_2))
  (bind _ascanvas_panel_slot_2 (Utilities|Casting|CastToCanvasPanelSlot (Variables|/Script/UMG.Widget|GetSlot _squadselectionpanel)))
  (Class|CanvasPanelSlot|SetSize _ascanvas_panel_slot_2 "(X=512.000000,Y=644.000000)")
  (Class|CanvasPanelSlot|SetLayout _ascanvas_panel_slot (Class|CanvasPanelSlot|GetLayout _ascanvas_panel_slot_2))
  (Class|CanvasPanelSlot|SetPosition _ascanvas_panel_slot (Math|Vector2D|MakeVector2D (.X (Math|Vector2D|BreakVector2D (Class|CanvasPanelSlot|GetPosition _ascanvas_panel_slot_2))) -3e+02))
  (Class|CanvasPanelSlot|SetSize _ascanvas_panel_slot "(X=512.000000,Y=40.000000)"))

(fn UpdateUI
  (Widget|SetVisibility (Variables|Logic|GetMiniScoreboardWidget) (select (Variables|Logic|GetbScoreboardShown) "Visible" "Hidden"))
  (Widget|SetVisibility (Variables|/HDCore/UI/DeployMenu/WBP_DeployMenu.WBP_DeployMenu_C|GetSquadSelectionPanel (Variables|Logic|GetDeployMenu)) (select (Variables|Logic|GetbScoreboardShown) "Hidden" "Visible")))

(fn SetMinimapLastPosition
  (params (LastPosition :type Vector))
  (bind _aswbp_deploy_menu_spawn_minimap_ex_cqb (Utilities|Casting|CastToWBP_DeployMenu_SpawnMinimap_Ex_CQB (Variables|/HDCore/UI/DeployMenu/SpawnMap/WBP_DeployMenu_SpawnMapView.WBP_DeployMenu_SpawnMapView_C|GetMinimap (Variables|/HDCore/UI/DeployMenu/WBP_DeployMenu.WBP_DeployMenu_C|GetSpawnMapView (Variables|Logic|GetDeployMenu)))))
  (Default|SetLastWorldPosition _aswbp_deploy_menu_spawn_minimap_ex_cqb LastPosition))

(fn ClearMinimapLastPosition
  (bind _aswbp_deploy_menu_spawn_minimap_ex_cqb (Utilities|Casting|CastToWBP_DeployMenu_SpawnMinimap_Ex_CQB (Variables|/HDCore/UI/DeployMenu/SpawnMap/WBP_DeployMenu_SpawnMapView.WBP_DeployMenu_SpawnMapView_C|GetMinimap (Variables|/HDCore/UI/DeployMenu/WBP_DeployMenu.WBP_DeployMenu_C|GetSpawnMapView (Variables|Logic|GetDeployMenu)))))
  (Default|Reset _aswbp_deploy_menu_spawn_minimap_ex_cqb))

(fn GrabSuicideButton
  (Variables|Logic|SetSuicideButton (Variables|/HDCore/UI/DeployMenu/WBP_DeployMenu.WBP_DeployMenu_C|GetSuicideBtn (Variables|Logic|GetDeployMenu))))

(fn IsPlayerAlive
  (bind _ascontroller (Utilities|Casting|CastToController (Components|GetOwner))
    (:then
      (bind _asdfbase_character (Utilities|Casting|CastToDFBaseCharacter (Pawn|GetControlledPawn _ascontroller))
        (:then
          (return (Class|DFBaseCharacter|IsAlive _asdfbase_character)))
        (:CastFailed
          _)))
    (:CastFailed
      _))
  (return false))

(fn SetBackgroundVisibility
  (Utilities|IsValid (Variables|Logic|GetBackgroundWidget)
    (:Is%20Valid
      (Widget|SetVisibility (Variables|Logic|GetBackgroundWidget) (select (not (Logic|IsPlayerAlive)) "Visible" "Hidden")))))

(fn HookClassSelectionScroll
  (EventDispatchers|BindEventtoOnUserScrolled (Variables|/HDCore/UI/DeployMenu/ClassSelection/WBP_DeployMenu_ClassSelectionPanel.WBP_DeployMenu_ClassSelectionPanel_C|GetClassScrollBox (Variables|/HDCore/UI/DeployMenu/WBP_DeployMenu.WBP_DeployMenu_C|GetClassSelectionPanel (Variables|Logic|GetDeployMenu))) (EventDispatchers|CreateEvent :!event Custom|OnClassSelectionScroll)))

(fn SetClassSelectionScrollPos
  (bind _deploymenu (Variables|Logic|GetDeployMenu))
  (Utilities|IsValid _deploymenu
    (:Is%20Valid
      (Class|ScrollBox|SetScrollOffset (Variables|/HDCore/UI/DeployMenu/ClassSelection/WBP_DeployMenu_ClassSelectionPanel.WBP_DeployMenu_ClassSelectionPanel_C|GetClassScrollBox (Variables|/HDCore/UI/DeployMenu/WBP_DeployMenu.WBP_DeployMenu_C|GetClassSelectionPanel _deploymenu)) (Variables|Logic|GetUserClassSelectionScrollPos)))))

(fn StartStopBackgroundSFX
  (params (Start :type Boolean))
  (if Start
    (Utilities|IsValid (Variables|Logic|GetBackgroundSFX)
      (:Is%20Not%20Valid
        (bind _returnvalue (Audio|SpawnSound2D "/CasualCQB/Root/Audio/industrial-pulse-drone-27456.industrial-pulse-drone-27456" (Variables|Logic-Config|GetBackgroundSFXVolume) 1.0 0.0 0))
        (Variables|Logic|SetBackgroundSFX _returnvalue)))
    (else
      (Utilities|IsValid (Variables|Logic|GetBackgroundSFX)
        (:Is%20Valid
          (Audio|Components|Audio|FadeOut (Variables|Logic|GetBackgroundSFX) (Variables|Logic-Config|GetBackgroundSFXVolume_FadeOutSeconds) 0.0 "Logarithmic" :!class /Script/Engine.AudioComponent))))))