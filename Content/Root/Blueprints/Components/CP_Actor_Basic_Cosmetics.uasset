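; Actor component that provides basic cosmetic effects: a ghost material swap and an outline-style highlight.
; Ghosting swaps slot 0 on static meshes tagged BasicGhost, caching originals for restore, while highlighting toggles custom depth on meshes tagged BasicHighlight.
; Initialise adds a post-process material to a given camera, defaulting to an outline instance, and Remove strips matching entries.
; All events except Remove are gated by CanExecuteCosmeticEvents.
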(event Custom|Initialise
  (params (Camera :type Camera%20Component%20Object%20Reference) (PostProcessMaterial :type Material%20Instance%20Object%20Reference))
  (Networking|CanExecuteCosmeticEvents
    (:True
      (Utilities|Array|AddUnique (Utilities|Struct|BreakWeightedBlendables (Utilities|Struct|BreakPostProcessSettings (Variables|/Script/Engine.CameraComponent|GetPostProcessSettings Camera))) (Utilities|Struct|MakeWeightedBlendable 1.0 (select (Utilities|IsValid PostProcessMaterial) PostProcessMaterial "/Detonation/Root/Materials/M_Outline_Only_Inst.M_Outline_Only_Inst"))))))

(event Custom|Remove
  (params (Camera :type Camera%20Component%20Object%20Reference) (PostProcessMaterial :type Material%20Instance%20Object%20Reference))
  (bind _postprocesssettings (Variables|/Script/Engine.CameraComponent|GetPostProcessSettings Camera))
  (bind _weightedblendables (Utilities|Struct|BreakPostProcessSettings _postprocesssettings))
  (bind _array (Utilities|Struct|BreakWeightedBlendables _weightedblendables))
  (for _array_element _array
    (if (== (.Object (Utilities|Struct|BreakWeightedBlendable _array_element)) PostProcessMaterial)
      (Utilities|Array|AddUnique (Variables|Logic|GetRemoveAt) _array_element)))
  (for _array_element_2 (Variables|Logic|GetRemoveAt)
    (Utilities|Array|RemoveItem _array _array_element_2)))

(event EventBeginPlay)

(event EventSetHighlightState
  (params (Enabled :type Boolean))
  (Networking|CanExecuteCosmeticEvents
    (:True
      (for _array_element (Actor|GetComponentsbyTag (Components|GetOwner) "/Script/Engine.MeshComponent" "BasicHighlight")
        (bind _asmesh_component (Utilities|Casting|CastToMeshComponent _array_element))
        (Rendering|SetRenderCustomDepth _asmesh_component Enabled)))))

(event EventSetGhostState
  (params (Enabled :type Boolean))
  (Networking|CanExecuteCosmeticEvents
    (:True
      (for _array_element (Actor|GetComponentsbyTag (Components|GetOwner) "/Script/Engine.StaticMeshComponent" "BasicGhost")
        (bind _asstatic_mesh_component (Utilities|Casting|CastToStaticMeshComponent _array_element))
        (if Enabled
          (Utilities|Map|Add (Variables|Logic|GetOriginalMaterials) _asstatic_mesh_component (Rendering|Material|GetMaterial _asstatic_mesh_component 0))
          (Rendering|Material|SetMaterial _asstatic_mesh_component 0 (Variables|Logic|GetGhostMaterial))
          (elif (.ReturnValue (Utilities|Map|Find (Variables|Logic|GetOriginalMaterials) _asstatic_mesh_component))
            (Rendering|Material|SetMaterial _asstatic_mesh_component 0 (.Value (Utilities|Map|Find (Variables|Logic|GetOriginalMaterials) _asstatic_mesh_component)))))))))