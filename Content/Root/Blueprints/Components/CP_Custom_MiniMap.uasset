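; Component that shows custom point-of-interest icons on the minimap of the deploy menu's spawn map.
; Initialise stores the menu and scans all actors, creating the widget class specified by each CP_CustomPOI component on the map canvas.
; Tick repositions each icon by projecting its actor's world location into map space, offset by the current map position.
; Icons are bound to actor destruction for cleanup.
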(event Custom|Initialise
  (params (DeployMenu :type WBP%20Deploy%20Menu%20Object%20Reference))
  (Variables|Logic|SetDeployMenu DeployMenu)
  (bind _outactors (Actor|GetAllActorsOfClass "/Script/Engine.Actor"))
  (for _array_element _outactors
    (CallFunction|AddActor _array_element)))

(event EventBeginPlay)

(event EventTick
  (params (DeltaSeconds :type Float%20%28single-precision%29))
  (for _array_element (Variables|Logic|GetPOIActors)
    (CallFunction|UpdateWidget _array_element)))

(fn CreateWidget
  (params (Actor :type Actor%20Object%20Reference))
  (bind _returnvalue (Actor|GetComponentbyClass Actor "/CasualCQB/Root/Blueprints/Components/CP_CustomPOI.CP_CustomPOI_C"))
  (LocalVariables|SetOwner Actor)
  (bind _returnvalue_2 (UserInterface|CreateWidget (Variables|/CasualCQB/Root/Blueprints/Components/CP_CustomPOI.CP_CustomPOI_C|GetWidgetClass _returnvalue)))
  (bind _aswbp_poi_icon_base (Utilities|Casting|CastToWBP_POI_Icon_Base _returnvalue_2)
    (:then
      (Default|AssignOwner _aswbp_poi_icon_base (LocalVariables|GetOwner)))
    (:CastFailed
      _))
  (bind _returnvalue_3 (Widget|Panel|AddChild (Variables|/Script/DonkehFrameworkUI.DFMinimap|GetMapCanvas (Variables|/HDCore/UI/DeployMenu/SpawnMap/WBP_DeployMenu_SpawnMapView.WBP_DeployMenu_SpawnMapView_C|GetMinimap (Variables|/HDCore/UI/DeployMenu/WBP_DeployMenu.WBP_DeployMenu_C|GetSpawnMapView (Variables|Logic|GetDeployMenu)))) _returnvalue_2))
  (bind _ascanvas_panel_slot (Utilities|Casting|CastToCanvasPanelSlot _returnvalue_3))
  (Class|CanvasPanelSlot|SetAlignment _ascanvas_panel_slot "(X=0.500000,Y=0.500000)")
  (Class|CanvasPanelSlot|SetSize _ascanvas_panel_slot "(X=32.000000,Y=32.000000)")
  (Game|BindEventtoOnDestroyed Actor (EventDispatchers|CreateEvent :!event HandleActorDestroy))
  (Variables|/CasualCQB/Root/Blueprints/Components/CP_CustomPOI.CP_CustomPOI_C|SetAssociatedWidget _returnvalue _returnvalue_2)
  (Utilities|Array|Add (Variables|Logic|GetPOIActors) Actor))

(fn HandleActorDestroy
  (params (DestroyedActor :type Actor%20Object%20Reference))
  (Widget|RemovefromParent (Variables|/CasualCQB/Root/Blueprints/Components/CP_CustomPOI.CP_CustomPOI_C|GetAssociatedWidget (Actor|GetComponentbyClass DestroyedActor "/CasualCQB/Root/Blueprints/Components/CP_CustomPOI.CP_CustomPOI_C"))))

(fn UpdateWidget
  (params (Actor :type Actor%20Object%20Reference))
  (bind _deploymenu (Variables|Logic|GetDeployMenu))
  (bind _spawnmapview (Variables|/HDCore/UI/DeployMenu/WBP_DeployMenu.WBP_DeployMenu_C|GetSpawnMapView _deploymenu))
  (bind _minimap (Variables|/HDCore/UI/DeployMenu/SpawnMap/WBP_DeployMenu_SpawnMapView.WBP_DeployMenu_SpawnMapView_C|GetMinimap _spawnmapview))
  (Utilities|IsValid Actor
    (:Is%20Valid
      (Class|Widget|SetRenderTranslation (Variables|/CasualCQB/Root/Blueprints/Components/CP_CustomPOI.CP_CustomPOI_C|GetAssociatedWidget (Actor|GetComponentbyClass Actor "/CasualCQB/Root/Blueprints/Components/CP_CustomPOI.CP_CustomPOI_C")) (.WidgetLocation (Class|DFMinimap|ConvertMapLocationtoLocalWidgetLocation _minimap (+ (* (Variables|/Script/DonkehFrameworkUI.DFMinimap|GetCurrentMapPos _minimap) -1.0) (.MapLocation (Class|DFMinimap|ProjectWorldLocationtoMap _minimap (Transformation|GetWorldLocation (Variables|/Script/Engine.Actor|GetRootComponent Actor)))))))))))

(fn AddActor
  (params (Actor :type Actor%20Object%20Reference))
  (Utilities|IsValid (Variables|Logic|GetDeployMenu)
    (:Is%20Valid
      (if (Utilities|IsValid (Actor|GetComponentbyClass Actor "/CasualCQB/Root/Blueprints/Components/CP_CustomPOI.CP_CustomPOI_C"))
        (CallFunction|CreateWidget Actor)))))