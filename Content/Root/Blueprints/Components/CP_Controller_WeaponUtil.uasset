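; Controller component that remembers the selected fire mode for each weapon class, when the client config enables it.
; Tick polls the controlled character's equipped weapon on cosmetic-capable instances and saves weapon or fire mode changes to a class-keyed map.
; After a reset clears Ready, it waits for a populated, valid inventory, then forces saved modes onto matching weapons before tracking resumes.
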(event Custom|OnReset
  (Variables|Logic|SetbReady false))

(event EventBeginPlay
  (|CallParentFunction))

(event EventTick
  (params (DeltaSeconds :type Float%20%28single-precision%29))
  (|CallParentFunction DeltaSeconds)
  (if (Variables|/CasualCQB/Root/Core/ClientSettings_CQB.ClientSettings_CQB_C|GetbRememberFireMode (CallFunction|GetClientConfig))
    (Networking|CanExecuteCosmeticEvents
      (:True
        (if (Variables|Logic|GetbReady)
          (bind _weapon (Logic|GetEquippedWeapon))
          (Utilities|IsValid _weapon
            (:Is%20Valid
              (if (!= (Variables|Logic|GetLastWeaponClass) (Utilities|GetClass _weapon))
                (Variables|Logic|SetLastWeaponClass (Utilities|GetClass _weapon))
                (Logic|AddMapping _weapon)
                (Variables|Logic|SetLastFireMode (Class|DFBaseGun|GetSelectedFireMode _weapon))
                (elif (!= (Variables|Logic|GetLastFireMode) (Class|DFBaseGun|GetSelectedFireMode _weapon))
                  (Logic|AddMapping _weapon)
                  (Variables|Logic|SetLastFireMode (Class|DFBaseGun|GetSelectedFireMode _weapon))))))
          (else
            (Logic|ApplyMappings)))))))

(fn GetEquippedWeapon
  (bind _character (Logic|GetCharacter))
  (Utilities|IsValid _character
    (:Is%20Valid
      (return (Variables|/HDCore/Core/BP_HDPlayerCharacterBase.BP_HDPlayerCharacterBase_C|GetEquippedWeapon _character)))))

(fn GetCharacter
  (bind _ascontroller (Utilities|Casting|CastToController (Components|GetOwner)))
  (bind _asbp_hdplayer_character_base (Utilities|Casting|CastToBP_HDPlayerCharacterBase (Pawn|GetControlledPawn _ascontroller)))
  (return _asbp_hdplayer_character_base))

(fn AddMapping
  (params (Weapon :type BP%20HD%20Weapon%20Base%20Object%20Reference))
  (Utilities|IsValid Weapon
    (:Is%20Valid
      (Utilities|Map|Add (Variables|Logic|GetFireModeMapping) (Utilities|GetClass Weapon) (Class|DFBaseGun|GetSelectedFireMode Weapon)))))

(fn ApplyMappings
  (bind _character (Logic|GetCharacter))
  (bind _returnvalue (Class|DFBaseCharacter|GetInventory _character))
  (bind _items (Variables|/Script/DonkehFramework.DFInventoryComponent|GetItems _returnvalue))
  (Utilities|IsValid _character
    (:Is%20Valid
      (Utilities|IsValid _returnvalue
        (:Is%20Valid
          (for _array_element _items
            (if (not (Class|DFBlueprintFunctions|IsValidActor _array_element))
              (LocalVariables|SetbAbort true)))
          (if (not (or (== (Utilities|Array|Length _items) 0) (LocalVariables|GetbAbort)))
            (Utilities|FlowControl|Sequence
              (:then_0
                (for _array_element_2 _items
                  (bind _asbp_hdweapon_base (Utilities|Casting|CastToBP_HDWeaponBaseClass (Utilities|GetClass _array_element_2)))
                  (if (.ReturnValue (Utilities|Map|Find (Variables|Logic|GetFireModeMapping) _asbp_hdweapon_base))
                    (bind _asbp_hdweapon_base_2 (Utilities|Casting|CastToBP_HDWeaponBase _array_element_2))
                    (Class|DFBaseGun|SetFireMode _asbp_hdweapon_base_2 (.Value (Utilities|Map|Find (Variables|Logic|GetFireModeMapping) _asbp_hdweapon_base)) false true))))
              (:then_1
                (Variables|Logic|SetbReady true)))))))))