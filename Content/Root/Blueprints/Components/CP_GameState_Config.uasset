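; Game State component that holds match rule settings such as HUD options, revive, spawning, damage and player movement.
; When ready, it caches a loaded CQB client settings object, copies client config values over its own on a non-dedicated authority, then sets Ready.
; WaitFor exposes Ready for the Config check, and server variable changes trigger CallOnServerChange.
; TimeToContinue and EnableDevelopment overrides stay disconnected because the UI cannot edit them.
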(event Custom|OnReady
  (Logic|CacheClientSettings)
  (Logic|LoadClientOverrides)
  (Variables|Logic|SetbReady true))

(event Custom|OnServerVarChange
  (Default|CallOnServerChange))

(event EventBeginPlay)

(event EventTick
  (params (DeltaSeconds :type Float%20%28single-precision%29)))

(fn LoadClientOverrides
  (bind _clientsettings (CallFunction|GetClientConfig))
  (bind _clientsettings_2 (CallFunction|GetClientConfig))
  (if (and (Ability|HasAuthority (Components|GetOwner)) (not (Networking|IsDedicatedServer)))
    (Utilities|FlowControl|Sequence
      (:then_0
        (Variables|ServerVariables|SetEnableEnemyTags (Variables|/CasualCQB/Root/Core/ClientSettings_CQB.ClientSettings_CQB_C|GetbEnableEnemyTags _clientsettings_2))
        (Variables|ServerVariables|SetEnableDeathCamera (Variables|/CasualCQB/Root/Core/ClientSettings_CQB.ClientSettings_CQB_C|GetbEnableDeathCamera _clientsettings_2))
        (Variables|ServerVariables|SetAllowMinimap (Variables|/CasualCQB/Root/Core/ClientSettings_CQB.ClientSettings_CQB_C|GetbAllowMinimap _clientsettings_2))
        (Variables|ServerVariables|SetEnableRedDot (Variables|/CasualCQB/Root/Core/ClientSettings_CQB.ClientSettings_CQB_C|GetbEnableRedDot _clientsettings_2))
        (Variables|ServerVariables|SetEnableSuppressionEffect (Variables|/CasualCQB/Root/Core/ClientSettings_CQB.ClientSettings_CQB_C|GetbEnableSuppressionEffect _clientsettings_2))
        (Variables|ServerVariables|SetEnableSuppressionMovement (Variables|/CasualCQB/Root/Core/ClientSettings_CQB.ClientSettings_CQB_C|GetbEnableSuppressionMovement _clientsettings_2))
        (Variables|ServerVariables|SetAllowSquadSpawn (Variables|/CasualCQB/Root/Core/ClientSettings_CQB.ClientSettings_CQB_C|GetbAllowSquadSpawn _clientsettings_2))
        (Variables|ServerVariables|SetAllowRevive (Variables|/CasualCQB/Root/Core/ClientSettings_CQB.ClientSettings_CQB_C|GetbAllowRevive _clientsettings_2))
        (Variables|ServerVariables|SetbAllowKillFeed (Variables|/CasualCQB/Root/Core/ClientSettings_CQB.ClientSettings_CQB_C|GetbAllowKillFeed _clientsettings_2))
        (Variables|ServerVariables|SetSquadSpawnAdditionalDelay (Variables|/CasualCQB/Root/Core/ClientSettings_CQB.ClientSettings_CQB_C|GetSquadSpawnAdditionalDelay _clientsettings_2))
        (Variables|ServerVariables|SetRadialDamageMultiplier (Variables|/CasualCQB/Root/Core/ClientSettings_CQB.ClientSettings_CQB_C|GetRadialDamageMultiplier _clientsettings_2))
        (Variables|ServerVariables|SetbAllowPlayerTags (Variables|/CasualCQB/Root/Core/ClientSettings_CQB.ClientSettings_CQB_C|GetbAllowPlayerTags _clientsettings_2)))
      (:then_1
        (Variables|ServerVariables|SetbEnableSpawnProtection (Variables|/CasualCQB/Root/Core/ClientSettings_CQB.ClientSettings_CQB_C|GetbEnableSpawnProtection _clientsettings))
        (Variables|ServerVariables|SetMinRespawnDelay (Variables|/CasualCQB/Root/Core/ClientSettings_CQB.ClientSettings_CQB_C|GetMinRespawnDelay _clientsettings))
        (Variables|ServerVariables|SetMinGiveUpDelay (Variables|/CasualCQB/Root/Core/ClientSettings_CQB.ClientSettings_CQB_C|GetMinGiveUpDelay _clientsettings))
        (Variables|ServerVariables|SetPlayerSprintAcceleration (Variables|/CasualCQB/Root/Core/ClientSettings_CQB.ClientSettings_CQB_C|GetPlayerSprintAcceleration _clientsettings))
        (Variables|ServerVariables|SetPlayerSprintStrafingThreashold (Variables|/CasualCQB/Root/Core/ClientSettings_CQB.ClientSettings_CQB_C|GetPlayerSprintStrafingThreashold _clientsettings))
        (Variables|ServerVariables|SetPlayerMaxWalkSpeed (Variables|/CasualCQB/Root/Core/ClientSettings_CQB.ClientSettings_CQB_C|GetPlayerMaxWalkSpeed _clientsettings))
        (Variables|ServerVariables|SetPlayerFallDamageDivisor (Variables|/CasualCQB/Root/Core/ClientSettings_CQB.ClientSettings_CQB_C|GetPlayerFallDamageDivisor _clientsettings))
        (Variables|ServerVariables|SetbNoReviveOnHeadshot (Variables|/CasualCQB/Root/Core/ClientSettings_CQB.ClientSettings_CQB_C|GetbNoReviveOnHeadshot _clientsettings))))))

(fn CacheClientSettings
  (bind _returnvalue (Game|ConstructObjectfromClass "/CasualCQB/Root/Core/ClientSettings_CQB.ClientSettings_CQB_C" (Game|GetGameInstance)))
  (Class|GameUserSettings|LoadSettings _returnvalue false)
  (Variables|Logic|SetCachedClientSettings _returnvalue))

(fn GetClientSettings
  (return (Variables|Logic|GetCachedClientSettings)))

(fn Waitfor
  (params (IsReady :type String))
  (switch string IsReady
    (:Default
      (return false))
    (:Config
      (return (Variables|Logic|GetbReady)))))