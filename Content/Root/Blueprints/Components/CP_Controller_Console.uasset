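; Player controller component that provides a toggleable text console for entering commands and viewing a log.
; Toggling creates or removes the console widget, restoring the stored log text, which persists in the component until cleared.
; Submitted text is split on commas into a command and parameters, then broadcast through an event dispatcher.
; Typing focus is set on release only after a time threshold since the console appeared.
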(event Custom|SetText
  (params (Text :type String))
  (bind _console (Variables|Logic|GetConsole))
  (Utilities|IsValid _console
    (:Is%20Valid
      (Default|SetText _console Text))))

(event Custom|ToggleConsole
  (Utilities|IsValid (Variables|Logic|GetConsole)
    (:Is%20Valid
      (Widget|RemovefromParent (Variables|Logic|GetConsole))
      (Variables|Logic|SetConsole 0))
    (:Is%20Not%20Valid
      (bind _asplayer_controller (Utilities|Casting|CastToPlayerController (Components|GetOwner)))
      (bind _returnvalue (UserInterface|CreateWidget "/CasualCQB/Root/UI/HUD/WBP_Console.WBP_Console_C" _asplayer_controller))
      (bind _output_get (Variables|Logic|SetConsole _returnvalue))
      (EventDispatchers|BindEventtoExecuteCommandText _output_get (delegate Custom|OnExecuteCommandText))
      (EventDispatchers|BindEventtoClearConsole _output_get (delegate Custom|OnClearConsole))
      (UserInterface|Viewport|AddtoViewport _output_get 2)
      (CallFunction|SetText (Variables|Logic|GetLogText))
      (Variables|Logic|SetShownGameTime (Utilities|Time|GetGameTimeinSeconds)))))

(event Custom|AddLogText
  (params (Text :type String) (Prefix :type String))
  (CallFunction|AddLogTextRaw (Utilities|String|ToString(Text) (Utilities|Text|FormatText "{Prefix}: {Text}" Prefix Text))))

(event Custom|Reset
  (bind _output_get (Variables|Logic|SetLogText ""))
  (CallFunction|SetText _output_get))

(event Custom|AddLogTextRaw
  (params (Text :type String))
  (bind _output_get (Variables|Logic|SetLogText (Utilities|String|Append (Variables|Logic|GetLogText) (Utilities|String|Append Text " 
"))))
  (Networking|CanExecuteCosmeticEvents
    (:True
      (CallFunction|SetText _output_get))))

(event Custom|OnExecuteCommandText
  (params (CommandText :type String))
  (bind _returnvalue (Utilities|String|ParseIntoArray CommandText ","))
  (bind _output_get (Variables|Logic|SetLastCommand (Utilities|Array|Get(acopy) _returnvalue)))
  (Variables|Logic|SetTempStringArray _returnvalue)
  (Utilities|Array|RemoveIndex (Variables|Logic|GetTempStringArray)) ; XXX: weird work-around needed for remove to work, no idea why?
  (Default|CallExecuteCommandText _output_get (Variables|Logic|GetTempStringArray)))

(event Custom|OnClearConsole
  (CallFunction|Reset))

(event Custom|OnReleased
  (bind _console (Variables|Logic|GetConsole))
  (if (>= (- (Utilities|Time|GetGameTimeinSeconds) (Variables|Logic|GetShownGameTime)) (Variables|Logic-Config|GetFocusTimeThreashold))
    (Utilities|IsValid _console
      (:Is%20Valid
        (Default|SetTypingFocus _console)))))

(event EventBeginPlay
  (|CallParentFunction))

(event EventTick
  (params (DeltaSeconds :type Float%20%28single-precision%29)))