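; Character component that records a recent safe transform to serve as a spawn point, such as for squad spawning.
; A looping timer, also active on clients, captures a provisional transform while the owner is grounded and not downed, correcting height for crouch and prone.
; It promotes that transform once the owner moves over a metre away or on initialisation.
; GetSpawnSave returns the saved transform while the character lives, ignoring its MinimumDistance input.
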(event Custom|OnUpdate
  (bind (_result _isvalid) (Logic|GetSaveTransform))
  (Utilities|FlowControl|Sequence
    (:then_0
      (if (and _isvalid (not (Variables|Logic|GetbSpawnProvisional)))
        (Variables|Logic|SetSpawnProvisional _result)
        (Variables|Logic|SetbSpawnProvisional true)))
    (:then_1
      (if (or (> (Math|Vector|VectorLength (- (Transformation|GetActorLocation (Components|GetOwner)) (.Location (Math|Transform|BreakTransform (Variables|Logic|GetSpawnProvisional))))) 1e+02) (Variables|Logic|GetbSpawnAlgoInitialise))
        (if (Variables|Logic|GetbSpawnProvisional)
          (Variables|Logic|SetSpawnSave (Variables|Logic|GetSpawnProvisional))
          (Variables|Logic|SetbSpawnSave true)
          (Variables|Logic|SetbSpawnProvisional false)
          (Variables|Logic|SetbSpawnAlgoInitialise false))))))

(event EventBeginPlay
  (|CallParentFunction)
  (if true ; NOTE: we have turned this on for clients\nso we can do squad spawn client UI etc.
    (Utilities|Time|SetTimerbyEvent (delegate Custom|OnUpdate) (Variables|Logic-Config|GetUpdateFrequencySeconds) true)))

(fn GetSpawnSave
  (params (MinimumDistance :type Float%20%28single-precision%29))
  (bind _asdfbase_character (Utilities|Casting|CastToDFBaseCharacter (Components|GetOwner)))
  (if (Math|Boolean|ANDBoolean (Class|DFBaseCharacter|IsAlive _asdfbase_character) (Variables|Logic|GetbSpawnSave) true)
    (return (Variables|Logic|GetSpawnSave) true)))

(fn GetSaveTransform
  (bind _asdfbase_character (Utilities|Casting|CastToDFBaseCharacter (Components|GetOwner)))
  (if (and (not (Logic|IsDownedorDead)) (AI|Components|NavMovement|IsMovingonGround (Variables|/Script/Engine.Character|GetCharacterMovement _asdfbase_character)))
    (bind _result (Logic|ValidateTransform (Components|GetOwner) (Math|Transform|MakeTransform (+ (Math|Vector|SelectVector "0, 0,32.000000" (Math|Vector|SelectVector "0, 0,70.000000" "0, 0, 0" (Variables|/Script/DonkehFramework.DFBaseCharacter|GetbIsProne _asdfbase_character)) (Variables|/Script/Engine.Character|GetbIsCrouched _asdfbase_character)) (.Location (Math|Transform|BreakTransform (Transformation|GetActorTransform _asdfbase_character)))) (.Rotation (Math|Transform|BreakTransform (Transformation|GetActorTransform _asdfbase_character))) (.Scale (Math|Transform|BreakTransform (Transformation|GetActorTransform _asdfbase_character))))))
    (return (Math|Transform|MakeTransform (+ (Math|Vector|SelectVector "0, 0,32.000000" (Math|Vector|SelectVector "0, 0,70.000000" "0, 0, 0" (Variables|/Script/DonkehFramework.DFBaseCharacter|GetbIsProne _asdfbase_character)) (Variables|/Script/Engine.Character|GetbIsCrouched _asdfbase_character)) (.Location (Math|Transform|BreakTransform (Transformation|GetActorTransform _asdfbase_character)))) (.Rotation (Math|Transform|BreakTransform (Transformation|GetActorTransform _asdfbase_character))) (.Scale (Math|Transform|BreakTransform (Transformation|GetActorTransform _asdfbase_character)))) _result)
    (else
      (return "" false))))

(fn IsDownedorDead
  (bind _ragdollcontrol (Class|IFCharacterCQB|GetRagDollControl(Message) (Components|GetOwner)))
  (Utilities|IsValid _ragdollcontrol
    (:Is%20Valid
      (return (Default|IsDownedorDead _ragdollcontrol)))
    (:Is%20Not%20Valid
      (return false))))

(fn ValidateTransform
  (params (Actor :type Actor%20Object%20Reference) (Transform :type Transform))
  (if (Class|KismetMathLibrary|NearlyEqualTransformTransform Transform (Math|Transform|MakeTransform "0, 0, 0") 0.0001 0.0001 0.0001)
    (return false)
    (else
      (return true))))