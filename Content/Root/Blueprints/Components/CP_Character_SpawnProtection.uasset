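; Character component that sets up team spawn protection zones and tracks whether its owning character is in a safe zone.
; On BeginPlay with authority, it spawns a BP_SpawnProtection at each TriggerSphere tagged SpawnProtection, owned by the character and initialised from that sphere.
; BluFor and OpFor tags on each sphere set the zone's team to Blue or Red.
; A ServerSetSafeZone event updates the InSafeZone flag, which IsInSafeZone exposes.
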(event Custom|ServerSetSafeZone
  (params (Active :type Boolean))
  (Logic|SetSafeZone Active))

(event EventBeginPlay
  (Utilities|SwitchHasAuthority
    (:Authority
      (Logic|CreateDynamicSpawnProtection (Components|GetOwner)))))

(event EventTick
  (params (DeltaSeconds :type Float%20%28single-precision%29)))

(fn CreateDynamicSpawnProtection
  (params (CreatedFor :type Actor%20Object%20Reference))
  (bind _outactors (Actor|GetAllActorsOfClasswithTag "/Script/Engine.TriggerSphere" "SpawnProtection"))
  (for _array_element _outactors
    (bind _returnvalue (Game|SpawnActorfromClass "/CasualCQB/Root/Blueprints/BP_SpawnProtection.BP_SpawnProtection_C" (Transformation|GetActorTransform _array_element) "Undefined" CreatedFor 0))
    (if (Actor|ActorHasTag _array_element "BluFor")
      (Variables|/CasualCQB/Root/Blueprints/BP_Interactive_Device.BP_Interactive_Device_C|SetOwning%20Team _returnvalue "Blue"))
    (if (Actor|ActorHasTag _array_element "OpFor")
      (Variables|/CasualCQB/Root/Blueprints/BP_Interactive_Device.BP_Interactive_Device_C|SetOwning%20Team _returnvalue "Red"))
    (Default|Initialise _returnvalue _array_element)))

(fn SetSafeZone
  (params (Active :type Boolean))
  (bind _output_get (Variables|Logic|SetInSafeZone Active))
  (if _output_get
    _))

(fn IsinSafeZone
  (return (Variables|Logic|GetInSafeZone)))