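; Controller component that manages widgets by Z-order and updates registered interactive devices for the owning controller.
; On cosmetic ticks it scores relevant, observable non-always-visible devices by view rotation, showing only the best match and hiding the rest.
; Server events forward lock and unlock requests for a player to the device, and DestroyUI removes all tracked widgets from their parents.
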(event Custom|ServerLockForPlayer
  (params (InteractiveDevice :type BP%20Interactive%20Device%20Object%20Reference) (PlayerId :type Integer) (Action :type String) (Token :type Actor%20Object%20Reference) (PlayerState :type Player%20State%20Object%20Reference))
  (Utilities|IsValid InteractiveDevice
    (:Is%20Valid
      (bind _ascontroller (Utilities|Casting|CastToController (Components|GetOwner)))
      (Default|LockforPlayer InteractiveDevice PlayerId Action _ascontroller Token PlayerState))))

(event Custom|DestroyUI
  (Logic|RemoveDevices))

(event Custom|ServerUnlockForPlayer
  (params (InteractiveDevice :type BP%20Interactive%20Device%20Object%20Reference) (PlayerId :type Integer))
  (Utilities|IsValid InteractiveDevice
    (:Is%20Valid
      (Default|UnlockforPlayer InteractiveDevice PlayerId))))

(event EventBeginPlay
  (|CallParentFunction))

(event EventTick
  (params (DeltaSeconds :type Float%20%28single-precision%29))
  (|CallParentFunction DeltaSeconds)
  (Networking|CanExecuteCosmeticEvents
    (:True
      (Logic|TestDeviceVisibility)
      (Logic|UpdateDevices DeltaSeconds))))

(fn SetWidget
  (params (Zorder :type Integer) (Widget :type Widget%20Object%20Reference))
  (Utilities|IsValid Widget
    (:Is%20Valid
      (Utilities|Map|Add (Variables|Logic|GetCurrentWidgets) Zorder Widget))
    (:Is%20Not%20Valid
      (Utilities|Map|Remove (Variables|Logic|GetCurrentWidgets) Zorder))))

(fn GetWidget
  (params (Zorder :type Integer))
  (bind _currentwidgets (Variables|Logic|GetCurrentWidgets))
  (bind (_value _returnvalue) (Utilities|Map|Find _currentwidgets Zorder))
  (return _value _returnvalue))

(fn HasInteractWidget
  (return (Utilities|Map|Contains (Variables|Logic|GetCurrentWidgets) -1)))

(fn RegisterDevice
  (params (Device :type BP%20Interactive%20Device%20Object%20Reference))
  (Utilities|Array|AddUnique (Variables|Logic|GetAllDevices) Device)
  (if (not (Variables|/CasualCQB/Root/Blueprints/BP_Interactive_Device.BP_Interactive_Device_C|GetAlwaysVisible Device))
    (Utilities|Array|AddUnique (Variables|Logic|GetDynamicDevices) Device)))

(fn UnregisterDevice
  (params (Device :type BP%20Interactive%20Device%20Object%20Reference))
  (Utilities|Array|RemoveItem (Variables|Logic|GetDynamicDevices) Device)
  (Utilities|Array|RemoveItem (Variables|Logic|GetAllDevices) Device))

(fn UpdateDevices
  (params (DeltaSeconds :type Float%20%28single-precision%29))
  (for _array_element (Variables|Logic|GetAllDevices)
    (Default|Update _array_element DeltaSeconds)))

(fn TestDeviceVisibility
  (for _array_element (Variables|Logic|GetDynamicDevices)
    (if (Default|GetIsRelevantto _array_element (Logic|GetController))
      (bind (_result _rotation) (Default|IsObservable _array_element _array_element 0.95 2e+02))
      (if _result
        (Utilities|Map|Add (LocalVariables|GetResults) _array_element _rotation))))
  (bind _values (Utilities|Map|Values (LocalVariables|GetResults)))
  (Utilities|Array|FloatSort _values true)
  (for _array_element_2 (Variables|Logic|GetDynamicDevices)
    (if (.ReturnValue (Utilities|Map|Find (LocalVariables|GetResults) _array_element_2))
      (Default|ShowHide _array_element_2 (and (Math|Float|NearlyEqual(Float) (.Value (Utilities|Map|Find (LocalVariables|GetResults) _array_element_2)) (Utilities|Array|Get(acopy) _values) 1e-06) (LocalVariables|GetNotShown)))
      (LocalVariables|SetNotShown (not (and (Math|Float|NearlyEqual(Float) (.Value (Utilities|Map|Find (LocalVariables|GetResults) _array_element_2)) (Utilities|Array|Get(acopy) _values) 1e-06) (LocalVariables|GetNotShown))))
      (else
        (Default|ShowHide _array_element_2 false)))))

(fn NumDevices
  (return (Utilities|Array|Length (Variables|Logic|GetDynamicDevices))))

(fn RemoveDevices
  (bind _values (Utilities|Map|Values (Variables|Logic|GetCurrentWidgets)))
  (for _array_element _values
    (Utilities|IsValid _array_element
      (:Is%20Valid
        (Widget|RemovefromParent _array_element)))))

(fn GetController
  (bind _ascontroller (Utilities|Casting|CastToController (Components|GetOwner)))
  (return _ascontroller))