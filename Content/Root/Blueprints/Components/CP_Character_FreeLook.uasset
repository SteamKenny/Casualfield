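; Character component that lets a locally controlled player free-look with the camera, turning off aiming, controller-yaw rotation and controller look input while active.
; Look input builds clamped yaw and pitch, but only yaw drives the camera, adding scaled pitch correction and height offset.
; Firing or aiming exits and yaw eases back to centre; being downed, dead or losing local control exits with a reset.
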(event Custom|OnEnterFreeLook
  (bind _character (Variables|Logic|GetCharacter))
  (bind _character_2 (Variables|Logic|GetCharacter))
  (Class|DFBaseCharacter|UnAim _character_2)
  (Variables|/Script/Engine.Pawn|SetbUseControllerRotationYaw _character_2 false)
  (Variables|Logic|SetIsFreeLookActive true)
  (Class|HDPlayerCharacter|SetAllowFreeAim _character false)
  (bind _asdfbase_player_controller (Utilities|Casting|CastToDFBasePlayerController (Pawn|GetController _character)))
  (Variables|/Script/Engine.PlayerController|SetInputYawScale _asdfbase_player_controller 0.0) ; Disable yaw input
  (Variables|/Script/Engine.PlayerController|SetInputPitchScale _asdfbase_player_controller 0.0) ; Disable pitch input
)

(event Custom|OnExitFreeLook
  (params (Reset :type Boolean))
  (bind _character (Variables|Logic|GetCharacter))
  (if Reset
    (CallFunction|Reset))
  (Variables|/Script/Engine.Pawn|SetbUseControllerRotationYaw (Variables|Logic|GetCharacter) true)
  (Variables|/Script/Engine.SpringArmComponent|SetbInheritYaw (Variables|Logic|GetSpringArm) true)
  (Variables|Logic|SetIsFreeLookActive false)
  (Class|HDPlayerCharacter|SetAllowFreeAim _character true)
  (bind _asdfbase_player_controller (Utilities|Casting|CastToDFBasePlayerController (Pawn|GetController _character)))
  (Variables|/Script/Engine.PlayerController|SetInputYawScale _asdfbase_player_controller (Variables|Logic|GetSavedInputYawScale)) ; Restore yaw input
  (Variables|/Script/Engine.PlayerController|SetInputPitchScale _asdfbase_player_controller (Variables|Logic|GetSavedInputPitchScale)) ; Restore pitch input
)

(event Custom|OnPitchInput
  (params (PitchDelta :type Float%20%28single-precision%29))
  (Variables|Logic|SetLatestPitchInput PitchDelta))

(event Custom|OnYawInput
  (params (YawDelta :type Float%20%28single-precision%29))
  (Variables|Logic|SetLatestYawInput YawDelta))

(event Custom|OnInitialise
  (bind _asdfbase_player_controller (Utilities|Casting|CastToDFBasePlayerController (Pawn|GetController (Variables|Logic|GetCharacter))))
  (Variables|Logic|SetSavedInputYawScale (Variables|/Script/Engine.PlayerController|GetInputYawScale _asdfbase_player_controller))
  (Variables|Logic|SetSavedInputPitchScale (Variables|/Script/Engine.PlayerController|GetInputPitchScale _asdfbase_player_controller)))

(event Custom|OnCharacterFirePressed
  (CallFunction|OnExitFreeLook false))

(event EventBeginPlay)

(event EventTick
  (params (DeltaSeconds :type Float%20%28single-precision%29))
  (|CallParentFunction DeltaSeconds)
  (if (Class|DFBlueprintFunctions|IsLocallyPlayerControlled (Variables|Logic|GetCharacter))
    (bind (_exit _reset) (CallFunction|CheckforLookExit))
    (if _exit
      (CallFunction|OnExitFreeLook _reset)
      (else
        (if (Variables|Logic|GetIsFreeLookActive)
          (CallFunction|AnimationWhilstActive DeltaSeconds)
          (else
            (CallFunction|AnimationtoRest DeltaSeconds)))
        (CallFunction|Update)))
    (elif (Variables|Logic|GetIsFreeLookActive)
      (CallFunction|OnExitFreeLook true) ; Take account on unpossess/death
    )))

(fn Initialise
  (params (Movement :type DF%20Character%20Movement%20Component%20Object%20Reference) (SpringArm :type Spring%20Arm%20Component%20Object%20Reference) (Camera :type Camera%20Component%20Object%20Reference) (Character :type HD%20Player%20Character%20Object%20Reference))
  (Variables|Logic|SetMovement Movement)
  (Variables|Logic|SetSpringArm SpringArm)
  (Variables|Logic|SetCamera Camera)
  (Variables|Logic|SetCharacter Character)
  (CallFunction|OnInitialise))

(fn CheckforLookExit
  (bind _ragdollcontrol (Class|IFCharacterCQB|GetRagDollControl(Message) (Variables|Logic|GetCharacter)))
  (Utilities|IsValid _ragdollcontrol
    (:Is%20Valid
      (if (Default|IsDownedorDead _ragdollcontrol)
        (return true true)
        (else
          _)))
    (:Is%20Not%20Valid
      _))
  (return (and (Variables|Logic|GetIsFreeLookActive) (Math|Boolean|ORBoolean (Class|DFBaseCharacter|IsPrefiring (Variables|Logic|GetCharacter)) (Class|DFBaseCharacter|IsFiring (Variables|Logic|GetCharacter)) (Class|DFCharacterMovementComponent|IsAiming (Variables|Logic|GetMovement)))) false))

(fn AnimationtoRest
  (params (DeltaSeconds :type Float%20%28single-precision%29))
  (Variables|Logic|SetFreeLookYaw (Math|Float|Lerp (Variables|Logic|GetFreeLookYaw) 0.0 (* DeltaSeconds (Variables|Logic-Config|GetRestSpeedT))))
  (CallFunction|CalculateFreeLookYawT))

(fn AnimationWhilstActive
  (params (DeltaSeconds :type Float%20%28single-precision%29))
  (bind _maxyawangle (Variables|Logic-Config|GetMaxYawAngle))
  (bind _maxpitchangle (Variables|Logic-Config|GetMaxPitchAngle))
  (Variables|Logic|SetFreeLookYaw (Math|Float|ClampAngle (+ (Variables|Logic|GetFreeLookYaw) (* (Variables|Logic-Config|GetFreeLookSpeedT) (Variables|Logic|GetLatestYawInput))) (* _maxyawangle -1.0) _maxyawangle))
  (CallFunction|CalculateFreeLookYawT)
  (Variables|Logic|SetFreeLookPitch (Math|Float|ClampAngle (+ (Variables|Logic|GetFreeLookPitch) (* (Variables|Logic-Config|GetFreeLookSpeedT) (Variables|Logic|GetLatestPitchInput))) (* _maxpitchangle -1.0) _maxpitchangle)))

(fn Update
  (Utilities|FlowControl|Sequence
    (:then_0
      (Transformation|AddLocalRotation (Variables|Logic|GetCamera) (Math|Rotator|MakeRotator 0.0 (CallFunction|CalculatePitchCorrectionT) 0.0) false false) ; Apply pitch 1st
      (Transformation|AddLocalRotation (Variables|Logic|GetCamera) (Math|Rotator|MakeRotator 0.0 0.0 (Variables|Logic|GetFreeLookYaw)) false false) ; Apply yaw 2nd
    )
    (:then_1
      (Transformation|AddLocalOffset (Variables|Logic|GetCamera) (Math|Vector|MakeVector 0.0 0.0 (* (Variables|Logic|GetFreeLookYawT) (Variables|Logic-Config|GetMaxZAdjust))) false false))))

(fn CalculatePitchCorrectionT
  (bind _springarm (Variables|Logic|GetSpringArm))
  (bind _returnvalue (Class|SpringArmComponent|GetTargetRotation _springarm))
  (bind _pitch (Math|Rotator|BreakRotator _returnvalue))
  (return (* (Math|Float|SelectFloat (- 3.6e+02 _pitch) (* _pitch -1.0) (>= _pitch 1.8e+02)) (Variables|Logic|GetFreeLookYawT) (Variables|Logic-Config|GetPitchCorrectionMaxT))))

(fn CalculateFreeLookYawT
  (Variables|Logic|SetFreeLookYawT (Math|Float|Clamp(Float) (/ (Math|Float|Absolute(Float) (Variables|Logic|GetFreeLookYaw)) (Variables|Logic-Config|GetMaxYawAngle)))))

(fn Reset
  (Variables|Logic|SetFreeLookYaw 0.0)
  (Variables|Logic|SetFreeLookPitch 0.0)
  (Variables|Logic|SetIsFreeLookActive false)
  (Variables|Logic|SetFreeLookYawT 0.0)
  (Variables|Logic|SetLatestYawInput 0.0)
  (Variables|Logic|SetLatestPitchInput 0.0))