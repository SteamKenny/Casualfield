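; Character component that applies server-configured movement tuning to a character and its movement component.
; Initialise stores both references, binds to the server config's change event, then copies in sprint acceleration, sprint strafing threshold, max walk speed and fall damage divisor.
; Each server config change re-runs the same assignments, keeping the values in sync without using Tick.
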(event Custom|Initialise
  (params (Movement :type DF%20Character%20Movement%20Component%20Object%20Reference) (Character :type BP%20HD%20Player%20Character%20Base%20Object%20Reference))
  (bind _config (CallFunction|GetServerConfig))
  (Variables|Logic|SetMovement Movement)
  ;[1 1 1] Config change handling
  (Variables|Logic|SetCharacter Character)
  (EventDispatchers|BindEventtoOnServerChange _config (delegate Custom|OnServerChange))
  (Variables|/Script/DonkehFramework.DFCharacterMovementComponent|SetSprintAccelerationMultiplier (Variables|Logic|GetMovement) (Variables|/CasualCQB/Root/Blueprints/Components/CP_GameState_Config.CP_GameState_Config_C|GetPlayerSprintAcceleration _config))
  (Variables|/Script/DonkehFramework.DFCharacterMovementComponent|SetSprintStrafingThreshold (Variables|Logic|GetMovement) (Variables|/CasualCQB/Root/Blueprints/Components/CP_GameState_Config.CP_GameState_Config_C|GetPlayerSprintStrafingThreashold _config))
  (Variables|/Script/Engine.CharacterMovementComponent|SetMaxWalkSpeed (Variables|Logic|GetMovement) (Variables|/CasualCQB/Root/Blueprints/Components/CP_GameState_Config.CP_GameState_Config_C|GetPlayerMaxWalkSpeed _config))
  (Variables|/HDCore/Core/BP_HDPlayerCharacterBase.BP_HDPlayerCharacterBase_C|SetFallDamageDivisor (Variables|Logic|GetCharacter) (Variables|/CasualCQB/Root/Blueprints/Components/CP_GameState_Config.CP_GameState_Config_C|GetPlayerFallDamageDivisor _config)))

(event Custom|OnServerChange
  (bind _config (CallFunction|GetServerConfig))
  (bind _movement (Variables|Logic|GetMovement))
  ;[1 1 1] Config change handling
  (Variables|/Script/DonkehFramework.DFCharacterMovementComponent|SetSprintAccelerationMultiplier _movement (Variables|/CasualCQB/Root/Blueprints/Components/CP_GameState_Config.CP_GameState_Config_C|GetPlayerSprintAcceleration _config))
  (Variables|/Script/DonkehFramework.DFCharacterMovementComponent|SetSprintStrafingThreshold _movement (Variables|/CasualCQB/Root/Blueprints/Components/CP_GameState_Config.CP_GameState_Config_C|GetPlayerSprintStrafingThreashold _config))
  (Variables|/Script/Engine.CharacterMovementComponent|SetMaxWalkSpeed _movement (Variables|/CasualCQB/Root/Blueprints/Components/CP_GameState_Config.CP_GameState_Config_C|GetPlayerMaxWalkSpeed _config))
  (Variables|/HDCore/Core/BP_HDPlayerCharacterBase.BP_HDPlayerCharacterBase_C|SetFallDamageDivisor (Variables|Logic|GetCharacter) (Variables|/CasualCQB/Root/Blueprints/Components/CP_GameState_Config.CP_GameState_Config_C|GetPlayerFallDamageDivisor _config)))

(event EventBeginPlay
  (|CallParentFunction))

(event EventTick
  (params (DeltaSeconds :type Float%20%28single-precision%29)))