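; Game rules component that auto-generates spawn protection zones and a level bounds volume when its owner begins play.
; Unless tagged protection spheres already exist, it spawns TriggerSpheres at active, non-recapturable capture points, tagged OpFor or BluFor by starting team.
; It also spawns a LevelBounds-tagged TriggerBox from the world settings' minimap boundary and KillZ, slightly expanded.
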(event Custom|OnOwnerBeginPlay
  (CallFunction|AutoCreateSpawnProtectionNodes)
  (CallFunction|AutoCreateLevelBoundVolume))

(event EventTick
  (params (DeltaSeconds :type Float%20%28single-precision%29)))

(fn AutoCreateSpawnProtectionNodes
  ;[1 1 1] Do not execute if manually placed spawn protection nodes appear in the world
  (bind _outactors (Actor|GetAllActorsOfClasswithTag "/Script/Engine.TriggerSphere" "SpawnProtection"))
  (if (== (Utilities|Array|Length _outactors) 0)
    (bind _outactors_2 (Actor|GetAllActorsOfClass "/HDCore/Placeables/BP_HDCapturePointBase.BP_HDCapturePointBase_C"))
    (for _array_element _outactors_2
      (if (and (Variables|/Script/HDMain.HDBaseCapturePoint|GetbActive _array_element) (not (Variables|/Script/HDMain.HDBaseCapturePoint|GetbRecapturable _array_element)))
        (bind _returnvalue (Game|SpawnActorfromClass "/Script/Engine.TriggerSphere" (Transformation|GetWorldTransform (Variables|/Script/HDMain.HDBaseCapturePoint|GetSphereCollision _array_element)) "Undefined" 0 0))
        (Utilities|Array|Add (Variables|/Script/Engine.Actor|GetTags _returnvalue) "SpawnProtection")
        (switch Utilities|FlowControl|Switch|SwitchonEHDTeam (Variables|/Script/HDMain.HDBaseCapturePoint|GetStartingTeam _array_element)
          (:Red
            (Utilities|Array|Add (Variables|/Script/Engine.Actor|GetTags _returnvalue) "OpFor"))
          (:Blue
            (Utilities|Array|Add (Variables|/Script/Engine.Actor|GetTags _returnvalue) "BluFor")))
        (bind _assphere_collision (Utilities|Casting|CastToSphereComponent (Variables|/Script/Engine.TriggerBase|GetCollisionComponent _returnvalue)))
        (Components|Sphere|SetSphereRadius _assphere_collision (Variables|Logic|GetAutoSpawnRadius) true)))))

(fn AutoCreateLevelBoundVolume
  (bind _astbworld_settings (Utilities|Casting|CastToTBWorldSettings (Class|DFBlueprintFunctions|GetWorldSettings)))
  (bind _returnvalue (Game|SpawnActorfromClass "/Script/Engine.TriggerBox" (Math|Conversions|ToTransform(Vector) (.BoundaryMidPointLoc (Utilities|Struct|BreakMinimapGenerationSettings (Variables|/Script/Tinkerbox.TBWorldSettings|GetMinimapSettings _astbworld_settings)))) "Undefined" 0 0))
  (Utilities|Array|Add (Variables|/Script/Engine.Actor|GetTags _returnvalue) "LevelBounds")
  (bind _asbox_collision (Utilities|Casting|CastToBoxComponent (Variables|/Script/Engine.TriggerBase|GetCollisionComponent _returnvalue)))
  (Components|Box|SetBoxExtent _asbox_collision (+ (Math|Vector|MakeVector (/ (.PlayableBoundaryLength (Utilities|Struct|BreakMinimapGenerationSettings (Variables|/Script/Tinkerbox.TBWorldSettings|GetMinimapSettings _astbworld_settings))) 2.0) (/ (.PlayableBoundaryLength (Utilities|Struct|BreakMinimapGenerationSettings (Variables|/Script/Tinkerbox.TBWorldSettings|GetMinimapSettings _astbworld_settings))) 2.0) (Math|Float|Absolute(Float) (Variables|/Script/Engine.WorldSettings|GetKillZ (Class|DFBlueprintFunctions|GetWorldSettings)))) (Variables|Logic-Config|GetExpandAmount)) true))