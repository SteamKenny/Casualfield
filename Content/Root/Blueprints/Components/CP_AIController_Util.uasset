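; AI controller utility component that suspends a GOAP-driven AI and manages its voice while downed.
; Idle swaps in a basic idle behaviour state and disables sight, while Freeze stops the GOAP component's tick; both share one IsIdle flag.
; UnFreeze restores ticking and clears any valid enemy.
; A downed or silent voice profile temporarily replaces the current one, with Tick replaying death vocals at random intervals until reverted.
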(event EventBeginPlay
  (|CallParentFunction))

(event EventTick
  (params (DeltaSeconds :type Float%20%28single-precision%29))
  (|CallParentFunction DeltaSeconds)
  (Logic|UpdateVoice DeltaSeconds))

(fn Initialise
  (params (GOAPComp :type HDGOAP%20Component%20Object%20Reference) (PerceptionComp :type AI%20Perception%20Component%20Object%20Reference))
  (Variables|Logic|SetGOAPComp GOAPComp)
  (Variables|Logic|SetPerceptionComp PerceptionComp))

(fn EnterIdle
  (bind _goapcomp (Variables|Logic|GetGOAPComp))
  (bind _behaviorhandler (Variables|/Script/HDMain.HDGOAPComponent|GetBehaviorHandler _goapcomp))
  (if (not (Variables|Logic|GetbIsIdle))
    (bind _returnvalue (Game|ConstructObjectfromClass "/Script/HDMain.HDAIBehState_BasicAASIdle" self))
    (Variables|Logic|SetSavedAIBehaviour (Variables|/Script/HDMain.HDAIBehaviorHandler|GetCurrentBehaviorState _behaviorhandler))
    (Variables|/Script/HDMain.HDAIBehaviorHandler|SetCurrentBehaviorState _behaviorhandler _returnvalue)
    (Class|AIPerceptionComponent|SetSenseEnabled (Variables|Logic|GetPerceptionComp) "/Script/AIModule.AISense_Sight" false)
    (Variables|Logic|SetbIsIdle true)))

(fn ExitIdle
  (if (Variables|Logic|GetbIsIdle)
    (Variables|/Script/HDMain.HDAIBehaviorHandler|SetCurrentBehaviorState (Variables|/Script/HDMain.HDGOAPComponent|GetBehaviorHandler (Variables|Logic|GetGOAPComp)) (Variables|Logic|GetSavedAIBehaviour))
    (Class|AIPerceptionComponent|SetSenseEnabled (Variables|Logic|GetPerceptionComp) "/Script/AIModule.AISense_Sight" true)
    (Variables|Logic|SetSavedAIBehaviour 0)
    (Variables|Logic|SetbIsIdle false)))

(fn UseVoiceProfile
  (bind _goapcomp (Variables|Logic|GetGOAPComp))
  (bind _vocalhandler (Variables|/Script/HDMain.HDGOAPComponent|GetVocalHandler _goapcomp))
  (if (not (Variables|Logic|GetbIsUsingDownedVoiceProfile))
    (Variables|Logic|SetbIsUsingDownedVoiceProfile true)
    (Variables|Logic|SetSavedAIVoiceProfile (Variables|/Script/HDMain.HDAIVocalHandler|GetCurrentProfile _vocalhandler))
    (Variables|/Script/HDMain.HDAIVocalHandler|SetCurrentProfile _vocalhandler (select (Variables|Logic|GetbPlayDownedVocals) (Variables|Logic|GetDownedAIVoiceProfile) (Variables|Logic|GetSilentAIVoiceProfile)))
    (Logic|ResetVoice)))

(fn RevertVoiceProfile
  (if (Variables|Logic|GetbIsUsingDownedVoiceProfile)
    (Variables|Logic|SetbIsUsingDownedVoiceProfile false)
    (Variables|/Script/HDMain.HDAIVocalHandler|SetCurrentProfile (Variables|/Script/HDMain.HDGOAPComponent|GetVocalHandler (Variables|Logic|GetGOAPComp)) (Variables|Logic|GetSavedAIVoiceProfile))
    (Variables|Logic|SetSavedAIVoiceProfile "")
    (Variables|Logic|SetElapsed 0.0)
    (Variables|Logic|SetPlayAgainAt 0.0)))

(fn UpdateVoice
  (params (DeltaSeconds :type Float%20%28single-precision%29))
  (if (Variables|Logic|GetbIsUsingDownedVoiceProfile)
    (bind _output_get (Variables|Logic|SetElapsed (+ (Variables|Logic|GetElapsed) DeltaSeconds)))
    (if (>= _output_get (Variables|Logic|GetPlayAgainAt))
      (Class|HDAIVocalHandler|PlayVocalSound (Variables|/Script/HDMain.HDGOAPComponent|GetVocalHandler (Variables|Logic|GetGOAPComp)) "Death")
      (Logic|ResetVoice))))

(fn PlayDeathVocal
  (Class|HDAIVocalHandler|PlayVocalSound (Variables|/Script/HDMain.HDGOAPComponent|GetVocalHandler (Variables|Logic|GetGOAPComp)) "Death"))

(fn ResetVoice
  (Variables|Logic|SetPlayAgainAt (Math|Random|RandomFloatinRange (Variables|Logic|GetMinDeathFreq) (Variables|Logic|GetMaxDeathFreq)))
  (Variables|Logic|SetElapsed 0.0))

(fn Freeze
  (if (not (Variables|Logic|GetbIsIdle))
    (Components|Tick|SetComponentTickEnabled (Variables|Logic|GetGOAPComp) false) ; Basically just freezes the AI system
    (Variables|Logic|SetbIsIdle true)))

(fn UnFreeze
  (bind _goapcomp (Variables|Logic|GetGOAPComp))
  (bind _combathandler (Variables|/Script/HDMain.HDGOAPComponent|GetCombatHandler _goapcomp))
  (if (Variables|Logic|GetbIsIdle)
    (Components|Tick|SetComponentTickEnabled _goapcomp true) ; Unfreezes the AI system
    (if (Class|HDAICombatHandler|HasValidEnemy _combathandler false)
      (Class|HDAICombatHandler|SetEnemy _combathandler) ; Clear any notion of an enemy we had when entering idle
    )
    (Variables|Logic|SetbIsIdle false)))