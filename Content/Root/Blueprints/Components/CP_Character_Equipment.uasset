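; Character component that manages client-side weapon switching for human players and keeps the equipment selection HUD in sync with the loadout.
; HUD selection sets a requested item, which a looping timer re-equips until the swap completes.
; Fire and reload presses made mid-swap are buffered, then replayed by timer, with time limits on item-specific requests.
; As a hack, another timer validates HUD slots against loadout and inventory, requesting refreshes on mismatch.
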(event Custom|OnCheckEquipStatus
  (if (Variables|/CasualCQB/Root/Core/ClientSettings_CQB.ClientSettings_CQB_C|GetbEnableEquipmentLogic (CallFunction|GetClientConfig))
    (Utilities|IsValid (Variables|Logic|GetRequestedEquipItem)
      (:Is%20Valid
        (if (Logic|CheckItemIsStillValid (Variables|Logic|GetRequestedEquipItem))
          (if (and (not (Logic|RequestedEquipmentIsSet)) (not (Logic|EquipmentIsChanging)))
            (Class|DFBaseCharacter|EquipItem (Variables|Logic|GetOwnerCharacter) (Variables|Logic|GetRequestedEquipItem)))
          (else
            (Variables|Logic|SetRequestedEquipItem 0)))))))

(event Custom|OnEquippedItemChanged
  (params (Character :type DF%20Base%20Character%20Object%20Reference) (NewEquippedItem :type DF%20Base%20Item%20Object%20Reference) (PrevEquippedItem :type DF%20Base%20Item%20Object%20Reference))
  (Variables|Logic|SetChangedToEquipItem NewEquippedItem)
  (Variables|Logic|SetPreviousEquipItem PrevEquippedItem))

(event Custom|OnLoadoutChanged
  (Variables|Logic|SetPendingFireItem 0)
  (Variables|Logic|SetChangedToEquipItem 0)
  (Variables|Logic|SetRequestedEquipItem 0)
  (Variables|Logic|SetPreviousEquipItem 0)
  (CallFunction|CurrentLoadoutChanged))

(event Custom|OnCharacterFireReleased
  (Variables|Logic|SetPendingFireButton false))

(event Custom|OnCharacterReloadReleased)

(event Custom|OnCharacterFirePressed
  (bind _result (Logic|RequestedEquipmentIsSet))
  (bind _character (Logic|GetOwnerCharacter))
  (bind _requestedequipitem (Variables|Logic|GetRequestedEquipItem))
  (bind _returnvalue (Class|DFBaseCharacter|GetEquippedItem _character))
  (if (Variables|/CasualCQB/Root/Core/ClientSettings_CQB.ClientSettings_CQB_C|GetbEnableEquipmentLogic (CallFunction|GetClientConfig))
    (Utilities|FlowControl|Sequence
      (:then_0
        (if (or (not _result) (and _result (not (Logic|ChangedtoWeaponCanFire))))
          (Utilities|IsValid _requestedequipitem
            (:Is%20Valid
              (Variables|Logic|SetPendingFireItem _requestedequipitem)
              (Variables|Logic|SetPendingFireTimeStamp (Utilities|Time|GetGameTimeinSeconds))
              (Development|PrintString "PENDING EQU")))))
      (:then_1
        (Utilities|IsValid _returnvalue
          (:Is%20Valid
            (if (not (Class|DFBaseItem|CanFire _returnvalue))
              (Variables|Logic|SetPendingFireButton true)
              (Development|PrintString "PENDING NOR"))))))))

(event Custom|OnCheckPendingFireReload
  (bind _character (Logic|GetOwnerCharacter))
  (bind _returnvalue (Class|DFBaseCharacter|GetEquippedItem _character))
  (if (Variables|/CasualCQB/Root/Core/ClientSettings_CQB.ClientSettings_CQB_C|GetbEnableEquipmentLogic (CallFunction|GetClientConfig))
    (Utilities|FlowControl|Sequence
      (:then_0
        (if (Math|Boolean|ANDBoolean (Logic|RequestedEquipmentIsSet) (Logic|ChangedtoWeaponCanFire) (Logic|CheckPendingTimeIsStillValid))
          (Utilities|IsValid (Variables|Logic|GetPendingFireItem)
            (:Is%20Valid
              (if (== (Variables|Logic|GetChangedToEquipItem) (Variables|Logic|GetPendingFireItem))
                (Logic|FireCurrentItemOneShot))
              (Variables|Logic|SetPendingFireItem 0)))))
      (:then_1
        (Utilities|IsValid _returnvalue
          (:Is%20Valid
            (if (and (Class|DFBaseItem|CanFire _returnvalue) (Variables|Logic|GetPendingFireButton))
              (Logic|FireCurrentItem)
              (Variables|Logic|SetPendingFireButton false)))))
      (:then_2
        (if (and (Logic|RequestedEquipmentIsSet) (Logic|CheckPendingTimeIsStillValidReload))
          (Utilities|IsValid (Variables|Logic|GetPendingReloadItem)
            (:Is%20Valid
              (if (== (Variables|Logic|GetChangedToEquipItem) (Variables|Logic|GetPendingReloadItem))
                (Class|DFBaseCharacter|Reload (Variables|Logic|GetOwnerCharacter)))
              (Variables|Logic|SetPendingReloadItem 0))))))))

(event Custom|OnCharacterReloadPressed
  (bind _requestedequipitem (Variables|Logic|GetRequestedEquipItem))
  (if (and (not (Logic|RequestedEquipmentIsSet)) (Variables|/CasualCQB/Root/Core/ClientSettings_CQB.ClientSettings_CQB_C|GetbEnableEquipmentLogic (CallFunction|GetClientConfig)))
    (Utilities|IsValid _requestedequipitem
      (:Is%20Valid
        (Variables|Logic|SetPendingReloadItem _requestedequipitem)
        (Variables|Logic|SetPendingReloadTimeStamp (Utilities|Time|GetGameTimeinSeconds))
        (Development|PrintString "PENDING RELOAD")))
    (else
      (Class|DFBaseCharacter|Reload (Logic|GetOwnerCharacter)))))

(event EventBeginPlay
  (|CallParentFunction)
  (bind _asdfbase_player_character (Utilities|Casting|CastToDFBasePlayerCharacter (Components|GetOwner)))
  (Variables|Logic|SetOwnerCharacter _asdfbase_player_character)
  (if (not (Pawn|IsBotControlled _asdfbase_player_character))
    (Networking|CanExecuteCosmeticEvents
      (:True
        (Utilities|Time|SetTimerbyEvent (delegate Custom|OnCheckEquipStatus) (Variables|Logic-Config|GetTimerInterval) true)
        (EventDispatchers|BindEventtoOnEquippedItemChanged (Variables|Logic|GetOwnerCharacter) (delegate Custom|OnEquippedItemChanged))
        (Utilities|Time|SetTimerbyEvent (delegate Custom|OnCheckPendingFireReload) (Variables|Logic-Config|GetTimerInterval) true)))))

(event Custom|OnCheckState
  ;[1 1 1] Update Equipment Items for owning client
  (bind _result (Logic|ValidateEquipment (Variables|/Script/HDMain.HDPlayerCharacter|GetCurrentLoadout (Logic|GetOwnerCharacter)) (Class|DFBaseCharacter|GetInventory (Variables|Logic|GetOwnerCharacter))))
  (if (not _result)
    (Utilities|Time|ClearandInvalidateTimerbyHandle (stale Custom|CurrentLoadoutChanged _returnvalue))
    (CallFunction|CurrentLoadoutChanged)))

(event Custom|CurrentLoadoutChanged
  (bind _equipmentcheckintervalseconds (Variables|Logic-Config|GetEquipmentCheckIntervalSeconds))
  ;[1 1 1] Update Equipment Items for owning client
  (Utilities|Time|ClearandInvalidateTimerbyHandle (stale _returnvalue))
  (if (Class|DFBlueprintFunctions|IsLocallyPlayerControlled (Variables|Logic|GetOwnerCharacter))
    (Class|DFBlueprintFunctions|PrintStringtoLog "Current Loadout Changed" "VeryVerbose")
    (if (Class|DFBaseCharacter|IsAlive (Variables|Logic|GetOwnerCharacter))
      (Class|DFBlueprintFunctions|PrintStringtoLog "IsAlive returned True, proceeding to update Equipment Items..." "VeryVerbose")
      (Default|CallOnRequestUpdateEquipmentItems)
      (bind _returnvalue (Utilities|Time|SetTimerbyEvent (delegate Custom|OnCheckState) _equipmentcheckintervalseconds true _equipmentcheckintervalseconds))
      (else
        (Class|DFBlueprintFunctions|PrintStringtoLog "IsAlive returned False, no Equipment Items will be updated from the current loadout" "VeryVerbose")))))

(fn EquipSelectedItemfromInventory
  (params (SwitchFireModeForSelected :type Boolean))
  (bind _ashdplayer_controller (Utilities|Casting|CastToHDPlayerController (Pawn|GetController (Variables|Logic|GetOwnerCharacter))))
  (bind _asbp_hdhudbase (Utilities|Casting|CastToBP_HDHUDBase (HUD|GetHUD _ashdplayer_controller)))
  (if (.bFoundItem (Default|EquipmentGetSelectedItem _asbp_hdhudbase))
    (Utilities|IsValid (.OutItemToEquip (Default|EquipmentGetSelectedItem _asbp_hdhudbase))
      (:Is%20Valid
        (if (Utilities|IsValid (Class|DFBaseCharacter|GetEquippedItem (Variables|Logic|GetOwnerCharacter)))
          (if (!= (Class|DFBaseCharacter|GetEquippedItem (Variables|Logic|GetOwnerCharacter)) (.OutItemToEquip (Default|EquipmentGetSelectedItem _asbp_hdhudbase)))
            (if (Class|HDBaseWeapon|IsSelectableEquipment (.OutItemToEquip (Default|EquipmentGetSelectedItem _asbp_hdhudbase)))
              (Class|DFBaseCharacter|EquipItem (Variables|Logic|GetOwnerCharacter) (.OutItemToEquip (Default|EquipmentGetSelectedItem _asbp_hdhudbase)))
              (Default|ToggleEquipmentUI _asbp_hdhudbase false)
              (Variables|Logic|SetRequestedEquipItem (.OutItemToEquip (Default|EquipmentGetSelectedItem _asbp_hdhudbase))))
            (else
              ;[0.01636 0.9103 1] Switch Firing Mode if item to select is already selected and that we are allowed to by the caller
              (if SwitchFireModeForSelected
                (Class|DFBasePlayerCharacter|SwitchFireMode (Variables|Logic|GetOwnerCharacter)))))))
      (:Is%20Not%20Valid
        (Class|DFBlueprintFunctions|PrintStringtoLog "Equipment SelectedItem is not valid!" "Warning" true)))
    (else
      (Class|DFBlueprintFunctions|PrintStringtoLog "Equipment Item not found!" "Warning" true))))

(fn EquipmentIsChanging
  (bind _changedtoequipitem (Variables|Logic|GetChangedToEquipItem))
  (bind _requestedequipitem (Variables|Logic|GetRequestedEquipItem))
  (bind _previousequipitem (Variables|Logic|GetPreviousEquipItem))
  (Utilities|IsValid _changedtoequipitem
    (:Is%20Valid
      (if (Logic|ItemIsinFlux _changedtoequipitem)
        _
        (else
          (Utilities|IsValid _previousequipitem
            (:Is%20Valid
              (if (Logic|ItemIsinFlux _previousequipitem)
                _
                (else
                  (Utilities|IsValid _requestedequipitem
                    (:Is%20Valid
                      (if (Logic|ItemIsinFlux _requestedequipitem)
                        _
                        (else
                          (return false)))))))))))
      (return true))))

(fn RequestedEquipmentIsSet
  (Utilities|IsValid (Variables|Logic|GetChangedToEquipItem)
    (:Is%20Valid
      (Utilities|IsValid (Variables|Logic|GetRequestedEquipItem)
        (:Is%20Valid
          (return (and (== (Variables|Logic|GetChangedToEquipItem) (Variables|Logic|GetRequestedEquipItem)) (not (Logic|ItemIsinFlux (Variables|Logic|GetChangedToEquipItem))))))
        (:Is%20Not%20Valid
          _)))
    (:Is%20Not%20Valid
      _))
  (return true) ; We can treat this state as "set"
)

(fn ItemIsinFlux
  (params (Item :type DF%20Base%20Item%20Object%20Reference))
  (Utilities|IsValid Item
    (:Is%20Valid
      (return (or (Class|DFBaseItem|IsEquipping Item) (Class|DFBaseItem|IsUnEquipping Item))))))

(fn ChangedtoWeaponCanFire
  (bind _changedtoequipitem (Variables|Logic|GetChangedToEquipItem))
  (Utilities|IsValid _changedtoequipitem
    (:Is%20Valid
      (return (Class|DFBaseItem|CanFire _changedtoequipitem)))))

(fn FireCurrentItem
  (switch Utilities|FlowControl|Switch|SwitchonEItemType (Class|DFBaseItem|GetItemType (Class|DFBaseCharacter|GetEquippedItem (Logic|GetOwnerCharacter)))
    (:Pistol
      _)
    (:Rifle
      _))
  (Class|DFBasePlayerCharacter|OnFirePressed (Variables|Logic|GetOwnerCharacter)))

(fn FireCurrentItemOneShot
  (bind _ownercharacter (Variables|Logic|GetOwnerCharacter))
  (switch Utilities|FlowControl|Switch|SwitchonEItemType (Class|DFBaseItem|GetItemType (Variables|Logic|GetChangedToEquipItem))
    (:Throwable
      _)
    (:Equipment
      _))
  (Class|DFBasePlayerCharacter|OnFirePressed _ownercharacter)
  (Class|DFBasePlayerCharacter|OnFireReleased _ownercharacter))

(fn CheckItemIsStillValid
  (params (Item :type DF%20Base%20Item%20Object%20Reference))
  (bind _ashdbase_weapon (Utilities|Casting|CastToHDBaseWeapon Item)
    (:then
      (return (Class|HDBaseWeapon|IsSelectableEquipment _ashdbase_weapon)))
    (:CastFailed
      (return true))))

(fn CheckPendingTimeIsStillValidReload
  (Utilities|IsValid (Variables|Logic|GetPendingReloadItem)
    (:Is%20Valid
      (if (<= (- (Utilities|Time|GetGameTimeinSeconds) (Variables|Logic|GetPendingReloadTimeStamp)) (Variables|Logic-Config|GetPendingReloadThreashold))
        (return true)
        (else
          _)))
    (:Is%20Not%20Valid
      _))
  (return false))

(fn CheckPendingTimeIsStillValid
  (Utilities|IsValid (Variables|Logic|GetPendingFireItem)
    (:Is%20Valid
      (if (<= (- (Utilities|Time|GetGameTimeinSeconds) (Variables|Logic|GetPendingFireTimeStamp)) (Variables|Logic-Config|GetPendingFireThreashold))
        (return true)
        (else
          _)))
    (:Is%20Not%20Valid
      _))
  (return false))

(fn ValidateEquipment
  (params (Loadout :type HD%20Kit%20Object%20Reference) (Inventory :type DF%20Inventory%20Component%20Object%20Reference))
  (Utilities|IsValid Loadout
    (:Is%20Valid
      (Utilities|FlowControl|Sequence
        (:then_0
          (bind _childwidget (Utilities|ForEachChildWidget (Variables|/HDCore/UI/HUD/EquipmentSelect/WBP_HUDElement_EquipmentSelect.WBP_HUDElement_EquipmentSelect_C|GetSlotVBox (Variables|/HDCore/UI/HUD/WBP_HUD.WBP_HUD_C|GetEquipmentSelect (Variables|/HDCore/Core/BP_HDHUDBase.BP_HDHUDBase_C|GetHUDContainerUW (CallFunction|GetHDHUDBP)))))
            (:LoopBody
              (bind _aswbp_equipment_select_eq_box (Utilities|Casting|CastToWBP_EquipmentSelect_EqBox _childwidget))
              (Utilities|Map|Add (LocalVariables|GetBoxMapping) (Variables|/HDCore/UI/HUD/EquipmentSelect/WBP_EquipmentSelect_EqBox.WBP_EquipmentSelect_EqBox_C|GetSlotNum _aswbp_equipment_select_eq_box) _aswbp_equipment_select_eq_box))))
        (:then_1
          (bind _array_element (Utilities|Array|ForEachLoopwithBreak (Variables|/Script/HDMain.HDKit|GetItemEntries Loadout) :!label _label)
            (:LoopBody
              (if (.ReturnValue (Utilities|Map|Find (LocalVariables|GetBoxMapping) (.SlotNum (Utilities|Struct|BreakHDItemEntry _array_element))))
                (if (not (== (.ItemClass (Utilities|Struct|BreakHDItemEntry _array_element)) (Utilities|GetClass (Variables|/HDCore/UI/HUD/EquipmentSelect/WBP_EquipmentSelect_EqBox.WBP_EquipmentSelect_EqBox_C|GetEqpItem (.Value (Utilities|Map|Find (LocalVariables|GetBoxMapping) (.SlotNum (Utilities|Struct|BreakHDItemEntry _array_element))))))))
                  (LocalVariables|SetValid false :!label _label_2)
                  (CallFunction|AddLogText "ValidateEquipment" "Fail Check 1" true)
                  (goto _label Break))
                (else
                  (goto _label_2))))
            (:Completed
              (if (not (LocalVariables|GetValid))
                (return false)))))
        (:then_2
          (bind _values (Utilities|Map|Values (LocalVariables|GetBoxMapping)))
          (bind _array_element_2 (Utilities|Array|ForEachLoopwithBreak _values :!label _label_3)
            (:LoopBody
              (if (Utilities|IsValid (Variables|/HDCore/UI/HUD/EquipmentSelect/WBP_EquipmentSelect_EqBox.WBP_EquipmentSelect_EqBox_C|GetEqpItem _array_element_2))
                (if (not (.ReturnValue (Class|DFInventoryComponent|Find Inventory (Variables|/HDCore/UI/HUD/EquipmentSelect/WBP_EquipmentSelect_EqBox.WBP_EquipmentSelect_EqBox_C|GetEqpItem _array_element_2))))
                  (LocalVariables|SetValid false :!label _label_4)
                  (CallFunction|AddLogText "ValidateEquipment" "Fail Check 2" true)
                  (goto _label_3 Break))
                (else
                  (goto _label_4))))
            (:Completed
              (return (LocalVariables|GetValid)))))))))

(fn GetOwnerCharacter
  (bind _asbp_hdplayer_character (Utilities|Casting|CastToBP_HDPlayerCharacter (Variables|Logic|GetOwnerCharacter)))
  (return _asbp_hdplayer_character))