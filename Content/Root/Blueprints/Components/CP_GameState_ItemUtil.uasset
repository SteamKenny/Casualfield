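; GameState component that resolves weapon actors and class paths to display names and icons.
; On BeginPlay it loads class-path remaps, maps every team kit's item classes by path, then caches matching name rows from the Weapon_mapping table.
; Actor lookup traces projectiles to their owner, remaps the path, then falls back to type-based names, recording detection failures.
; An experimental function, uncalled here, removes kits containing grenade or rocket launchers.
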(event EventBeginPlay
  (|CallParentFunction)
  (Logic|LoadRemapping)
  (Logic|EnumerateAllKitItemClasses)
  (Logic|ReduceMapstoKits))

(event EventTick
  (params (DeltaSeconds :type Float%20%28single-precision%29)))

(fn EnumerateAllKitItemClasses
  (for _array_element (Variables|/Script/DonkehFramework.DFBaseGameState|GetTeamArray (CallFunction|GetHDGameState))
    (bind _asteam_state__hd_ (Utilities|Casting|CastToHDTeamState _array_element))
    (bind _result (Utilities|Set|ToArray (Variables|/Script/HDMain.HDTeamState|GetKits _asteam_state__hd_)))
    (for _array_element_2 _result
      (bind _array_element_3 (Utilities|Array|ForEachLoopwithBreak (Variables|/Script/HDMain.HDKit|GetItemEntries _array_element_2))
        (:LoopBody
          (Utilities|Map|Add (Variables|Logic|GetStringToClassMap_Item) (Logic|GetClassPath (.ItemClass (Utilities|Struct|BreakHDItemEntry _array_element_3))) (.ItemClass (Utilities|Struct|BreakHDItemEntry _array_element_3))))))))

(fn FilterFactionKitsExperimental
  (for _array_element (Variables|/Script/DonkehFramework.DFBaseGameState|GetTeamArray (CallFunction|GetHDGameState))
    (bind _asteam_state__hd_ (Utilities|Casting|CastToHDTeamState _array_element))
    (bind _result (Utilities|Set|ToArray (Variables|/Script/HDMain.HDTeamState|GetKits _asteam_state__hd_)))
    (for _array_element_2 _result
      (bind _array_element_3 (Utilities|Array|ForEachLoopwithBreak (Variables|/Script/HDMain.HDKit|GetItemEntries _array_element_2) :!label _label)
        (:LoopBody
          (if (or (Utilities|Enum|Equal(Enum) (.SpecificItemType (Utilities|GetClassDefaults (.ItemClass (Utilities|Struct|BreakHDItemEntry _array_element_3)))) "GrenadeLauncher") (Utilities|Enum|Equal(Enum) (.SpecificItemType (Utilities|GetClassDefaults (.ItemClass (Utilities|Struct|BreakHDItemEntry _array_element_3)))) "RocketLauncher"))
            (Utilities|Set|Remove (Variables|/Script/HDMain.HDTeamState|GetKits _asteam_state__hd_) _array_element_2)
            (goto _label Break)))))))

(fn GetItemfromClassPath
  (params (ClassDisplayName :type String))
  (bind _stringtoclassmap_item (Variables|Logic|GetStringToClassMap_Item))
  (bind (_value _returnvalue) (Utilities|Map|Find _stringtoclassmap_item ClassDisplayName))
  (if _returnvalue
    (bind _asdfbase_item (Utilities|Casting|CastToDFBaseItemClass _value))
    (return _asdfbase_item)))

(fn GetWeaponIconfromClassPath
  (params (ClassPath :type String))
  (bind _stringtoclassmap_item (Variables|Logic|GetStringToClassMap_Item))
  (bind (_value _returnvalue) (Utilities|Map|Find _stringtoclassmap_item ClassPath))
  (if _returnvalue
    (bind _ashdbase_weapon (Utilities|Casting|CastToHDBaseWeaponClass _value))
    (return (Utilities|GetClassDefaults _ashdbase_weapon))))

(fn GetWeaponNamefromClassPath
  (params (ClassPath :type String))
  (bind _stringtoweaponstr (Variables|Logic|GetStringToWeaponStr))
  (bind (_value _returnvalue) (Utilities|Map|Find _stringtoweaponstr ClassPath))
  (bind (_shortfriendlyname _longfriendlyname) (Utilities|Struct|BreakSTR_WeaponMapping _value))
  (if _returnvalue
    (return _shortfriendlyname _longfriendlyname)))

(fn GetWeaponNameandIconfromActor
  (params (Actor :type Actor%20Object%20Reference))
  (Utilities|IsValid Actor
    (:Is%20Valid
      (bind _output_get (LocalVariables|SetCurrentWeapon Actor))
      (Utilities|FlowControl|Sequence
        (:then_0
          (bind _ashdbase_projectile (Utilities|Casting|CastToHDBaseProjectile _output_get))
          (Utilities|IsValid (Components|GetOwner _ashdbase_projectile)
            (:Is%20Valid
              (LocalVariables|SetCurrentWeapon (Components|GetOwner _ashdbase_projectile)))
            (:Is%20Not%20Valid
              (Logic|RecordWeaponDetectionFailure "INVALID OWNER" _output_get)
              (return "INVALID OWNER" "/CasualCQB/Root/Textures/no-weapon-icon_240x82.no-weapon-icon_240x82"))))
        (:then_1
          (bind _out (Logic|RemapWeaponClassString (Logic|GetClassPath (Utilities|GetClass _output_get))))
          (LocalVariables|SetCurrentWeaponClassPath _out))
        (:then_2
          (if (not (Class|DFBlueprintFunctions|IsEmptyorWhitespace (.Short (Logic|GetWeaponNamefromClassPath (LocalVariables|GetCurrentWeaponClassPath)))))
            (return (.Short (Logic|GetWeaponNamefromClassPath (LocalVariables|GetCurrentWeaponClassPath))) (Logic|GetWeaponIconfromClassPath (LocalVariables|GetCurrentWeaponClassPath)))))
        (:then_3
          (bind _ashdbase_weapon (Utilities|Casting|CastToHDBaseWeapon (LocalVariables|GetCurrentWeapon))
            (:then
              (return (Utilities|String|EnumtoString (Class|DFBaseItem|GetSpecificItemType _ashdbase_weapon)) (Variables|/Script/HDMain.HDBaseWeapon|GetDisplayIcon _ashdbase_weapon)))
            (:CastFailed
              (Utilities|Casting|CastToBP_HDProj_GrenadeBase (LocalVariables|GetCurrentWeapon)
                (:then
                  (return "Grenade" "/CasualCQB/Root/Textures/no-weapon-icon_240x82.no-weapon-icon_240x82"))
                (:CastFailed
                  (Utilities|Casting|CastToBP_HDProj_RocketBase (LocalVariables|GetCurrentWeapon)
                    (:then
                      (return "Rocket" "/CasualCQB/Root/Textures/no-weapon-icon_240x82_r.no-weapon-icon_240x82_r"))
                    (:CastFailed
                      (Logic|RecordWeaponDetectionFailure "UNKNOWN" (LocalVariables|GetCurrentWeapon))
                      (return "UNKNOWN" "/CasualCQB/Root/Textures/no-weapon-icon_240x82.no-weapon-icon_240x82"))))))))))
    (:Is%20Not%20Valid
      (Logic|RecordWeaponDetectionFailure "INVALID ACTOR")
      (return "INVALID ACTOR" "/CasualCQB/Root/Textures/no-weapon-icon_240x82.no-weapon-icon_240x82"))))

(fn RemapWeaponClassString
  (params (In :type String))
  (bind _stringtostringmap_remap (Variables|Logic|GetStringToStringMap_Remap))
  (bind (_value _returnvalue) (Utilities|Map|Find _stringtostringmap_remap In))
  (if _returnvalue
    (return _value)
    (else
      (return In))))

(fn ReduceMapstoKits
  (bind _keys (Utilities|Map|Keys (Variables|Logic|GetStringToClassMap_Item)))
  (for _array_element _keys
    (bind _returnvalue (Utilities|GetDataTableRow "/CasualCQB/Root/Data/weapon_mapping.weapon_mapping" (Utilities|String|StringToName _array_element))
      (:then
        (Utilities|Map|Add (Variables|Logic|GetStringToWeaponStr) _array_element _returnvalue)))))

(fn GetWeaponNamefromClassPathAll
  (params (ClassPath :type String))
  (bind _returnvalue (Utilities|GetDataTableRow "/CasualCQB/Root/Data/weapon_mapping.weapon_mapping" (Utilities|String|StringToName ClassPath))
    (:then
      (return (.ShortFriendlyName (Utilities|Struct|BreakSTR_WeaponMapping _returnvalue)) (.LongFriendlyName (Utilities|Struct|BreakSTR_WeaponMapping _returnvalue))))))

(fn LoadRemapping
  (bind (_rowname _rowindex _tablerow) (Utilities|ForEachDataTableRow "/CasualCQB/Root/Data/weapon_remapping.weapon_remapping")
    (:LoopBody
      (Utilities|Map|Add (Variables|Logic|GetStringToStringMap_Remap) (Utilities|String|ToString(Name) _rowname) (Utilities|Struct|BreakSTR_Weapon_Remapping _tablerow)))))

(fn GetClassPath
  (params (Class :type Actor%20Class%20Reference))
  (return (Utilities|ToString(SoftClassReference) (Utilities|ResolveSoftReference Class))))

(fn RecordWeaponDetectionFailure
  (params (Description :type String) (Class :type Actor%20Object%20Reference))
  (Utilities|Array|Add (Variables|Logic|GetWeaponDetectionFailures) (Utilities|Struct|MakeSTR_Weapon_Detection_Failure Description (select (Utilities|IsValid Class) (Utilities|GetClass Class) 0))))