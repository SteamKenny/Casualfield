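; Character component that controls the downed and dead ragdoll state of a player or AI character.
; Separate server and client setup functions toggle collision, with the client also switching mesh physics, camera arm, first-person mesh, player input, tag attachment and weapon visibility.
; Tick tracks downed time, stops movement, blocks firing, catches weapons missed during switching and strips most mesh collision on death.
; Abort functions turn downed into dead.
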(event EventBeginPlay
  (|CallParentFunction))

(event EventTick
  (params (DeltaSeconds :type Float%20%28single-precision%29))
  (|CallParentFunction DeltaSeconds)
  (Logic|UpdateTime DeltaSeconds)
  (Utilities|FlowControl|Sequence
    (:then_0
      (Networking|CanExecuteCosmeticEvents
        (:True
          (Logic|HideWeapons) ; Catch any weapons that were missed in Setup due to in-progress switching
        )))
    (:then_1
      (Logic|UpdateMovement) ; Stop movement when downed
      (Logic|UpdateWeapon) ; Prevent both players & AI firing when downed
      (Logic|UpdateDeath) ; Set collisions when dead
    )))

(fn SetupCharacterServer
  (params (Downed :type Boolean))
  (bind _returnvalue (select Downed "ECR_Ignore" "ECR_Block"))
  (if Downed
    (Variables|Logic|SetbIsDowned true) ; Set flag before setting collision responses so overlaps trigger after we set flag
  )
  (if (Variables|Logic|GetbInitialised)
    (if Downed
      (Class|DFBaseCharacter|GoProne (Logic|GetCharacter)))
    (Collision|SetCollisionResponsetoChannel (Variables|Logic|GetCapsuleComponent) "ECC_Pawn" _returnvalue) ; Prevent server pawn collision when downed
    (Collision|SetCollisionResponsetoChannel (Variables|Logic|GetMesh) "ECC_Visibility" _returnvalue) ; Prevent server visibility when downed (for AI)
    (Collision|SetCollisionResponsetoChannel (Variables|Logic|GetCapsuleComponent) "ECC_WorldDynamic" _returnvalue) ; Prevent server pawn from "taking" capture points
  )
  (if (not Downed)
    (Variables|Logic|SetbIsDowned false) ; Clear flag after setting collision responses so overlaps trigger before we clear flag
  ))

(fn SetupCharacterClient
  (params (Downed :type Boolean) (KillVelocity :type Boolean))
  (bind _character (Logic|GetCharacter))
  (bind _capsulecomponent (Variables|Logic|GetCapsuleComponent))
  (bind _springarm (Variables|Logic|GetSpringArm))
  (bind _mesh1p (Variables|Logic|GetMesh1P))
  (bind _mesh1p_2 (Variables|Logic|GetMesh1P))
  (bind _mesh (Variables|Logic|GetMesh))
  (bind _springarm_2 (Variables|Logic|GetSpringArm))
  (bind _mesh_2 (Variables|Logic|GetMesh))
  (bind _capsulecomponent_2 (Variables|Logic|GetCapsuleComponent))
  (Variables|Logic|SetbIsDowned Downed)
  (if (Variables|Logic|GetbInitialised)
    (if (Variables|Logic|GetbIsDowned)
      (Class|DFBaseCharacter|UnAim _character)
      (Class|DFBaseCharacter|GoProne _character)
      (if false
        (bind _returnvalue (Physics|GetPhysicsLinearVelocity _mesh_2 "Pelvis"))
        (Class|PrimitiveComponent|SetAllPhysicsLinearVelocity _mesh_2 (* _returnvalue (Variables|Logic|GetVelocityKillMultiplier)) false))
      (Physics|SetSimulatePhysics _mesh_2 true)
      (Collision|SetCollisionResponsetoChannel _capsulecomponent "ECC_Pawn" "ECR_Ignore")
      (Collision|SetCollisionResponsetoChannel _capsulecomponent "ECC_WorldDynamic" "ECR_Ignore") ; Prevent client pawn from "showing" in capture points
      (Collision|SetCollisionResponsetoChannel _mesh_2 "ECC_GameTraceChannel1" "ECR_Ignore")
      (Collision|SetCollisionEnabled _mesh_2 "QueryAndPhysics")
      (Variables|/Script/Engine.SpringArmComponent|SetbUsePawnControlRotation _springarm_2 false)
      (Variables|/Script/Engine.SpringArmComponent|SetbDoCollisionTest _springarm_2 true)
      (Variables|/Script/Engine.SpringArmComponent|SetProbeSize _springarm_2 1.5e+02) ; WARNING: HARD-CODES!
      (Utilities|IsValid _mesh1p_2
        (:Is%20Valid
          (Rendering|SetVisibility _mesh1p_2 false false))
        (:Is%20Not%20Valid
          _))
      (Logic|HideWeapons)
      (Input|DisableInput (Logic|GetCharacter) (Logic|GetPlayerController)) ; NOTE: only works for players, not AI
      (Transformation|AttachComponentToComponent (Variables|Logic|GetPlayerTag) (Variables|Logic|GetMesh) "pelvis" "KeepRelative" "SnapToTarget" "SnapToTarget" true)
      (else
        (Physics|SetSimulatePhysics _mesh false)
        (Collision|SetCollisionResponsetoChannel _capsulecomponent_2 "ECC_Pawn" "ECR_Block")
        (Collision|SetCollisionResponsetoChannel _capsulecomponent_2 "ECC_WorldDynamic" "ECR_Block") ; Allow client pawn from "showing" in capture points
        (Collision|SetCollisionResponsetoChannel _mesh "ECC_GameTraceChannel1" "ECR_Block")
        (Collision|SetCollisionEnabled _mesh "QueryOnly")
        (Transformation|AttachComponentToComponent _mesh (Variables|Logic|GetCapsuleComponent) "None" "KeepRelative" "KeepRelative" "KeepRelative" true)
        (Transformation|SetRelativeRotation _mesh "0,-90.000000, 0" false true) ; WARNING: HARD-CODES!
        (Transformation|SetRelativeLocation _mesh (Logic|GetMeshOffsetforState) false true)
        (Variables|/Script/Engine.SpringArmComponent|SetbUsePawnControlRotation _springarm true)
        (Variables|/Script/Engine.SpringArmComponent|SetbDoCollisionTest _springarm false)
        (Variables|/Script/Engine.SpringArmComponent|SetProbeSize _springarm 12.0) ; WARNING: HARD-CODES!
        (Utilities|IsValid _mesh1p
          (:Is%20Valid
            (Rendering|SetVisibility _mesh1p true false))
          (:Is%20Not%20Valid
            _))
        (Logic|ShowWeapons)
        (Input|EnableInput (Logic|GetCharacter) (Logic|GetPlayerController)) ; NOTE: only works for players, not AI
        (Transformation|AttachComponentToComponent (Variables|Logic|GetPlayerTag) (Variables|Logic|GetMesh) "head" "KeepRelative" "SnapToTarget" "SnapToTarget" true)))))

(fn AbortServer
  (Variables|Logic|SetbIsDowned false)
  (Variables|Logic|SetbIsDead true)
  (Variables|Logic|SetResuscitator 0))

(fn AbortClient
  (Variables|Logic|SetbIsDowned false)
  (Variables|Logic|SetbIsDead true)
  (if (Variables|Logic|GetbInitialised)
    (Logic|ShowWeapons)
    (Variables|Logic|SetResuscitator 0)))

(fn GetCharacter
  (bind _asdfbase_character (Utilities|Casting|CastToDFBaseCharacter (Components|GetOwner)))
  (return _asdfbase_character))

(fn Initialise
  (params (Mesh :type Skeletal%20Mesh%20Component%20Object%20Reference) (Mesh1P :type Skeletal%20Mesh%20Component%20Object%20Reference) (CapsuleComponent :type Capsule%20Component%20Object%20Reference) (SpringArm :type Spring%20Arm%20Component%20Object%20Reference) (PlayerTag :type Widget%20Component%20Object%20Reference))
  (Variables|Logic|SetMesh Mesh)
  (Variables|Logic|SetMesh1P Mesh1P)
  (Variables|Logic|SetCapsuleComponent CapsuleComponent)
  (Variables|Logic|SetSpringArm SpringArm)
  (Variables|Logic|SetPlayerTag PlayerTag)
  (Variables|Logic|SetbInitialised true))

(fn GrabEquippedWeapon
  (bind _asbp_hdplayer_character_base (Utilities|Casting|CastToBP_HDPlayerCharacterBase (Logic|GetCharacter)))
  (return (Variables|/HDCore/Core/BP_HDPlayerCharacterBase.BP_HDPlayerCharacterBase_C|GetEquippedWeapon _asbp_hdplayer_character_base)))

(fn HideWeapons
  (bind _equippedweapon (Logic|GrabEquippedWeapon))
  (if (Variables|Logic|GetbIsDowned)
    (if (== (Utilities|Array|FindItem (Variables|Logic|GetHiddenWeapons) _equippedweapon) -1)
      (Utilities|Array|AddUnique (Variables|Logic|GetHiddenWeapons) _equippedweapon)
      (CallFunction|SetActorVisibility _equippedweapon false))))

(fn ShowWeapons
  (for _array_element (Variables|Logic|GetHiddenWeapons)
    (CallFunction|SetActorVisibility _array_element true))
  (Utilities|Array|Clear (Variables|Logic|GetHiddenWeapons)))

(fn SetIsDowned
  (Variables|Logic|SetbIsDowned true))

(fn IsDownedorDead
  (return (or (Variables|Logic|GetbIsDowned) (Variables|Logic|GetbIsDead))))

(fn GetPlayerController
  (bind _asplayer_controller (Utilities|Casting|CastToPlayerController (Pawn|GetController (Logic|GetCharacter))))
  (return _asplayer_controller))

(fn UpdateTime
  (params (DeltaSeconds :type Float%20%28single-precision%29))
  (if (Variables|Logic|GetbIsDowned)
    (Variables|Logic|SetDownedElapsed (+ (Variables|Logic|GetDownedElapsed) DeltaSeconds))
    (else
      (Variables|Logic|SetDownedElapsed 0.0))))

(fn UpdateWeapon
  (bind _equippedweapon (Logic|GrabEquippedWeapon))
  (Utilities|IsValid _equippedweapon
    (:Is%20Valid
      (Variables|/Script/DonkehFramework.DFBaseItem|SetbDisableFireInput _equippedweapon (Variables|Logic|GetbIsDowned)))))

(fn UpdateMovement
  (if (Variables|Logic|GetbIsDowned)
    (Class|NavMovementComponent|StopActiveMovement (Variables|/Script/DonkehFramework.DFBaseCharacter|GetDFCharacterMovement (Logic|GetCharacter)))))

(fn UpdateDeath
  (bind _mesh (Variables|Logic|GetMesh))
  (if (Variables|Logic|GetbIsDead)
    (Collision|SetCollisionResponsetoAllChannels _mesh "ECR_Ignore")
    (Collision|SetCollisionResponsetoChannel _mesh "ECC_WorldStatic" "ECR_Block")))

(fn DeathCameraUpdate
  (bind _resuscitator (Variables|Logic|GetResuscitator))
  (Utilities|IsValid _resuscitator
    (:Is%20Valid
      (Default|UpdatePosition _resuscitator))))

(fn DeathScreenExecute
  (bind _resuscitator (Variables|Logic|GetResuscitator))
  (Utilities|IsValid _resuscitator
    (:Is%20Valid
      (if (Default|GetAllowGiveUp _resuscitator)
        (Default|DontRespawn _resuscitator)))))

(fn CharacterIsBot
  (Utilities|Casting|CastToAIController (Pawn|GetController (Logic|GetCharacter))
    (:then
      (return true))
    (:CastFailed
      (return false))))

(fn GetMeshOffsetforState
  (bind _character (Logic|GetCharacter))
  (bind _dfcharactermovement (Variables|/Script/DonkehFramework.DFBaseCharacter|GetDFCharacterMovement _character))
  (if (Class|DFCharacterMovementComponent|IsProne _dfcharactermovement)
    (return "0.000000, 0,-24.000000")
    (elif (AI|Components|NavMovement|IsCrouching _dfcharactermovement)
      (return "0, 0,-62.000000")
      (else
        (return "0, 0,-94.000000")))))