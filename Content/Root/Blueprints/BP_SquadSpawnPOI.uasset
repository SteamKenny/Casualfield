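; BP_SquadSpawnPOI is a point-of-interest actor, owned by a player controller, that marks the player's available squad spawn location.
; A looping two-second timer runs while the server allows squad spawning and the game has not ended.
; Without a living pawn, it teleports to the controller's FindSquadSpawn result and shows itself, hiding if none is valid or the player is alive.
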(event Custom|OnUpdate
  (bind _asbp_hdplayer_controller_cqb (Utilities|Casting|CastToBP_HDPlayerController_CQB (Components|GetOwner)))
  (if (and (Variables|/CasualCQB/Root/Blueprints/Components/CP_GameState_Config.CP_GameState_Config_C|GetAllowSquadSpawn (CallFunction|GetServerConfig)) (not (Default|HasGameEnded _asbp_hdplayer_controller_cqb)))
    (bind _asdfbase_player_character (Utilities|Casting|CastToDFBasePlayerCharacter (Pawn|GetControlledPawn _asbp_hdplayer_controller_cqb))
      (:then
        (if (Class|DFBaseCharacter|IsAlive _asdfbase_player_character)
          (Variables|Logic|SetVisible false :!label _label)
          (Default|CallOnShowHide false)
          (else
            (bind (_result _valid) (Default|FindSquadSpawn _asbp_hdplayer_controller_cqb :!label _label_2))
            (if _valid
              (Transformation|SetActorTransform _result false true)
              (Variables|Logic|SetUpdateTime (Utilities|Time|GetGameTimeinSeconds))
              (Variables|Logic|SetVisible true)
              (Default|CallOnShowHide true)
              (else
                (goto _label))))))
      (:CastFailed
        (goto _label_2)))))

(event EventBeginPlay
  (|CallParentFunction)
  (Utilities|Time|SetTimerbyEvent (delegate Custom|OnUpdate) 2.0 true))

(event Collision|EventActorBeginOverlap
  (params (OtherActor :type Actor%20Object%20Reference)))

(event EventTick
  (params (DeltaSeconds :type Float%20%28single-precision%29)))

(fn ConstructionScript)