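; Per-player spawn protection actor that treats a trigger volume as a safe zone for the owning team and a kill zone for others.
; On authority, it waits for the owner's team state, then watches the trigger for that character's overlaps.
; Same-team owners get safe-zone status, while others start a short suicide timer that is cleared on leaving.
; Local owners see a matching widget during matches, and the actor destroys itself with its owner.
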(event Custom|Initialise
  (params (Trigger :type Actor%20Object%20Reference))
  (Networking|SwitchHasAuthority
    (:Authority
      (bind _result (Logic|IsOwnerStateAvailable :!label _label))
      (if _result
        (Collision|BindEventtoOnActorEndOverlap Trigger (delegate Custom|LeaveEvent))
        (Collision|BindEventtoOnActorBeginOverlap Trigger (delegate Custom|EnterEvent))
        (for _array_element (Collision|GetOverlappingActors Trigger "/HDAssets/Core/BP_HDPlayerCharacter.BP_HDPlayerCharacter_C" :!class /Script/Engine.Actor)
          (bind _result_2 (Logic|ActorIsOwner _array_element))
          (if _result_2
            (bind _result_3 (Logic|IsSafeZone))
            (if _result_3
              (Logic|SetSafeZone true)
              (CallFunction|LogicUpdateClient true)
              (else
                (bind _returnvalue (Utilities|Time|SetTimerbyEvent (delegate Custom|Die) 5.0))
                (CallFunction|LogicUpdateClient true)))))
        (else
          (Utilities|FlowControl|Delay 0.2)
          (goto _label))))))

(event Custom|Die
  (Logic|RequestSuicide))

(event Custom|LeaveEvent
  (params (OverlappedActor :type Actor%20Object%20Reference) (OtherActor :type Actor%20Object%20Reference))
  (bind _result (Logic|ActorIsOwner OtherActor))
  (if _result
    (bind _result_2 (Logic|IsSafeZone))
    (if _result_2
      (Logic|SetSafeZone false)
      (CallFunction|LogicUpdateClient false)
      (else
        (Utilities|Time|ClearandInvalidateTimerbyHandle (stale Custom|Initialise _returnvalue))
        (CallFunction|LogicUpdateClient false)))))

(event Custom|LogicUpdateClient
  (params (Show :type Boolean))
  (if (Logic|OwnerIsLocal)
    (Networking|CanExecuteCosmeticEvents
      (:True
        (CallFunction|ShowHide (and (Default|IsMatchinProgress (CallFunction|GetGameStateCQB)) Show))))))

(event Custom|EnterEvent
  (params (OverlappedActor :type Actor%20Object%20Reference) (OtherActor :type Actor%20Object%20Reference))
  (bind _result (Logic|ActorIsOwner OtherActor))
  (if _result
    (bind _result_2 (Logic|IsSafeZone))
    (if _result_2
      (Logic|SetSafeZone true)
      (CallFunction|LogicUpdateClient true)
      (else
        (bind _returnvalue (Utilities|Time|SetTimerbyEvent (delegate Custom|Die) 5.0))
        (CallFunction|LogicUpdateClient true)))))

(event Custom|OnOwnerDestroyed
  (params (DestroyedActor :type Actor%20Object%20Reference))
  (Actor|DestroyActor))

(event EventBeginPlay
  (|CallParentFunction)
  (Game|BindEventtoOnDestroyed (Components|GetOwner) (delegate Custom|OnOwnerDestroyed)))

(event Collision|EventActorBeginOverlap
  (params (OtherActor :type Actor%20Object%20Reference))
  (|CallParentFunction OtherActor) ; This node is disabled and will not be called.\nDrag off pins to build functionality.
)

(fn ConstructionScript
  (|CallParentFunction))

(fn ActorIsOwner
  (params (Actor :type Actor%20Object%20Reference))
  (return Actor (== Actor (Components|GetOwner))))

(fn ShowHideLogic
  ;[1 1 1] Disable Parent Logic
)

(fn SetSafeZone
  (params (Active :type Boolean))
  (bind _spawnprotection (Class|IFCharacter|GetSpawnProtection(Message) (Components|GetOwner)))
  (Utilities|IsValid _spawnprotection
    (:Is%20Valid
      (Default|ServerSetSafeZone _spawnprotection Active))))

(fn RequestSuicide
  (bind _ashdplayer_character (Utilities|Casting|CastToHDPlayerCharacter (Components|GetOwner)))
  (if (Class|DFBaseCharacter|IsAlive _ashdplayer_character)
    (Class|DFBaseCharacter|Suicide _ashdplayer_character)))

(fn IsOwnerStateAvailable
  (bind _ashdplayer_character (Utilities|Casting|CastToHDPlayerCharacter (Components|GetOwner))
    (:then
      (Utilities|IsValid _ashdplayer_character
        (:Is%20Valid
          (return (Utilities|IsValid (Variables|/Script/HDMain.HDPlayerCharacter|GetHDTeamState _ashdplayer_character))))))
    (:CastFailed
      (return false))))

(fn OwnerIsLocal
  (bind _aspawn (Utilities|Casting|CastToPawn (Components|GetOwner)))
  (return (Class|DFBlueprintFunctions|IsLocallyPlayerControlled _aspawn)))

(fn IsSafeZone
  (bind _ashdplayer_character (Utilities|Casting|CastToHDPlayerCharacter (Components|GetOwner)))
  (return (== (Variables|Default|GetOwning%20Team) (Class|HDTeamState|GetTeam (Variables|/Script/HDMain.HDPlayerCharacter|GetHDTeamState _ashdplayer_character)))))

(fn GetUIWidgetClass
  (|CallParentFunction)
  (bind _result (Logic|IsSafeZone))
  (return (select _result "/CasualCQB/Root/UI/HUD/WBP_SafeZone.WBP_SafeZone_C" "/CasualCQB/Root/UI/HUD/WBP_InvalidZone.WBP_InvalidZone_C")))