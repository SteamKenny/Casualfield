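; Interactable actor for a downed player or bot that manages ragdoll state until revival or death.
; Interacting revives the pawn, faster for medics; timeout or the owner giving up after a server-configured delay kills it.
; The owning client reports pelvis position, which the server uses to move the pawn and other clients follow via PhysicsHandle.
; A widget icon shows to able, nearby players filtered by relationship and medic role.
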(event Custom|DoRespawn
  (if (Utilities|Enum|Equal(Enum) (Variables|Logic|GetSpawnAction) "NewEnumerator0")
    (Logic|RespawnPlayer)
    (CallFunction|OnRespawn)))

(event Custom|DontRespawn
  (if (Utilities|Enum|Equal(Enum) (Variables|Logic|GetSpawnAction) "NewEnumerator0")
    (Logic|KillPlayer) ; NOTE: this will trigger the character death handler above
  ))

(event Custom|StartWait
  (Utilities|FlowControl|Delay (Math|Float|SelectFloat (Variables|Logic-Config|GetTimeToDieAI) (Variables|Logic-Config|GetTimeToDiePlayer) (Logic|IsOwnerAI)))
  (if (Utilities|Enum|Equal(Enum) (Variables|Logic|GetSpawnAction) "NewEnumerator0")
    (Logic|KillPlayer) ; NOTE: this will trigger the character death handler above
  ))

(event Custom|OnDontRespawn
  (Variables|Logic|SetSpawnAction "NewEnumerator2") ; Ensure this is set using a reliable event
  (Logic|AbortCharacter)
  (CallFunction|ShowHide false)
  (Logic|ReleasePhysicsHandler))

(event Custom|ServerUpdateCenterPosition
  (params (Feedback :type Vector))
  (bind _output_get (Variables|Logic|SetCenterPosition Feedback))
  (Variables|Logic|SetReplicatedCenterPosition _output_get)
  (Logic|MoveCharacter))

(event Custom|OnClientFeedback
  (bind _result (Logic|UpdatePosition))
  (if _result
    (CallFunction|ServerUpdateCenterPosition (Variables|Logic|GetCenterPosition))))

(event Custom|OnRespawn
  (Variables|Logic|SetSpawnAction "NewEnumerator1") ; Ensure this is set using a reliable event
  (Logic|SetupCharacter false)
  (CallFunction|ShowHide false)
  (Logic|ReleasePhysicsHandler))

(event Custom|OnCharacterDeath
  (params (VictimPawn :type Pawn%20Object%20Reference) (VictimController :type Controller%20Object%20Reference) (KillingDamage :type Float%20%28single-precision%29) (DamageEvent :type Damage%20Event%20Structure%20%28by%20ref%29) (InstigatingPawn :type Pawn%20Object%20Reference) (DamageCauser :type Actor%20Object%20Reference))
  (CallFunction|OnDontRespawn))

(event EventBeginPlay
  (|CallParentFunction)
  (if (Utilities|Enum|Equal(Enum) (Variables|Logic|GetSpawnAction) "NewEnumerator0")
    (Actor|SetLifeSpan (Variables|Logic-Config|GetMaxLifespan)) ; Make sure we never live for more than 1 minute
    (Logic|SetupCharacter true)
    (Utilities|FlowControl|Sequence
      (:then_0
        (Networking|SwitchHasAuthority
          (:Authority
            (bind _asdfbase_character (Utilities|Casting|CastToDFBaseCharacter (Variables|Logic|GetOwnerPawn)))
            (EventDispatchers|BindEventtoOnCharacterDeath _asdfbase_character (delegate Custom|OnCharacterDeath)))))
      (:then_1
        (Networking|CanExecuteCosmeticEvents
          (:True
            (Logic|InitialiseWidget)
            (CallFunction|Update 0.0) ; Initial client update
            (if (== (Game|GetPlayerController 0) (Components|GetOwner))
              (Utilities|Time|SetTimerbyEvent (delegate Custom|OnClientFeedback) (Variables|Logic-Config|GetFeedbackInitialDelay) true (Variables|Logic-Config|GetFeedbackInitialDelay)))))))
    (else
      (Components|DestroyComponent (Variables|Default|GetIconWidget) :!pinned true) ; We can't destroy any replicated versions that are passed the non-set state, we have to wait for server death\nAt least we can remove the 3D UI for these "dead" replicated actors
    )))

(event EventOnUsePressed
  (if (== (CallFunction|GetClientControlledPawn) (Variables|Logic|GetOwnerPawn))
    (if (Logic|GetAllowGiveUp)
      (CallFunction|DontRespawn))
    (else
      (|CallParentFunction))))

(event EventDestroyed)

(event EventOnInteracted
  (CallFunction|DoRespawn))

(event EventUpdate
  (params (DeltaSeconds :type Float%20%28single-precision%29))
  (|CallParentFunction DeltaSeconds)
  (Logic|CalculateDistanceto)
  (Logic|UpdateWidgetVisibility))

(event EventTick
  (params (DeltaSeconds :type Float%20%28single-precision%29))
  (|CallParentFunction DeltaSeconds)
  (Logic|Calculate DeltaSeconds)
  (Networking|SwitchHasAuthority
    (:Authority
      (Logic|CheckforAllowGiveUp))))

(fn ConstructionScript)

(fn UpdatePosition
  (bind _ownerpawn (Variables|Logic|GetOwnerPawn))
  (bind (_asbp_hdplayer_character _bsuccess) (Utilities|Casting|CastToBP_HDPlayerCharacter _ownerpawn))
  (if (Math|Boolean|ANDBoolean (Class|DFBlueprintFunctions|IsValidActor _ownerpawn) (Utilities|Enum|Equal(Enum) (Variables|Logic|GetSpawnAction) "NewEnumerator0") (Variables|Logic|GetbIsSetup))
    (if _bsuccess
      (Variables|Logic|SetCenterPosition (Transformation|GetSocketLocation (Variables|/Script/Engine.Character|GetMesh _asbp_hdplayer_character) "Pelvis"))
      (return true)
      (else
        _)))
  (return false))

(fn InitialiseWidget
  (bind _aswbp_resuscitator (Utilities|Casting|CastToWBP_Resuscitator (UserInterface|GetUserWidgetObject (Variables|Default|GetIconWidget))))
  (Default|Initialise _aswbp_resuscitator (Variables|Default|GetIconWidget)))

(fn UpdateWidgetVisibility
  (bind _iconwidget (Variables|Default|GetIconWidget))
  (Utilities|IsValid _iconwidget
    (:Is%20Valid
      (Rendering|SetVisibility _iconwidget (Math|Boolean|ANDBoolean (CallFunction|GetIsRelevantto (Widget|GetOwningPlayer (UserInterface|GetUserWidgetObject _iconwidget))) (not (CallFunction|IsShowingUI)) (< (Variables|Logic|GetDistanceTo) (Variables|Logic-Config|GetDistanceCutOff))) false))))

(fn RespawnPlayer
  (Logic|MoveCharacter))

(fn KillPlayer
  (Transformation|SetActorLocation (Variables|Logic|GetOwnerPawn) (Variables|Logic|GetCenterPosition) false true) ; Sync server position so kit drop happens in correct location
  (bind _ashdplayer_character (Utilities|Casting|CastToHDPlayerCharacter (Variables|Logic|GetOwnerPawn)))
  (Class|DFBaseCharacter|Die _ashdplayer_character 0.0 (Utilities|Struct|MakeDamageEvent)) ; We don't connect 'Killer' because any score credit has already been given
)

(fn OnRepClientCenterPosition
  (Networking|CanExecuteCosmeticEvents
    (:True
      (if (Math|Boolean|ANDBoolean (!= (Game|GetPlayerController 0) (Components|GetOwner)) (Class|DFBlueprintFunctions|IsValidActor (Variables|Logic|GetOwnerPawn)) (Utilities|Enum|Equal(Enum) (Variables|Logic|GetSpawnAction) "NewEnumerator0"))
        (bind _asbp_hdplayer_character_cqb (Utilities|Casting|CastToBP_HDPlayerCharacter_CQB (Variables|Logic|GetOwnerPawn)))
        (Utilities|IsValid (Class|PhysicsHandleComponent|GetGrabbedComponent (Variables|/CasualCQB/Root/Core/BP_HDPlayerCharacter_CQB.BP_HDPlayerCharacter_CQB_C|GetPhysicsHandle _asbp_hdplayer_character_cqb))
          (:Is%20Valid
            _)
          (:Is%20Not%20Valid
            (bind (_outposition _outrotation) (Class|SkinnedMeshComponent|TransformfromBoneSpace (Variables|/Script/Engine.Character|GetMesh _asbp_hdplayer_character_cqb) "Pelvis" "0, 0, 0" "0, 0, 0"))
            (Physics|Components|PhysicsHandle|GrabComponentatLocationwithRotation (Variables|/CasualCQB/Root/Core/BP_HDPlayerCharacter_CQB.BP_HDPlayerCharacter_CQB_C|GetPhysicsHandle _asbp_hdplayer_character_cqb) (Variables|/Script/Engine.Character|GetMesh _asbp_hdplayer_character_cqb) "Pelvis" _outposition _outrotation)))
        (Physics|Components|PhysicsHandle|SetTargetLocation (Variables|/CasualCQB/Root/Core/BP_HDPlayerCharacter_CQB.BP_HDPlayerCharacter_CQB_C|GetPhysicsHandle _asbp_hdplayer_character_cqb) (Variables|Logic|GetReplicatedCenterPosition))))))

(fn ReleasePhysicsHandler
  (bind _ownerpawn (Variables|Logic|GetOwnerPawn))
  (if (Class|DFBlueprintFunctions|IsValidActor _ownerpawn)
    (bind _asbp_hdplayer_character_cqb (Utilities|Casting|CastToBP_HDPlayerCharacter_CQB _ownerpawn))
    (Utilities|IsValid (Class|PhysicsHandleComponent|GetGrabbedComponent (Variables|/CasualCQB/Root/Core/BP_HDPlayerCharacter_CQB.BP_HDPlayerCharacter_CQB_C|GetPhysicsHandle _asbp_hdplayer_character_cqb))
      (:Is%20Valid
        (Physics|Components|PhysicsHandle|ReleaseComponent (Variables|/CasualCQB/Root/Core/BP_HDPlayerCharacter_CQB.BP_HDPlayerCharacter_CQB_C|GetPhysicsHandle _asbp_hdplayer_character_cqb))))))

(fn SetupCharacter
  (params (IsDowned :type Boolean))
  (bind _ownercontroller (Variables|Logic|GetOwnerController))
  (Utilities|FlowControl|Sequence
    (:then_0
      (Networking|SwitchHasAuthority
        (:Authority
          (bind _ragdollcontrol (Class|IFCharacterCQB|GetRagDollControl(Message) (Variables|Logic|GetOwnerPawn)))
          (Utilities|IsValid _ragdollcontrol
            (:Is%20Valid
              (Default|SetupCharacterServer _ragdollcontrol IsDowned)
              (Variables|/CasualCQB/Root/Blueprints/Components/CP_Character_RagDollControl.CP_Character_RagDollControl_C|SetResuscitator _ragdollcontrol (select IsDowned self 0))
              (if (not IsDowned)
                (bind _asbp_hdplayer_controller_cqb (Utilities|Casting|CastToBP_HDPlayerController_CQB _ownercontroller)
                  (:then
                    (Default|OnPlayerResuscitatedServer _asbp_hdplayer_controller_cqb)
                    (bind _result (CallFunction|FriendorFoe 0 (Variables|Logic|GetOwnerPawn)))
                    (Default|OnPlayerResuscitatedClient _asbp_hdplayer_controller_cqb (CallFunction|GetPlayerNamefromPlayerState (Variables|Default|GetLockedPlayerState)) _result))
                  (:CastFailed
                    (bind _asbp_hdaicontroller_cqb (Utilities|Casting|CastToBP_HDAIController_CQB (Variables|Logic|GetOwnerController)))
                    (Default|OnBotResuscitated _asbp_hdaicontroller_cqb)))
                (else
                  (bind _asbp_hdplayer_controller_cqb_2 (Utilities|Casting|CastToBP_HDPlayerController_CQB _ownercontroller)
                    (:then
                      (Default|OnPlayerDownedServer _asbp_hdplayer_controller_cqb_2 self)
                      (Default|OnPlayerDownedClient _asbp_hdplayer_controller_cqb_2))
                    (:CastFailed
                      (bind _asbp_hdaicontroller_cqb_2 (Utilities|Casting|CastToBP_HDAIController_CQB (Variables|Logic|GetOwnerController)))
                      (Default|OnBotDowned _asbp_hdaicontroller_cqb_2))))))))))
    (:then_1
      (Networking|CanExecuteCosmeticEvents
        (:True
          (bind _ragdollcontrol_2 (Class|IFCharacterCQB|GetRagDollControl(Message) (Variables|Logic|GetOwnerPawn)))
          (Utilities|IsValid _ragdollcontrol_2
            (:Is%20Valid
              (Default|SetupCharacterClient _ragdollcontrol_2 IsDowned (!= (CallFunction|GetClientControlledPawn) (Variables|Logic|GetOwnerPawn)))
              (Variables|/CasualCQB/Root/Blueprints/Components/CP_Character_RagDollControl.CP_Character_RagDollControl_C|SetResuscitator _ragdollcontrol_2 (select IsDowned self 0)))))))
    (:then_2
      (Variables|Logic|SetbIsSetup true))))

(fn GetIsRelevantto
  (params (Controller :type Controller%20Object%20Reference))
  (bind _playerstate (Variables|/Script/Engine.Controller|GetPlayerState Controller))
  (if (Math|Boolean|ANDBoolean (Utilities|Enum|Equal(Enum) (Variables|Logic|GetSpawnAction) "NewEnumerator0") (Variables|Logic|GetbIsSetup) (Logic|PawnIsAble (Pawn|GetControlledPawn (Game|GetPlayerController 0))) (!= (Pawn|GetControlledPawn (Game|GetPlayerController 0)) (Variables|Logic|GetOwnerPawn)) (Class|DFBlueprintFunctions|IsValidActor (Variables|Logic|GetOwnerPawn)))
    (Utilities|IsValid Controller
      (:Is%20Valid
        (Utilities|IsValid _playerstate
          (:Is%20Valid
            (if true ; TODO: re-implement some kind of velocity test - but has to be reliable
              (bind _result (CallFunction|FriendorFoe _playerstate 0 0 (Variables|Logic|GetOwnerPawn)))
              (return (or (and (Logic|PlayerStateIsMedic _playerstate) (Utilities|Enum|Equal(Enum) _result "NewEnumerator2")) (Utilities|Enum|Equal(Enum) _result "NewEnumerator0")))))
          (:Is%20Not%20Valid
            (return false))))
      (:Is%20Not%20Valid
        (return false)))
    (else
      (return false))))

(fn AbortCharacter
  (Utilities|FlowControl|Sequence
    (:then_0
      (Networking|SwitchHasAuthority
        (:Authority
          (Utilities|FlowControl|Sequence
            (:then_0
              (bind _ragdollcontrol (Class|IFCharacterCQB|GetRagDollControl(Message) (Variables|Logic|GetOwnerPawn)))
              (Default|AbortServer _ragdollcontrol))
            (:then_1
              (bind _asbp_hdplayer_controller_cqb (Utilities|Casting|CastToBP_HDPlayerController_CQB (Variables|Logic|GetOwnerController))
                (:then
                  (Default|OnPlayerNotResuscitatedServer _asbp_hdplayer_controller_cqb (Variables|Logic|GetDownedSeconds)))
                (:CastFailed
                  (bind _asbp_hdaicontroller_cqb (Utilities|Casting|CastToBP_HDAIController_CQB (Variables|Logic|GetOwnerController)))
                  (Default|OnBotAborted _asbp_hdaicontroller_cqb))))))))
    (:then_1
      (Networking|CanExecuteCosmeticEvents
        (:True
          (bind _ragdollcontrol_2 (Class|IFCharacterCQB|GetRagDollControl(Message) (Variables|Logic|GetOwnerPawn)))
          (Default|AbortClient _ragdollcontrol_2))))))

(fn IsOwnerAI
  (Utilities|Casting|CastToAIController (Variables|Logic|GetOwnerController)
    (:then
      (return true))
    (:CastFailed
      (return false))))

(fn PawnIsMedic
  (params (Pawn :type Pawn%20Object%20Reference))
  (bind _playerstate (Variables|/Script/Engine.Pawn|GetPlayerState Pawn))
  (Utilities|IsValid Pawn
    (:Is%20Valid
      (Utilities|IsValid _playerstate
        (:Is%20Valid
          (return (Logic|PlayerStateIsMedic _playerstate)))
        (:Is%20Not%20Valid
          _)))
    (:Is%20Not%20Valid
      _))
  (return false))

(fn LockforPlayer
  (params (PlayerId :type Integer) (Action :type String) (Controller :type Controller%20Object%20Reference) (Token :type Actor%20Object%20Reference) (PlayerState :type Player%20State%20Object%20Reference))
  (|CallParentFunction PlayerId Action Controller Token PlayerState)
  (Variables|Default|SetInteractSpeed (Math|Float|SelectFloat (Variables|Logic-Config|GetInteractSpeedMedic) (Variables|Logic-Config|GetInteractSpeedDefault) (Logic|PawnIsMedic (Pawn|GetControlledPawn Controller)))))

(fn FindBestRespawnLocation
  (params (OriginalLocation :type Vector))
  (bind (_x _y) (Math|Vector|BreakVector OriginalLocation))
  (bind (_outhit _returnvalue) (Collision|LineTraceByChannel OriginalLocation (Math|Vector|MakeVector _x _y (Variables|/Script/Engine.WorldSettings|GetKillZ (Class|DFBlueprintFunctions|GetWorldSettings))) "TraceTypeQuery3" false 0 "None"))
  (if _returnvalue
    (bind _asdfbase_character (Utilities|Casting|CastToDFBaseCharacter (Variables|Logic|GetOwnerPawn))
      (:then
        (return (Math|Vector|MakeVector (.X (Math|Vector|BreakVector (.ImpactPoint (Collision|BreakHitResult _outhit)))) (.Y (Math|Vector|BreakVector (.ImpactPoint (Collision|BreakHitResult _outhit)))) (+ (.Z (Math|Vector|BreakVector (.ImpactPoint (Collision|BreakHitResult _outhit)))) (Components|Capsule|GetScaledCapsuleHalfHeight (Variables|/Script/Engine.Character|GetCapsuleComponent _asdfbase_character))))))
      (:CastFailed
        _)))
  (return OriginalLocation))

(fn PlayerStateIsMedic
  (params (PlayerState :type Player%20State%20Object%20Reference))
  (bind _ashdplayer_state (Utilities|Casting|CastToHDPlayerState PlayerState)
    (:then
      (Utilities|IsValid (Variables|/Script/HDMain.HDPlayerState|GetCurrentLoadout _ashdplayer_state)
        (:Is%20Valid
          (bind _array_element (Utilities|Array|ForEachLoopwithBreak (Variables|/Script/HDMain.HDKit|GetItemEntries (Variables|/Script/HDMain.HDPlayerState|GetCurrentLoadout _ashdplayer_state)))
            (:LoopBody
              (if (Utilities|Enum|Equal(Enum) (.SpecificItemType (Utilities|GetClassDefaults (.ItemClass (Utilities|Struct|BreakHDItemEntry _array_element)))) "MedicBag")
                (LocalVariables|SetbHasMedicBag true)))
            (:Completed
              (return (or (LocalVariables|GetbHasMedicBag) (Utilities|String|Contains (Utilities|String|ToString(Text) (Variables|/Script/HDMain.HDKit|GetKitDisplayName (Variables|/Script/HDMain.HDPlayerState|GetCurrentLoadout _ashdplayer_state))) "medic"))))))
        (:Is%20Not%20Valid
          (return false))))
    (:CastFailed
      (return false))))

(fn CalculateDistanceto
  (bind _iconwidget (Variables|Default|GetIconWidget))
  (bind _returnvalue (UserInterface|GetUserWidgetObject _iconwidget))
  (bind _returnvalue_2 (Class|UserWidget|GetOwningPlayerPawn _returnvalue))
  (Utilities|IsValid _iconwidget
    (:Is%20Valid
      (Utilities|IsValid _returnvalue_2
        (:Is%20Valid
          (Variables|Logic|SetDistanceTo (/ (Math|Vector|Distance2D(Vector) (Transformation|GetActorLocation) (Transformation|GetActorLocation _returnvalue_2)) (Variables|Logic-Config|GetDistanceCutOff))))))))

(fn GetAllowGiveUp
  (return (>= (Variables|Logic|GetDownedSeconds) (Math|Conversions|ToFloat(Integer) (Variables|/CasualCQB/Root/Blueprints/Components/CP_GameState_Config.CP_GameState_Config_C|GetMinGiveUpDelay (CallFunction|GetServerConfig))))))

(fn CheckforAllowGiveUp
  (if (not (Variables|Logic|GetbReviveAllowed))
    (if (Logic|GetAllowGiveUp)
      (Variables|Logic|SetbReviveAllowed true)
      (bind _asbp_hdplayer_controller_cqb (Utilities|Casting|CastToBP_HDPlayerController_CQB (Variables|Logic|GetOwnerController)))
      (Default|OnPlayerAllowGiveUpClient _asbp_hdplayer_controller_cqb))))

(fn Calculate
  (params (DeltaSeconds :type Float%20%28single-precision%29))
  (Variables|Logic|SetDownedSeconds (+ DeltaSeconds (Variables|Logic|GetDownedSeconds))))

(fn PawnIsAble
  (params (Pawn :type Pawn%20Object%20Reference))
  (Utilities|IsValid Pawn
    (:Is%20Valid
      (bind _ragdollcontrol (Class|IFCharacterCQB|GetRagDollControl(Message) Pawn))
      (Utilities|IsValid _ragdollcontrol
        (:Is%20Valid
          (return (not (Default|IsDownedorDead _ragdollcontrol))))
        (:Is%20Not%20Valid
          (return (Class|DFBlueprintFunctions|IsValidActor Pawn)))))
    (:Is%20Not%20Valid
      (return false))))

(fn GetCenterPosition
  (bind _asbp_hdplayer_character (Utilities|Casting|CastToBP_HDPlayerCharacter (Variables|Logic|GetOwnerPawn)))
  (return (Class|SkeletalMeshComponent|GetSkeletalCenterOfMass (Variables|/Script/Engine.Character|GetMesh _asbp_hdplayer_character))))

(fn MoveCharacter
  (bind _centerposition (Variables|Logic|GetCenterPosition))
  (if (not (Math|Vector|VectorIsZero _centerposition)) ; Don't use a zero vector if the variable has never been updated
    (bind _bestlocation (Logic|FindBestRespawnLocation _centerposition))
    (Transformation|SetActorLocation (Variables|Logic|GetOwnerPawn) _bestlocation false true)))