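; BP_Controller_SquadSpawner is a spawn point provider that exposes a single spawn point, apparently for squad spawning.
; Its Update event rebuilds that point from a supplied transform with a fixed ID of zero, and GetAllSpawnPointsBP returns it as the only entry.
; Restart and actor spawn checks always pass, FindSpawnPointBP reports success without looking up the ID, and collision handling is not overridden.
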(event Custom|Update
  (params (Spawn%20Transform :type Transform))
  (Variables|Logic|SetSpawnPoint (Utilities|Struct|MakeSpawnPointDef 0 Spawn%20Transform)))

(event EventBeginPlay
  (|CallParentFunction))

(event Collision|EventActorBeginOverlap
  (params (OtherActor :type Actor%20Object%20Reference)))

(event EventTick
  (params (DeltaSeconds :type Float%20%28single-precision%29)))

(fn ConstructionScript)

(fn CanRestartPlayerfromSpawnPointBP
  (params (SpawnPoint :type Spawn%20Point%20Def%20Structure%20%28by%20ref%29) (Player :type Controller%20Object%20Reference) (PlayerPawnClass :type Pawn%20Class%20Reference))
  (return true))

(fn CanSpawnActorfromSpawnPointBP
  (params (SpawnPoint :type Spawn%20Point%20Def%20Structure%20%28by%20ref%29) (SpawnActorClass :type Actor%20Class%20Reference))
  (return true))

(fn FindSpawnPointBP
  (params (SpawnPointID :type Integer))
  (return "" true))

(fn GetAllSpawnPointsBP
  (return (Utilities|Array|MakeArray (Variables|Logic|GetSpawnPoint)) 1))

(fn GetSpawnPointCollisionHandlingOverrideBP
  (params (SpawnPoint :type Spawn%20Point%20Def%20Structure%20%28by%20ref%29))
  (return "Undefined" false))