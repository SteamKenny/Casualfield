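; Blueprint function library of shared helpers for the CQB game mode code, covering typed getters for game mode, game state, controllers, HUD, configs and UI manager.
; UI helpers classify pawns as squad, team or enemy with matching colours, re-sort and shade scoreboard rows by score, and convert world positions to minimap coordinates.
; Other utilities cover camera look-at tests, actor hiding including shadows, player lookups by ID, log text and delayed-init registration.
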(fn GetHDGameModeSkirmishCQB
  (bind _asbp_hdgame_skirmish_cqb (Utilities|Casting|CastToBP_HDGame_Skirmish_CQB (Game|GetGameMode)))
  (return _asbp_hdgame_skirmish_cqb))

(fn FriendorFoe
  (params (PawnState :type Player%20State%20Object%20Reference) (Pawn :type Pawn%20Object%20Reference) (OtherPawnState :type Player%20State%20Object%20Reference) (OtherPawn :type Pawn%20Object%20Reference))
  (bind _returnvalue (Utilities|IsValid PawnState))
  (bind _returnvalue_2 (Utilities|IsValid OtherPawnState))
  (Utilities|FlowControl|Sequence
    (:then_0
      (if (and (or _returnvalue (Utilities|IsValid Pawn)) (or _returnvalue_2 (Utilities|IsValid OtherPawn)))
        (bind _ashdplayer_state (Utilities|Casting|CastToHDPlayerState (select _returnvalue_2 OtherPawnState (Variables|/Script/Engine.Pawn|GetPlayerState OtherPawn))))
        (bind _ashdplayer_state_2 (Utilities|Casting|CastToHDPlayerState (select _returnvalue PawnState (Variables|/Script/Engine.Pawn|GetPlayerState Pawn))))
        (LocalVariables|SetInSameSquad (Math|Boolean|ANDBoolean (Utilities|IsValid (.squadstate (Variables|/Script/HDMain.HDPlayerState|GetSquadInfo _ashdplayer_state_2))) (== (.squadstate (Variables|/Script/HDMain.HDPlayerState|GetSquadInfo _ashdplayer_state_2)) (.squadstate (Variables|/Script/HDMain.HDPlayerState|GetSquadInfo _ashdplayer_state))) (Utilities|IsValid (.squadstate (Variables|/Script/HDMain.HDPlayerState|GetSquadInfo _ashdplayer_state)))))
        (LocalVariables|SetInSameTeam (== (Class|DFBasePlayerState|GetTeam _ashdplayer_state_2) (Class|DFBasePlayerState|GetTeam _ashdplayer_state)))))
    (:then_1
      (return (select (LocalVariables|GetInSameSquad) "NewEnumerator0" (select (LocalVariables|GetInSameTeam) "NewEnumerator2" "NewEnumerator3"))))))

(fn PawnRelationshiptoColourLight
  (params (Relationship :type PawnRelationship%20Enum :default "NewEnumerator0"))
  (return (Utilities|Select :Index Relationship :NewEnumerator0 (Utilities|Struct|MakeSlateColor "(R=0.250000,G=1.000000,B=0.250000,A=1.000000)") :NewEnumerator2 (Utilities|Struct|MakeSlateColor "(R=0.250000,G=0.750000,B=1.000000,A=1.000000)") :NewEnumerator3 (Utilities|Struct|MakeSlateColor "(R=1.000000,G=0.250000,B=0.250000,A=1.000000)"))))

(fn PawnRelationshiptoColour
  (params (Relationship :type Byte :default 0))
  (return (Utilities|Select :Index Relationship :Option%200 (Utilities|Struct|MakeSlateColor "(R=0.000000,G=0.750000,B=0.000000,A=1.000000)") :Option%201 (Utilities|Struct|MakeSlateColor "(R=0.000000,G=0.250000,B=1.000000,A=1.000000)") :Option%202 (Utilities|Struct|MakeSlateColor "(R=0.750000,G=0.000000,B=0.000000,A=1.000000)"))))

(fn SortPlayerList
  (params (RefPlayerList :type Scroll%20Box%20Object%20Reference) (PlayerState :type Player%20State%20Object%20Reference))
  (Utilities|FlowControl|Sequence
    (:then_0
      (bind _childwidget (Utilities|ForEachChildWidget RefPlayerList)
        (:LoopBody
          (bind _aswbp_hdscoreboard_menu_player_listing_cqb (Utilities|Casting|CastToWBP_HDScoreboardMenu_PlayerListing_CQB _childwidget))
          (Utilities|Map|Add (LocalVariables|GetPlayerMapping) (- (* (Math|Conversions|ToInteger(Byte) (Utilities|String|ToString(Text) (Class|TextBlock|GetText (Variables|/Script/HDMain.HDScoreboardListingRowBase|GetScore _aswbp_hdscoreboard_menu_player_listing_cqb)))) 100) (Class|PanelWidget|GetChildIndex RefPlayerList _aswbp_hdscoreboard_menu_player_listing_cqb)) _aswbp_hdscoreboard_menu_player_listing_cqb))))
    (:then_1
      (Widget|Panel|ClearChildren RefPlayerList))
    (:then_2
      (bind _keys (Utilities|Map|Keys (LocalVariables|GetPlayerMapping)))
      (Utilities|Array|Int32Sort _keys true)
      (for (_array_element _array_index) _keys
        (Widget|Panel|AddChild RefPlayerList (.Value (Utilities|Map|Find (LocalVariables|GetPlayerMapping) _array_element)))
        (bind _result (Math|Integer|IncrementInt (|Copy _array_index))
          (:%20%20
            (Rendering|Components|TextRender|SetText (Variables|/Script/HDMain.HDScoreboardListingRowBase|GetPlayerNumber (.Value (Utilities|Map|Find (LocalVariables|GetPlayerMapping) _array_element))) (Utilities|Text|ToText(Integer) _result))
            (Scoreboard|SetRowBackgroundColour (.Value (Utilities|Map|Find (LocalVariables|GetPlayerMapping) _array_element)) _array_index PlayerState)))))))

(fn SetRowBackgroundColour
  (params (Row :type HD%20Scoreboard%20Listing%20Row%20Base%20Object%20Reference) (RowWidgetIndex :type Integer) (PlayerState :type Player%20State%20Object%20Reference))
  (bind _returnvalue (Math|Integer|%(Integer) RowWidgetIndex 2))
  (bind _oddrowentrycolor (LocalVariables|GetOddRowEntryColor))
  (bind _evenrowentrycolor (LocalVariables|GetEvenRowEntryColor))
  (bind _returnvalue_2 (== _returnvalue 0))
  (bind _returnvalue_3 (Math|Color|SelectColor _evenrowentrycolor _oddrowentrycolor _returnvalue_2))
  (bind _aswbp_hdscoreboard_menu_player_listing_cqb (Utilities|Casting|CastToWBP_HDScoreboardMenu_PlayerListing_CQB Row))
  (if (Utilities|IsValid PlayerState)
    (Class|Border|SetBrushColor (Variables|/CasualCQB/Root/UI/ScoreboardMenu/WBP_HDScoreboardMenu_PlayerListing_CQB.WBP_HDScoreboardMenu_PlayerListing_CQB_C|GetBorderList _aswbp_hdscoreboard_menu_player_listing_cqb) (Math|Color|SelectColor (LocalVariables|GetOwnerRowEntryColor) _returnvalue_3 (== (Variables|/Script/Engine.PlayerState|GetPlayerId (Variables|/Script/HDMain.HDScoreboardListingRowBase|GetPlayerState _aswbp_hdscoreboard_menu_player_listing_cqb)) (Variables|/Script/Engine.PlayerState|GetPlayerId PlayerState))))
    (else
      (Class|Border|SetBrushColor (Variables|/CasualCQB/Root/UI/ScoreboardMenu/WBP_HDScoreboardMenu_PlayerListing_CQB.WBP_HDScoreboardMenu_PlayerListing_CQB_C|GetBorderList _aswbp_hdscoreboard_menu_player_listing_cqb) _returnvalue_3))))

(fn CalcCameraLookat
  (params (LookAt :type Vector) (RotationTollerace :type Float%20%28single-precision%29) (DistanceTollerance :type Float%20%28single-precision%29))
  (bind _returnvalue (Game|GetPlayerCameraManager 0))
  (bind _returnvalue_2 (Camera|GetCameraRotation _returnvalue))
  (bind _transformcomponent (Variables|/Script/Engine.PlayerCameraManager|GetTransformComponent _returnvalue))
  (bind _returnvalue_3 (Transformation|GetWorldLocation _transformcomponent))
  (bind _returnvalue_4 (Math|Vector|GetForwardVector _returnvalue_2))
  (bind _returnvalue_5 (Math|Vector|Distance(Vector) LookAt _returnvalue_3))
  (bind _returnvalue_6 (Math|Rotator|FindLookatRotation LookAt _returnvalue_3))
  (bind _returnvalue_7 (Math|Vector|GetForwardVector _returnvalue_6))
  (bind _returnvalue_8 (Math|Vector|DotProduct _returnvalue_7 _returnvalue_4))
  (bind _returnvalue_9 (* _returnvalue_8 -1.0))
  (return (and (<= _returnvalue_5 DistanceTollerance) (or (>= _returnvalue_9 RotationTollerace) (== RotationTollerace 0.0))) _returnvalue_9 _returnvalue_5))

(fn GetHDPlayerCharacterBPCQB
  (params (PlayerIndex :type Integer))
  (bind _asbp_hdplayer_character_base (Utilities|Casting|CastToBP_HDPlayerCharacterBase (Game|GetPlayerCharacter 0 PlayerIndex))
    (:then
      (return _asbp_hdplayer_character_base))
    (:CastFailed
      (return 0))))

(fn SetBrushfromTextureHighQuality
  (params (Image :type Image%20Object%20Reference) (Texture :type Texture%202D%20Object%20Reference) (MatchSize :type Boolean))
  (Variables|/Script/Engine.Texture|SetFilter Texture "TF_Trilinear")
  (Appearance|SetBrushfromTexture Image Texture MatchSize))

(fn GetAllChildWidgets
  (params (Panel :type Panel%20Widget%20Object%20Reference) (Widgets :type Array%20of%20Widget%20Object%20References))
  (bind _childwidget (Utilities|ForEachChildWidget Panel)
    (:LoopBody
      (bind _aspanel_widget (Utilities|Casting|CastToPanelWidget _childwidget)
        (:then
          (Widget|GetAllChildWidgets _aspanel_widget Widgets))
        (:CastFailed
          (Utilities|Array|AddUnique Widgets _childwidget))))))

(fn CalculateMinimapPixelScale
  (params (Minimap :type WBP%20Deploy%20Menu%20Spawn%20Minimap%20Object%20Reference) (WorldLength :type Float%20%28single-precision%29))
  (return (Class|KismetMathLibrary|GetAbs2D (- (.WidgetLocation (Class|DFMinimap|ConvertMapLocationtoLocalWidgetLocation Minimap (.MapLocation (Class|DFMinimap|ProjectWorldLocationtoMap Minimap (Math|Vector|MakeVector WorldLength WorldLength 0.0))))) (.WidgetLocation (Class|DFMinimap|ConvertMapLocationtoLocalWidgetLocation Minimap (.MapLocation (Class|DFMinimap|ProjectWorldLocationtoMap Minimap "0, 0, 0"))))))))

(fn CalculateMinimapWidgetLocation
  (params (Minimap :type WBP%20Deploy%20Menu%20Spawn%20Minimap%20Object%20Reference) (LocationIn :type Vector))
  (bind _maplocation (Class|DFMinimap|ProjectWorldLocationtoMap Minimap LocationIn))
  (bind _currentmappos (Variables|/Script/DonkehFrameworkUI.DFMinimap|GetCurrentMapPos Minimap))
  (bind _returnvalue (- _maplocation _currentmappos))
  (bind (_widgetlocation _returnvalue_2) (Class|DFMinimap|ConvertMapLocationtoLocalWidgetLocation Minimap _returnvalue))
  (return _widgetlocation _returnvalue_2))

(fn GetClientConfig
  (bind _config_component (Class|IFGameStateCQB|GetConfig(Message) (Game|GetGameState)))
  (Utilities|IsValid _config_component
    (:Is%20Valid
      (return (Default|GetClientSettings _config_component)))
    (:Is%20Not%20Valid
      (return 0))))

(fn GetServerConfig
  (bind _config_component (Class|IFGameStateCQB|GetConfig(Message) (Game|GetGameState)))
  (return _config_component))

(fn ZoomtoFactor
  (params (Zoom :type Float%20%28single-precision%29))
  (return (/ 1.0 (- 1.0 Zoom))))

(fn SetActorVisibility
  (params (Actor :type Actor%20Object%20Reference) (Visible :type Boolean))
  (Collision|SetActorEnableCollision Actor Visible)
  (Rendering|SetActorHiddenInGame Actor (not Visible))
  (for _array_element (Actor|GetComponentsByClass Actor "/Script/Engine.MeshComponent")
    (Rendering|SetCastShadow _array_element Visible) ; Setting actor hidden does not unfortunatley hide the shadows
  ))

(fn GetClientControlledPawn
  (bind _playercontroller (Core|GetClientPlayerController))
  (Utilities|IsValid _playercontroller
    (:Is%20Valid
      (return (Pawn|GetControlledPawn _playercontroller)))))

(fn GetClientPlayerControllerCQB
  (bind _asbp_hdplayer_controller_cqb (Utilities|Casting|CastToBP_HDPlayerController_CQB (Core|GetClientPlayerController)))
  (return _asbp_hdplayer_controller_cqb))

(fn GetClientPlayerController
  (bind _returnvalue (Game|GetPlayerController 0))
  (Utilities|IsValid _returnvalue
    (:Is%20Valid
      (return _returnvalue))))

(fn SinSmoothT
  (params (Tin :type Float%20%28single-precision%29))
  (return (Math|Trig|Sin(Radians) (* (Math|Float|MultiplybyPi Tin) 0.5))))

(fn GetPlayerStatefromPlayerId
  (params (PlayerId :type Integer))
  (for _array_element (Variables|/Script/Engine.GameStateBase|GetPlayerArray (Game|GetGameState))
    (if (== (Variables|/Script/Engine.PlayerState|GetPlayerId _array_element) PlayerId)
      (return _array_element))))

(fn GetPlayerNamefromPlayerId
  (params (PlayerId :type Integer))
  (for _array_element (Variables|/Script/Engine.GameStateBase|GetPlayerArray (Game|GetGameState))
    (if (== (Variables|/Script/Engine.PlayerState|GetPlayerId _array_element) PlayerId)
      (return (PlayerState|GetPlayerName _array_element))))
  (return "Player Unknown"))

(fn GetPlayerNamefromPlayerState
  (params (PlayerState :type Player%20State%20Object%20Reference))
  (Utilities|IsValid PlayerState
    (:Is%20Valid
      (return (PlayerState|GetPlayerName PlayerState)))
    (:Is%20Not%20Valid
      (return "Player Unknown"))))

(fn AddLogText
  (params (Prefix :type String) (Text :type String) (Enabled :type Boolean))
  (if Enabled
    (bind _asbp_hdplayer_controller_cqb (Utilities|Casting|CastToBP_HDPlayerController_CQB (Game|GetPlayerController 0)))
    (Default|AddLogText _asbp_hdplayer_controller_cqb Prefix Text)))

(fn AddLogTextRaw
  (params (Text :type String) (Enabled :type Boolean))
  (if Enabled
    (bind _asbp_hdplayer_controller_cqb (Utilities|Casting|CastToBP_HDPlayerController_CQB (Game|GetPlayerController 0)))
    (Default|AddLogTextRaw _asbp_hdplayer_controller_cqb Text)))

(fn GetClassPath
  (params (Class :type Actor%20Class%20Reference))
  (return (Utilities|ToString(SoftClassReference) (Utilities|ResolveSoftReference Class))))

(fn GetActorClassPath
  (params (Actor :type Actor%20Object%20Reference))
  (return (Actor|GetClassPath (Utilities|GetClass Actor))))

(fn GetHUDCQB
  (params (PlayerIndex :type Integer))
  (bind _asbp_hdhud_cqb (Utilities|Casting|CastToBP_HDHUD_CQB (HUD|GetHUD (Game|GetPlayerController 0 PlayerIndex))))
  (return _asbp_hdhud_cqb))

(fn GetGameStateCQB
  (bind _asbp_hdgame_state_cqb (Utilities|Casting|CastToBP_HDGameState_CQB (Game|GetGameState)))
  (return _asbp_hdgame_state_cqb))

(fn RegisterforDelayedInit
  (params (Interface :type IF%20Delayed%20Init%20Interface) (Object :type Object%20Object%20Reference))
  (bind _asbp_hdgame_state_base (Utilities|Casting|CastToBP_HDGameState_Base (Game|GetGameState)))
  (Default|RegisterDelayedInit _asbp_hdgame_state_base Interface Object))

(fn ClipTexttoLength
  (params (In :type String) (NametagTextLengthMax :type Integer))
  (if (> (Utilities|String|Len In) NametagTextLengthMax)
    (return (Utilities|String|Append (Utilities|String|GetSubstring In 0 NametagTextLengthMax) "..."))
    (else
      (return In))))

(fn GetUIManager
  (bind _uimanager (Class|IFControllerCQB|GetUIManager(Message) (Game|GetPlayerController 0)))
  (Utilities|IsValid _uimanager
    (:Is%20Valid
      (return _uimanager true))
    (:Is%20Not%20Valid
      (return 0 false))))

(fn GetCaptureRadius
  (params (CapturePoint :type BP%20HD%20Capture%20Point%20Base%20Object%20Reference))
  (return (Math|Float|Max(Float) (Variables|/Script/HDMain.HDBaseCapturePoint|GetCaptureRadius CapturePoint) (Components|Sphere|GetScaledSphereRadius (Variables|/Script/HDMain.HDBaseCapturePoint|GetSphereCollision CapturePoint)))))