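; BP_PlayArea is a per-player actor that kills its owning character for staying outside the level bounds during a match.
; On authority, Initialise counts the owner's overlaps with LevelBounds-tagged actors, then updates that count from their overlap events, ignoring downed owners.
; At zero, unless the owner is a collision-less ghost, a short timer leads to suicide; re-entry clears it.
; The local client toggles the out-of-bounds display, and the actor is destroyed with its owner.
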(event Custom|EnterEvent
  (params (OverlappedActor :type Actor%20Object%20Reference) (OtherActor :type Actor%20Object%20Reference))
  (bind _result (Logic|ActorIsRelevant OtherActor))
  (if _result
    (Math|Integer|IncrementInt (Variables|Logic|GetAreaCount)
      (:%20%20
        (CallFunction|LogicUpdateServer)))))

(event Custom|Die
  (if (Default|IsMatchinProgress (CallFunction|GetGameStateCQB))
    (Logic|RequestSuicide)))

(event Custom|LeaveEvent
  (params (OverlappedActor :type Actor%20Object%20Reference) (OtherActor :type Actor%20Object%20Reference))
  (bind _result (Logic|ActorIsRelevant OtherActor))
  (if _result
    (Math|Integer|DecrementInt (Variables|Logic|GetAreaCount)
      (:%20%20
        (CallFunction|LogicUpdateServer)))))

(event Custom|LogicUpdateClient
  (params (IsOutOfBounds :type Boolean))
  (if (Logic|OwnerIsLocal)
    (Networking|CanExecuteCosmeticEvents
      (:True
        (CallFunction|ShowHide (and (Default|IsMatchinProgress (CallFunction|GetGameStateCQB)) IsOutOfBounds))))))

(event Custom|LogicUpdateServer
  (bind _result (Logic|IsOutOfBounds))
  (if _result
    (bind _returnvalue (Utilities|Time|SetTimerbyEvent (delegate Custom|Die) 5.0))
    (else
      (Utilities|Time|ClearandInvalidateTimerbyHandle _returnvalue)))
  (CallFunction|LogicUpdateClient _result))

(event Custom|OnOwnerDestroyed
  (params (DestroyedActor :type Actor%20Object%20Reference))
  (Actor|DestroyActor))

(event Custom|Initialise
  (Networking|SwitchHasAuthority
    (:Authority
      (bind _outactors (Actor|GetAllActorswithTag "LevelBounds"))
      (for _array_element _outactors
        (Utilities|FlowControl|Sequence
          (:then_0
            (for _array_element_2 (Collision|GetOverlappingActors _array_element "/HDAssets/Core/BP_HDPlayerCharacter.BP_HDPlayerCharacter_C" :!class /Script/Engine.Actor)
              (bind _result (Logic|ActorIsRelevant _array_element_2))
              (if _result
                (Math|Integer|IncrementInt (Variables|Logic|GetAreaCount)))))
          (:then_1
            (Collision|BindEventtoOnActorEndOverlap _array_element (delegate Custom|LeaveEvent))
            (Collision|BindEventtoOnActorBeginOverlap _array_element (delegate Custom|EnterEvent))))))))

(event EventBeginPlay
  (|CallParentFunction)
  (Game|BindEventtoOnDestroyed (Components|GetOwner) (delegate Custom|OnOwnerDestroyed)))

(event Collision|EventActorBeginOverlap
  (params (OtherActor :type Actor%20Object%20Reference))
  (|CallParentFunction OtherActor) ; This node is disabled and will not be called.\nDrag off pins to build functionality.
)

(fn ConstructionScript
  (|CallParentFunction))

(fn ActorIsRelevant
  (params (Actor :type Actor%20Object%20Reference))
  (return (and (== Actor (Components|GetOwner)) (not (Logic|OwnerIsDowned)))))

(fn ShowHideLogic
  ;[1 1 1] Disable Parent Logic
)

(fn RequestSuicide
  (bind _returnvalue (Components|GetOwner))
  (if (not (Class|DFBlueprintFunctions|IsPendingKillPending _returnvalue))
    (bind _ashdplayer_character (Utilities|Casting|CastToHDPlayerCharacter _returnvalue))
    (if (Class|DFBaseCharacter|IsAlive _ashdplayer_character)
      (Class|DFBaseCharacter|Suicide _ashdplayer_character))))

(fn OwnerIsLocal
  (bind _aspawn (Utilities|Casting|CastToPawn (Components|GetOwner)))
  (return (Class|DFBlueprintFunctions|IsLocallyPlayerControlled _aspawn)))

(fn OwnerIsDowned
  (bind _returnvalue (Components|GetOwner))
  (if (Class|DFBlueprintFunctions|IsValidActor _returnvalue)
    (bind _ragdollcontrol (Class|IFCharacterCQB|GetRagDollControl(Message) _returnvalue))
    (Utilities|IsValid _ragdollcontrol
      (:Is%20Valid
        (return (Variables|/CasualCQB/Root/Blueprints/Components/CP_Character_RagDollControl.CP_Character_RagDollControl_C|GetbIsDowned _ragdollcontrol)))
      (:Is%20Not%20Valid
        (return false)))))

(fn OwnerIsGhost
  (bind _asdfbase_character (Utilities|Casting|CastToDFBaseCharacter (Components|GetOwner))
    (:then
      (if (Class|DFBlueprintFunctions|IsValidActor _asdfbase_character)
        (return (Utilities|Enum|Equal(Enum) (Collision|GetCollisionEnabled (Variables|/Script/Engine.Character|GetCapsuleComponent _asdfbase_character)) "NoCollision"))
        (else
          _)))
    (:CastFailed
      _))
  (return false))

(fn IsOutOfBounds
  (return (and (< (Variables|Logic|GetAreaCount) 1) (not (Logic|OwnerIsGhost)))))