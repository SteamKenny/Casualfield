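; Death camera that takes over the player's view, hides the HUD and highlights a first target with an outline post-process.
; After a delay it blends its look-at to the second target if that is the player's pawn, allowing orbit input while alive.
; Tick follows the second target, pulling in from a far transform.
; It reclaims view from the controller and self-destructs once another view target takes over.
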(event Custom|Initialise
  (params (FirstTargetActor :type Actor%20Object%20Reference) (SecondTargetActor :type Actor%20Object%20Reference) (OwnerController :type Player%20Controller%20Object%20Reference))
  (bind _returnvalue (Math|Vector|MakeVector -3e+02 0.0 1.5e+02))
  (bind _clientsettings (CallFunction|GetClientConfig))
  (bind _fartransform (Variables|Logic|GetFarTransform))
  (bind _camera (Variables|Default|GetCamera))
  (bind _cp_basic_cosmetics (Variables|Default|GetCP_Basic_Cosmetics))
  (bind (_location _rotation) (Math|Transform|BreakTransform _fartransform))
  (Utilities|FlowControl|Sequence
    (:then_0
      (Variables|Logic|SetBaseActor SecondTargetActor)
      (bind _output_get (Variables|Logic|SetOwnerController OwnerController))
      (Input|EnableInput _output_get)
      (Game|Player|SetViewTargetwithBlend (Variables|Logic|GetOwnerController) self 0.0 "VTBlend_Linear" 1.0 true)
      (bind _asbp_hdhudbase (Utilities|Casting|CastToBP_HDHUDBase (HUD|GetHUD (Variables|Logic|GetOwnerController))))
      (Variables|/Script/Engine.HUD|SetbShowHUD _asbp_hdhudbase false)
      (Default|Initialise (Variables|Default|GetCP_Basic_Cosmetics) (Variables|Default|GetCamera) "/CasualCQB/Root/Materials/M_Outline_Only_Inst_DeathCam.M_Outline_Only_Inst_DeathCam")
      (Transformation|SetWorldLocationAndRotation (CallFunction|GetCamera) _location _rotation false false)
      (Variables|Logic|SetPullInDestination (Math|Vector|RotateVector _returnvalue _rotation))
      (Variables|Logic|SetPullInStart (Variables|/Script/Engine.SceneComponent|GetRelativeLocation (CallFunction|GetCamera)))
      (bind _output_get_2 (Variables|Logic|SetAxisRotationTargetY (.Z (Math|Vector|BreakVector _returnvalue))))
      (Variables|Logic|SetAxisRotationY _output_get_2))
    (:then_1
      (Logic|SetTargetActor FirstTargetActor true false true)
      (Variables|/CasualCQB/Root/Core/ClientSettings_CQB.ClientSettings_CQB_C|SetDisableTagOutlines _clientsettings true)
      (Utilities|FlowControl|Delay (Variables|Logic|GetTargetSwitchDelay))
      (Variables|/CasualCQB/Root/Core/ClientSettings_CQB.ClientSettings_CQB_C|SetDisableTagOutlines _clientsettings false)
      (Default|Remove _cp_basic_cosmetics _camera "/CasualCQB/Root/Materials/M_Outline_Only_Inst_DeathCam.M_Outline_Only_Inst_DeathCam")
      (if (== SecondTargetActor (Pawn|GetControlledPawn (Variables|Logic|GetOwnerController)))
        (Logic|SetTargetActor SecondTargetActor true true false)
        (Default|Initialise _cp_basic_cosmetics _camera)))))

(event EventOnEndViewTarget
  (params (PC :type Player%20Controller%20Object%20Reference))
  ;[1 1 1] Prevent view target from changing to controller on death
  (|CallParentFunction PC)
  (Utilities|Casting|CastToController (Pawn|GetViewTarget PC))
  (Game|Player|SetViewTargetwithBlend PC self 0.0 "VTBlend_Linear" 0.0 false))

(event Collision|EventActorBeginOverlap
  (params (OtherActor :type Actor%20Object%20Reference)))

(event EventBeginPlay
  (|CallParentFunction))

(event EventTick
  (params (DeltaSeconds :type Float%20%28single-precision%29))
  (Logic|CalculateVectortoActor)
  (Logic|CalculateAxisRotationZ DeltaSeconds)
  (Logic|CalculateAxisRotationY DeltaSeconds)
  (Logic|UpdatePosition DeltaSeconds)
  (Logic|UpdateCameraLookat DeltaSeconds)
  (Logic|UpdateCameraPosition DeltaSeconds)
  (Logic|CheckforExit))

(fn ConstructionScript)

(fn SetTargetActor
  (params (TargetActor :type Actor%20Object%20Reference) (TargetLerp :type Boolean) (AxisControl :type Boolean) (Highlight :type Boolean))
  (bind _returnvalue (Actor|GetComponentbyClass TargetActor "/CasualCQB/Root/Blueprints/Components/CP_Actor_Basic_Cosmetics.CP_Actor_Basic_Cosmetics_C"))
  (Utilities|FlowControl|Sequence
    (:then_0
      (Utilities|IsValid (Variables|Logic|GetBasicCosmeticsTarget)
        (:Is%20Valid
          (Default|SetHighlightState (Variables|Logic|GetBasicCosmeticsTarget) false)
          (Variables|Logic|SetBasicCosmeticsTarget 0))))
    (:then_1
      (Utilities|IsValid TargetActor
        (:Is%20Valid
          (Utilities|IsValid _returnvalue
            (:Is%20Valid
              (bind _output_get (Variables|Logic|SetBasicCosmeticsTarget _returnvalue))
              (Default|SetHighlightState _output_get Highlight))
            (:Is%20Not%20Valid
              _))
          (Variables|Logic|SetUseAxisControl AxisControl)
          (if (and TargetLerp (Class|DFBlueprintFunctions|IsValidActor (Variables|Logic|GetTargetActor)))
            (Variables|Logic|SetPreviousTargetLookAt (Variables|Logic|GetCurrentTargetLookAt))
            (Variables|Logic|SetTargetLerpT 0.0)
            (else
              (Variables|Logic|SetPreviousTargetLookAt "0, 0, 0")
              (Variables|Logic|SetTargetLerpT 1.0)))
          (Variables|Logic|SetTargetActor TargetActor))))))

(fn GetTargetLookat
  (bind (_lookat _isvalid) (Class|IFCharacterCQB|GetCameraLookat(Message) (Variables|Logic|GetTargetActor)))
  (return (Math|Vector|SelectVector _lookat (Transformation|GetActorLocation (Variables|Logic|GetTargetActor)) _isvalid)))

(fn GetBasePosition
  (Utilities|IsValid (Variables|Logic|GetBaseActor)
    (:Is%20Valid
      (bind (_lookat _isvalid) (Class|IFCharacterCQB|GetCameraLookat(Message) (Variables|Logic|GetBaseActor)))
      (bind _output_get (Variables|Logic|SetLastBasePosition (Math|Vector|SelectVector _lookat (Transformation|GetActorLocation (Variables|Logic|GetBaseActor)) _isvalid)))
      (return _output_get))
    (:Is%20Not%20Valid
      (return (Variables|Logic|GetLastBasePosition)))))

(fn CalculateVectortoActor
  (bind _baseactor (Variables|Logic|GetBaseActor))
  (Utilities|IsValid _baseactor
    (:Is%20Valid
      (Variables|Logic|SetVectorToActor (- (Transformation|GetActorLocation _baseactor) (.Location (Math|Transform|BreakTransform (Variables|Logic|GetCameraTransform))))))))

(fn CalculateAxisRotationY
  (params (DeltaSeconds :type Float%20%28single-precision%29))
  (Variables|Logic|SetAxisRotationTargetY (Math|Float|Clamp(Float) (+ (* (Input|AxisValues|GetLookUp) (Math|Float|SelectFloat -15.0 0.0 (Math|Boolean|ANDBoolean (Variables|Logic|GetUseAxisControl) (== (Variables|Logic|GetTargetLerpT) 1.0) (Logic|GetTargetIsAlive)))) (Variables|Logic|GetAxisRotationTargetY)) 1e+01 2e+02))
  (Variables|Logic|SetAxisRotationY (Math|Interpolation|FInterpTo (Variables|Logic|GetAxisRotationY) (Math|Float|Clamp(Float) (+ (* (Input|AxisValues|GetLookUp) (Math|Float|SelectFloat -15.0 0.0 (Math|Boolean|ANDBoolean (Variables|Logic|GetUseAxisControl) (== (Variables|Logic|GetTargetLerpT) 1.0) (Logic|GetTargetIsAlive)))) (Variables|Logic|GetAxisRotationTargetY)) 1e+01 2e+02) DeltaSeconds (Variables|Logic|GetAxisRotationInterpSpeed))))

(fn CalculateAxisRotationZ
  (params (DeltaSeconds :type Float%20%28single-precision%29))
  (Variables|Logic|SetAxisRotationTargetZ (+ (* (Input|AxisValues|GetTurn) (Math|Float|SelectFloat 7.5 0.0 (Math|Boolean|ANDBoolean (Variables|Logic|GetUseAxisControl) (== (Variables|Logic|GetTargetLerpT) 1.0) (Logic|GetTargetIsAlive)))) (Variables|Logic|GetAxisRotationTargetZ)))
  (Variables|Logic|SetAxisRotationZ (Math|Interpolation|FInterpTo (Variables|Logic|GetAxisRotationZ) (+ (* (Input|AxisValues|GetTurn) (Math|Float|SelectFloat 7.5 0.0 (Math|Boolean|ANDBoolean (Variables|Logic|GetUseAxisControl) (== (Variables|Logic|GetTargetLerpT) 1.0) (Logic|GetTargetIsAlive)))) (Variables|Logic|GetAxisRotationTargetZ)) DeltaSeconds (Variables|Logic|GetAxisRotationInterpSpeed))))

(fn UpdateCameraLookat
  (params (DeltaSeconds :type Float%20%28single-precision%29))
  (Utilities|IsValid (Variables|Logic|GetTargetActor)
    (:Is%20Valid
      (Transformation|SetWorldRotation (CallFunction|GetCamera) (Math|Rotator|FindLookatRotation (Transformation|GetWorldLocation (CallFunction|GetCamera)) (Math|Vector|Lerp(Vector) (Variables|Logic|GetPreviousTargetLookAt) (Logic|GetTargetLookat) (CallFunction|SinSmoothT (Variables|Logic|GetTargetLerpT)))) false false)
      (Variables|Logic|SetCurrentTargetLookAt (Math|Vector|Lerp(Vector) (Variables|Logic|GetPreviousTargetLookAt) (Logic|GetTargetLookat) (CallFunction|SinSmoothT (Variables|Logic|GetTargetLerpT))))
      (Variables|Logic|SetTargetLerpT (Math|Float|Clamp(Float) (+ (Variables|Logic|GetTargetLerpT) (* DeltaSeconds 0.5)))))))

(fn UpdatePosition
  (params (DeltaSeconds :type Float%20%28single-precision%29))
  (Transformation|SetActorLocation (Logic|GetBasePosition) false true)
  (Transformation|SetActorRotation (Math|Rotator|MakeRotator 0.0 0.0 (Variables|Logic|GetAxisRotationZ))))

(fn CheckforExit
  (if (!= (Pawn|GetViewTarget (Variables|Logic|GetOwnerController)) self)
    (Logic|SetTargetActor 0 false false false)
    (Actor|DestroyActor)))

(fn UpdateCameraPosition
  (params (DeltaSeconds :type Float%20%28single-precision%29))
  (Transformation|SetRelativeLocation (CallFunction|GetCamera) (Math|Vector|MakeVector (.X (Math|Vector|BreakVector (Math|Vector|Lerp(Vector) (Variables|Logic|GetPullInStart) (Variables|Logic|GetPullInDestination) (Variables|Logic|GetPullInLerpT)))) (.Y (Math|Vector|BreakVector (Math|Vector|Lerp(Vector) (Variables|Logic|GetPullInStart) (Variables|Logic|GetPullInDestination) (Variables|Logic|GetPullInLerpT)))) (Variables|Logic|GetAxisRotationY)) false false)
  (Variables|Logic|SetPullInLerpT (Math|Float|Clamp(Float) (+ (Variables|Logic|GetPullInLerpT) (* DeltaSeconds 0.25)))))

(fn GetTargetIsAlive
  (if (Class|DFBlueprintFunctions|IsValidActor (Variables|Logic|GetTargetActor))
    (bind _ragdollcontrol (Class|IFCharacterCQB|GetRagDollControl(Message) (Variables|Logic|GetTargetActor)))
    (Utilities|IsValid _ragdollcontrol
      (:Is%20Valid
        (return (not (Variables|/CasualCQB/Root/Blueprints/Components/CP_Character_RagDollControl.CP_Character_RagDollControl_C|GetbIsDead _ragdollcontrol))))
      (:Is%20Not%20Valid
        (return true)))
    (else
      (return false))))

(fn GetCamera
  (return (Variables|Default|GetCamera)))