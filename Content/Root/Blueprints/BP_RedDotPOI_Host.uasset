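; Host actor that spawns a red dot POI (BP_RedDotPOI) for a local player who is not on its RelatedTeam.
; On BeginPlay it compares RelatedTeam with the team of player controller 0 and, for an opposing local controller, spawns the POI at its own transform.
; The POI inherits RelatedTeam, and both actors expire after LifeSpanDuration.
; The host's lifespan is set only when that controller is valid.
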(event EventBeginPlay
  (bind _hdpc (CallFunction|GetHDPlayerControllerBP))
  (bind _lifespanduration (Variables|Logic|GetLifeSpanDuration))
  (|CallParentFunction)
  (Utilities|IsValid _hdpc
    (:Is%20Valid
      (if (and (!= (Variables|Logic|GetRelatedTeam) (Class|HDTeamState|GetTeam (Default|GetHDTeamState _hdpc))) (Pawn|IsLocalPlayerController _hdpc))
        (bind _returnvalue (Game|SpawnActorfromClass "/CasualCQB/Root/Blueprints/BP_RedDotPOI.BP_RedDotPOI_C" (Transformation|GetActorTransform) "AlwaysSpawn" 0 (Variables|Logic|GetRelatedTeam) 0))
        (Actor|SetLifeSpan _returnvalue _lifespanduration))
      (Actor|SetLifeSpan _lifespanduration))))

(event Collision|EventActorBeginOverlap
  (params (OtherActor :type Actor%20Object%20Reference)))

(event EventTick
  (params (DeltaSeconds :type Float%20%28single-precision%29)))

(fn ConstructionScript)