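; BP_CapturePoint gives a referenced capture point a replacement icon widget that tracks the owning team.
; Initialise passes the point's index, component and owner to WBP_Capture_Item, syncs the current team and hides the point's original icon.
; BeginPlay binds team changes to update the widget's OwningTeam, while the bound progress handler is still empty.
; Entry and leave events hide and show the icon.
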(event Custom|OnOwningTeamUpdate
  (params (ControlPoint :type HD%20Base%20Capture%20Point%20Object%20Reference) (PrevTeam :type EHDTeam%20Enum :default "Red") (NewTeam :type EHDTeam%20Enum :default "Red") (bCaptured :type Boolean))
  (Logic|SetOwningTeamWidget NewTeam))

(event Custom|Initialise
  (Logic|InitialiseWidget)
  (Logic|RemoveOriginalUI))

(event Custom|OnCaptureProgressUpdated
  (params (ControlPoint :type HD%20Base%20Capture%20Point%20Object%20Reference) (bContested :type Boolean) (Progress :type Integer))
  ;[1 1 1] TODO
)

(event Custom|OnCapturePointLeave
  (Rendering|SetVisibility (Variables|Default|GetIconWidget) true false))

(event Custom|OnCapturePointEntry
  (Rendering|SetVisibility (Variables|Default|GetIconWidget) false false))

(event EventBeginPlay
  (EventDispatchers|BindEventtoOnOwningTeamUpdate (Variables|Logic|GetCapturePoint) (delegate Custom|OnOwningTeamUpdate))
  (EventDispatchers|BindEventtoOnCaptureProgressUpdated (Variables|Logic|GetCapturePoint) (delegate Custom|OnCaptureProgressUpdated)))

(event Collision|EventActorBeginOverlap
  (params (OtherActor :type Actor%20Object%20Reference)))

(event EventTick
  (params (DeltaSeconds :type Float%20%28single-precision%29)))

(fn ConstructionScript)

(fn SetOwningTeamWidget
  (params (Team :type EHDTeam%20Enum :default "Red"))
  (bind _aswbp_capture_item (Utilities|Casting|CastToWBP_Capture_Item (UserInterface|GetUserWidgetObject (Variables|Default|GetIconWidget))))
  (Variables|/CasualCQB/Root/UI/HUD/WBP_Capture_Item.WBP_Capture_Item_C|SetOwningTeam _aswbp_capture_item Team))

(fn InitialiseWidget
  (bind _aswbp_capture_item (Utilities|Casting|CastToWBP_Capture_Item (UserInterface|GetUserWidgetObject (Variables|Default|GetIconWidget))))
  (Variables|/CasualCQB/Root/UI/HUD/WBP_Capture_Item.WBP_Capture_Item_C|SetCapturePointIndex _aswbp_capture_item (Variables|Logic|GetCapturePointIndex))
  (Variables|/CasualCQB/Root/UI/HUD/WBP_Capture_Item.WBP_Capture_Item_C|SetIconWidget _aswbp_capture_item (Variables|Default|GetIconWidget))
  (Variables|/CasualCQB/Root/UI/HUD/WBP_Capture_Item.WBP_Capture_Item_C|SetOwner _aswbp_capture_item (Variables|Logic|GetCapturePoint))
  (Default|Initialise _aswbp_capture_item)
  (Logic|UpdateCaptureItem))

(fn RemoveOriginalUI
  (Development|SetHiddeninGame (Variables|/HDCore/Placeables/BP_HDCapturePointBase.BP_HDCapturePointBase_C|GetIconWidget (Variables|Logic|GetCapturePoint)) true false))

(fn UpdateCaptureItem
  (bind _capturepoint (Variables|Logic|GetCapturePoint))
  (Utilities|IsValid _capturepoint
    (:Is%20Valid
      (Logic|SetOwningTeamWidget (Variables|/Script/HDMain.HDBaseCapturePoint|GetOwningTeam _capturepoint)))))