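; Base interactive device that a player holds Use on to fill a progress value, firing a progress-interacted callback on completion.
; Use takes a server lock that starts interaction, deferred until the UI widget exists if needed; releasing or cancelling unlocks and resets progress.
; Tick advances progress locally, but only the authority completes it.
; A looping server timer copies progress to a coarse value whose RepNotify resyncs clients.
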(event Custom|StartInteract
  (Variables|Logic|SetInteracting true))

(event Custom|CancelInteract
  (Variables|Logic|SetUseKeyDown false)
  (CallFunction|ServerUnlockforPlayer))

(event Custom|StopInteract
  (Variables|Logic|SetInteracting false)
  (Variables|Logic|SetInteractT 0.0))

(event Custom|OnUseReleased
  (Variables|Logic|SetUseKeyDown false)
  (CallFunction|ServerUnlockforPlayer))

(event Custom|UpdateMacro
  (Variables|Logic|SetInteractT_Macro (Variables|Logic|GetInteractT)))

(event Custom|OnDeferredUseKeyDown
  (CallFunction|UpdateCanInteract)
  (if (Variables|Default|GetCanInteract)
    (if (CallFunction|IsShowingUI)
      (CallFunction|ServerLockforPlayer "Interact")
      (else
        (Variables|Logic|SetUseKeyDown true)))))

(event Custom|OnInteracted
  (Variables|Default|SetInteracted true)
  (Default|CallOnProgressInteracted true))

(event Custom|OnUsePressed
  (CallFunction|UpdateCanInteract)
  (if (Variables|Default|GetCanInteract)
    (if (CallFunction|IsShowingUI)
      (CallFunction|ServerLockforPlayer "Interact")
      (else
        (Variables|Logic|SetUseKeyDown true)))))

(event EventBeginPlay
  (bind _self self)
  (|CallParentFunction)
  (Networking|SwitchHasAuthority
    (:Authority
      (Utilities|Time|SetTimerbyEvent (delegate Custom|UpdateMacro) 1.0 true))
    (:Remote
      _))
  (Networking|CanExecuteCosmeticEvents
    (:True
      (CallFunction|RegisterforDelayedInit _self _self)
      (Input|EnableInput (Game|GetPlayerController 0)))))

(event Collision|EventActorBeginOverlap
  (params (OtherActor :type Actor%20Object%20Reference))
  (|CallParentFunction OtherActor) ; This node is disabled and will not be called.\nDrag off pins to build functionality.
)

(event EventDelayedInit
  (Input|EnableInput (Game|GetPlayerController 0)))

(event EventTick
  (params (DeltaSeconds :type Float%20%28single-precision%29))
  (|CallParentFunction DeltaSeconds)
  (Logic|UpdateInteract DeltaSeconds))

(event Input|ActionEvents|InputActionUse
  (params (Key :type Key%20Structure :default "None"))
  (:Pressed
    (CallFunction|OnUsePressed))
  (:Released
    (CallFunction|OnUseReleased)))

(fn ConstructionScript
  (|CallParentFunction))

(fn ExecuteLockAction
  (params (Action :type String) (Controller :type Controller%20Object%20Reference) (Token :type Actor%20Object%20Reference))
  (|CallParentFunction Action Controller Token)
  (switch string Action
    (:Interact
      (CallFunction|StartInteract))))

(fn ExecuteUnlockAction
  (|CallParentFunction)
  (CallFunction|StopInteract))

(fn UpdateInteract
  (params (Delta%20Seconds :type Float%20%28single-precision%29))
  (if (Variables|Logic|GetInteracting)
    (bind _output_get (Variables|Logic|SetInteractT (+ (Variables|Logic|GetInteractT) (* Delta%20Seconds (Variables|Logic|GetInteractSpeed)))))
    (if (>= _output_get 1.0)
      (Variables|Logic|SetInteractT 1.0)
      (Networking|SwitchHasAuthority
        (:Authority
          (Variables|Logic|SetInteracting false)
          (CallFunction|OnInteracted))))
    (else
      (Variables|Logic|SetInteractT 0.0))))

(fn OnRepInteractTMacro
  (Variables|Logic|SetInteractT (Variables|Logic|GetInteractT_Macro)))

(fn OnRepInteracting)

(fn UserWidgetCreated
  (params (Widget :type Widget%20Object%20Reference))
  (|CallParentFunction Widget)
  (if (Variables|Logic|GetUseKeyDown)
    (Variables|Logic|SetUseKeyDown false)
    (CallFunction|OnDeferredUseKeyDown)))

(fn UsePressedFilter)