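; Game state Blueprint for the CQB mode that holds match rules, server identity and timed admin messages.
; On BeginPlay the authority copies its gameplay, spawn and movement settings into CPGameStateConfig, stores the command line and loads server branding from a "ServerInformation" save slot.
; CPGameStateConfig.OnReady runs on both server and clients.
; Helpers parse command-line options, shielding quoted whitespace for server options, and expose match-in-progress, config and item utility.
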(event Custom|AdminMessage
  (params (Message :type String) (Time :type Float%20%28single-precision%29))
  (Variables|Logic|SetMessageBody Message)
  (Variables|Logic|SetMessageUntilTime (+ Time (GameState|GetServerWorldTimeSeconds))))

(event EventBeginPlay
  (bind _cp_gamestate_config (Variables|Default|GetCP_GameState_Config))
  (bind _cp_gamestate_config_2 (Variables|Default|GetCP_GameState_Config))
  (|CallParentFunction)
  (Utilities|FlowControl|Sequence
    (:then_0
      (Networking|SwitchHasAuthority
        (:Authority
          (bind _returnvalue (Utilities|GetCommandLine))
          (Variables|Default|SetServerCommandLine _returnvalue))))
    (:then_1
      (Networking|SwitchHasAuthority
        (:Authority
          (Variables|/CasualCQB/Root/Blueprints/Components/CP_GameState_Config.CP_GameState_Config_C|SetEnableEnemyTags _cp_gamestate_config_2 (Variables|Default|GetbEnableEnemyTags))
          (Variables|/CasualCQB/Root/Blueprints/Components/CP_GameState_Config.CP_GameState_Config_C|SetEnableDeathCamera _cp_gamestate_config_2 (Variables|Default|GetbEnableDeathCamera))
          (Variables|/CasualCQB/Root/Blueprints/Components/CP_GameState_Config.CP_GameState_Config_C|SetEnableRedDot _cp_gamestate_config_2 (Variables|Default|GetbEnableRedDot))
          (Variables|/CasualCQB/Root/Blueprints/Components/CP_GameState_Config.CP_GameState_Config_C|SetAllowMinimap _cp_gamestate_config_2 (Variables|Default|GetbAllowMinimap))
          (Variables|/CasualCQB/Root/Blueprints/Components/CP_GameState_Config.CP_GameState_Config_C|SetEnableSuppressionEffect _cp_gamestate_config_2 (Variables|Default|GetbEnableSuppressionEffect))
          (Variables|/CasualCQB/Root/Blueprints/Components/CP_GameState_Config.CP_GameState_Config_C|SetEnableSuppressionMovement _cp_gamestate_config_2 (Variables|Default|GetbEnableSuppressionMovement))
          (Variables|/CasualCQB/Root/Blueprints/Components/CP_GameState_Config.CP_GameState_Config_C|SetAllowSquadSpawn _cp_gamestate_config_2 (Variables|Default|GetbAllowSquadSpawn))
          (Variables|/CasualCQB/Root/Blueprints/Components/CP_GameState_Config.CP_GameState_Config_C|SetAllowRevive _cp_gamestate_config_2 (Variables|Default|GetbAllowRevive))
          (Variables|/CasualCQB/Root/Blueprints/Components/CP_GameState_Config.CP_GameState_Config_C|SetEnableDevelopment _cp_gamestate_config_2 (Variables|Default|GetbEnableDevelopment))
          (Variables|/CasualCQB/Root/Blueprints/Components/CP_GameState_Config.CP_GameState_Config_C|SetbAllowKillFeed _cp_gamestate_config_2 (Variables|Default|GetbAllowKillFeed))
          (Variables|/CasualCQB/Root/Blueprints/Components/CP_GameState_Config.CP_GameState_Config_C|SetSquadSpawnAdditionalDelay _cp_gamestate_config_2 (Variables|Default|GetSquadSpawnAdditionalDelay))
          (Variables|/CasualCQB/Root/Blueprints/Components/CP_GameState_Config.CP_GameState_Config_C|SetRadialDamageMultiplier _cp_gamestate_config_2 (Variables|Default|GetRadialDamageMultipler))
          (Variables|/CasualCQB/Root/Blueprints/Components/CP_GameState_Config.CP_GameState_Config_C|SetbAllowPlayerTags _cp_gamestate_config_2 (Variables|Default|GetbAllowPlayerTags)))))
    (:then_2
      (Networking|SwitchHasAuthority
        (:Authority
          (Variables|/CasualCQB/Root/Blueprints/Components/CP_GameState_Config.CP_GameState_Config_C|SetbEnableSpawnProtection _cp_gamestate_config (Variables|Default|GetbEnableSpawnProtection))
          (Variables|/CasualCQB/Root/Blueprints/Components/CP_GameState_Config.CP_GameState_Config_C|SetMinGiveUpDelay _cp_gamestate_config (Variables|Default|GetMinGiveUpDelay))
          (Variables|/CasualCQB/Root/Blueprints/Components/CP_GameState_Config.CP_GameState_Config_C|SetMinRespawnDelay _cp_gamestate_config (Variables|Default|GetMinRespawnDelay))
          (Variables|/CasualCQB/Root/Blueprints/Components/CP_GameState_Config.CP_GameState_Config_C|SetTimeToContinue _cp_gamestate_config (Variables|Default|GetTimeToContinue))
          (Variables|/CasualCQB/Root/Blueprints/Components/CP_GameState_Config.CP_GameState_Config_C|SetPlayerSprintAcceleration _cp_gamestate_config (Variables|Default|GetPlayerSprintAcceleration))
          (Variables|/CasualCQB/Root/Blueprints/Components/CP_GameState_Config.CP_GameState_Config_C|SetPlayerSprintStrafingThreashold _cp_gamestate_config (Variables|Default|GetPlayerSprintStrafingThreashold))
          (Variables|/CasualCQB/Root/Blueprints/Components/CP_GameState_Config.CP_GameState_Config_C|SetPlayerMaxWalkSpeed _cp_gamestate_config (Variables|Default|GetPlayerMaxWalkSpeed))
          (Variables|/CasualCQB/Root/Blueprints/Components/CP_GameState_Config.CP_GameState_Config_C|SetPlayerFallDamageDivisor _cp_gamestate_config (Variables|Default|GetPlayerFallDamageDivisor))
          (Variables|/CasualCQB/Root/Blueprints/Components/CP_GameState_Config.CP_GameState_Config_C|SetbNoReviveOnHeadshot _cp_gamestate_config (Variables|Default|GetbNoReviveOnHeadshot))
          (Variables|/CasualCQB/Root/Blueprints/Components/CP_GameState_Config.CP_GameState_Config_C|SetSquadSpawnEnemyRadius _cp_gamestate_config (Variables|Default|GetSquadSpawnEnemyRadius))
          (Variables|/CasualCQB/Root/Blueprints/Components/CP_GameState_Config.CP_GameState_Config_C|SetbEnableDeathInformation _cp_gamestate_config (Variables|Default|GetbEnableDeathInformation)))))
    (:then_3
      (Default|OnReady (Variables|Default|GetCP_GameState_Config))
      (Networking|SwitchHasAuthority
        (:Authority
          (bind _returnvalue_2 (SaveGame|LoadGamefromSlot "ServerInformation"))
          (bind _asserver_information (Utilities|Casting|CastToServerInformation _returnvalue_2))
          (Variables|Default|SetServerIconURL (Variables|/CasualCQB/Root/Core/ServerInformation.ServerInformation_C|GetServerIconURL _asserver_information))
          (Variables|Default|SetServerInformation (Variables|/CasualCQB/Root/Core/ServerInformation.ServerInformation_C|GetServerInformation _asserver_information))
          (Variables|Default|SetServerName (Variables|/CasualCQB/Root/Core/ServerInformation.ServerInformation_C|GetServerName _asserver_information))
          (Variables|Default|SetServerSubTitle (Variables|/CasualCQB/Root/Core/ServerInformation.ServerInformation_C|GetServerSubTitle _asserver_information))
          (Variables|Default|SetServerFlagIconURL (Variables|/CasualCQB/Root/Core/ServerInformation.ServerInformation_C|GetServerFlagURL _asserver_information))
          (Variables|Default|SetHaveServerInformation true))))))

(fn ConstructionScript
  (|CallParentFunction))

(fn GetServerCommandLineOption
  (params (Option :type String))
  (bind _out (Logic|ParseQuotes (Variables|Default|GetServerCommandLine) "¬"))
  (bind _value (Logic|ExtractCommandLineOption Option _out))
  (return (Utilities|String|Replace _value "¬" " ")))

(fn GetCommandLineOption
  (params (Option :type String))
  (bind _returnvalue (Utilities|GetCommandLine))
  (bind _value (Logic|ExtractCommandLineOption Option _returnvalue))
  (return _value))

(fn ExtractCommandLineOption
  (params (Option :type String) (CommandLine :type String))
  (for _array_element (Utilities|String|ParseIntoArray CommandLine " ")
    (if (Utilities|String|Contains _array_element Option)
      (return (.RightS (Utilities|String|Split _array_element "="))))))

(fn IsMatchinProgress
  (return (Utilities|Name|Equal(Name) (Variables|Default|GetMatchState) (Utilities|Name|MakeLiteralName "InProgress"))))

(fn ParseQuotes
  (params (In :type String) (Replace :type String))
  (for _array_element (Utilities|String|GetCharacterArrayfromString In)
    (if (Utilities|Enum|Equal(Enum) "\"" _array_element)
      (LocalVariables|SetInSection (Class|KismetMathLibrary|XORBoolean (LocalVariables|GetInSection) true))
      (elif (and (Class|DFBlueprintFunctions|IsEmptyorWhitespace _array_element) (LocalVariables|GetInSection))
        (LocalVariables|SetPendingOut (Utilities|String|Append (LocalVariables|GetPendingOut) Replace))
        (else
          (LocalVariables|SetPendingOut (Utilities|String|Append (LocalVariables|GetPendingOut) _array_element))))))
  (return (LocalVariables|GetPendingOut)))

(fn GetConfig
  (return (Variables|Default|GetCP_GameState_Config)))

(fn GetItemUtil
  (return (Variables|Default|GetCP_GameState_ItemUtil)))