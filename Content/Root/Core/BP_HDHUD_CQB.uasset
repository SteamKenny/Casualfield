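; HUD Blueprint that detects text blocks whose fonts cannot render their text and switches them to the Roboto_CQB fallback font.
; Text blocks are queued with their owners, then measured with GetTextSize during DrawHUD, and the queue is cleared.
; A width of 2 or less is treated as unrenderable, triggering the font swap and an owner notification.
; A helper restores a given font family, and HideHUDWidget sets ShowHUD to true.
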(event EventBeginPlay
  (|CallParentFunction) ; This node is disabled and will not be called.\nDrag off pins to build functionality.
)

(event Collision|EventActorBeginOverlap
  (params (OtherActor :type Actor%20Object%20Reference))
  (|CallParentFunction OtherActor) ; This node is disabled and will not be called.\nDrag off pins to build functionality.
)

(event EventTick
  (params (DeltaSeconds :type Float%20%28single-precision%29))
  (|CallParentFunction DeltaSeconds) ; This node is disabled and will not be called.\nDrag off pins to build functionality.
)

(event EventDrawHUD
  (params (SizeX :type Integer) (SizeY :type Integer))
  (Logic|CheckTextBlocks))

(event EventHideHUDWidget
  (params (bDestroyWidgetOnHide :type Boolean))
  (Variables|Default|SetbShowHUD true))

(fn ConstructionScript
  (|CallParentFunction))

(fn AddPendingTextBlockCheck
  (params (TextBlock :type Text%20Block%20Object%20Reference) (Owner :type Widget%20Object%20Reference))
  (Utilities|Array|AddUnique (Variables|Logic|GetTextBlocks) (Utilities|Struct|MakeSTR_TextBlock TextBlock Owner)))

(fn CheckTextBlocks
  (for _array_element (Variables|Logic|GetTextBlocks)
    (if (not (Class|DFBlueprintFunctions|TextIsEmptyorWhitespace (Class|TextBlock|GetText (.TextBlock (Utilities|Struct|BreakSTR_TextBlock _array_element))))) ; Can't calculate an empty string!
      (bind _asfont (Utilities|Casting|CastToFont (.FontObject (Utilities|Struct|BreakSlateFontInfo (Variables|/Script/UMG.TextBlock|GetFont (.TextBlock (Utilities|Struct|BreakSTR_TextBlock _array_element)))))))
      (if (<= (.OutWidth (Class|HUD|GetTextSize (Utilities|String|ToString(Text) (Class|TextBlock|GetText (.TextBlock (Utilities|Struct|BreakSTR_TextBlock _array_element)))) _asfont 1.0)) 2.0)
        (Class|TextBlock|SetFont (.TextBlock (Utilities|Struct|BreakSTR_TextBlock _array_element)) (Utilities|Struct|MakeSlateFontInfo "/CasualCQB/Root/Fonts/Roboto_CQB.Roboto_CQB" (.FontMaterial (Utilities|Struct|BreakSlateFontInfo (Variables|/Script/UMG.TextBlock|GetFont (.TextBlock (Utilities|Struct|BreakSTR_TextBlock _array_element))))) (.OutlineSettings (Utilities|Struct|BreakSlateFontInfo (Variables|/Script/UMG.TextBlock|GetFont (.TextBlock (Utilities|Struct|BreakSTR_TextBlock _array_element))))) (.TypefaceFontName (Utilities|Struct|BreakSlateFontInfo (Variables|/Script/UMG.TextBlock|GetFont (.TextBlock (Utilities|Struct|BreakSTR_TextBlock _array_element))))) (.Size (Utilities|Struct|BreakSlateFontInfo (Variables|/Script/UMG.TextBlock|GetFont (.TextBlock (Utilities|Struct|BreakSTR_TextBlock _array_element)))))))
        (Class|IFTextBlock|RequiresFontFallback(Message) (.Owner (Utilities|Struct|BreakSTR_TextBlock _array_element)) (.TextBlock (Utilities|Struct|BreakSTR_TextBlock _array_element))))
      (else
        (Development|PrintString "CTB: Empty string!"))))
  (Utilities|Array|Clear (Variables|Logic|GetTextBlocks)))

(fn ResetTextBlockFont
  (params (TextBlock :type Text%20Block%20Object%20Reference) (FontFamily :type Object%20Object%20Reference))
  (bind _font (Variables|/Script/UMG.TextBlock|GetFont TextBlock))
  (bind (_fontobject _fontmaterial _outlinesettings _typefacefontname _size) (Utilities|Struct|BreakSlateFontInfo _font))
  (Class|TextBlock|SetFont TextBlock (Utilities|Struct|MakeSlateFontInfo FontFamily _fontmaterial _outlinesettings _typefacefontname _size)))