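; Base game state Blueprint that provides a registry for delayed initialisation of other objects.
; RegisterDelayedInit adds each entry uniquely and maps its index to an owner object.
; Once StartDelayedInit is called, a looping short timer repeatedly invokes DelayedInit on every entry with a still-valid owner, counting the calls.
; The timer clears itself when its repeat count runs out, so entries can be initialised more than once.
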(event Custom|StartDelayedInit
  ;[1 1 1] Delayed Execution Repeat-a-tron
  (bind _returnvalue (Utilities|Time|SetTimerbyEvent (delegate Custom|Execute) 0.2 true)))

(event Custom|ExecuteDelayedInit
  ;[1 1 1] Delayed Initialisation Registration & Execution
  (for (_array_element _array_index) (Variables|Logic|GetDelayedInit)
    (if (.ReturnValue (Utilities|Map|Find (Variables|Logic|GetDelayedInitObj) _array_index))
      (Utilities|IsValid (.Value (Utilities|Map|Find (Variables|Logic|GetDelayedInitObj) _array_index))
        (:Is%20Valid
          (Default|DelayedInit _array_element)
          (Math|Integer|IncrementInt (Variables|Logic|GetDelayedInitNumCalled)))))))

(event Custom|RegisterDelayedInit
  (params (For :type IF%20Delayed%20Init%20Interface) (Owner :type Object%20Object%20Reference))
  ;[1 1 1] Delayed Initialisation Registration & Execution
  (bind _returnvalue (Utilities|Array|AddUnique (Variables|Logic|GetDelayedInit) For))
  (Utilities|Map|Add (Variables|Logic|GetDelayedInitObj) _returnvalue Owner))

(event Custom|Execute
  ;[1 1 1] Delayed Execution Repeat-a-tron
  (CallFunction|ExecuteDelayedInit)
  (bind _result (Math|Integer|DecrementInt (Variables|Logic|GetDelayedInitRepeatCount))
    (:%20%20
      (if (<= _result 0)
        (Utilities|Time|ClearandInvalidateTimerbyHandle (stale Custom|StartDelayedInit _returnvalue))))))

(event EventBeginPlay
  (|CallParentFunction))

(event EventTick
  (params (DeltaSeconds :type Float%20%28single-precision%29))
  (|CallParentFunction DeltaSeconds) ; This node is disabled and will not be called.\nDrag off pins to build functionality.
)

(fn ConstructionScript
  (|CallParentFunction))