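; Game Blueprint for the Skirmish CQB mode, built around CP game rules, state config and tickets objects.
; On BeginPlay it runs the parent logic, copies its AutoSpawnRadius into CPGameRules, then notifies the rules that the owner has begun play.
; GetConfig, GetRules and GetTickets each return the matching CP object.
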(event EventBeginPlay
  (bind _cp_game_rules (Variables|Default|GetCP_Game_Rules))
  (|CallParentFunction)
  (Variables|/CasualCQB/Root/Blueprints/Components/CP_Game_Rules.CP_Game_Rules_C|SetAutoSpawnRadius _cp_game_rules (Variables|Logic|GetAutoSpawnRadius))
  (Default|OnOwnerBeginPlay _cp_game_rules))

(event EventTick
  (params (DeltaSeconds :type Float%20%28single-precision%29))
  (|CallParentFunction DeltaSeconds) ; This node is disabled and will not be called.\nDrag off pins to build functionality.
)

(fn ConstructionScript
  (|CallParentFunction))

(fn GetConfig
  (return (Variables|Default|GetCP_GameState_Config)))

(fn GetRules
  (return (Variables|Default|GetCP_Game_Rules)))

(fn GetTickets
  (return (Variables|Default|GetCP_Game_Tickets)))