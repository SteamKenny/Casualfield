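; Experimental player character Blueprint that strips components from character instances not locally player-controlled, apparently to cut overhead.
; Five seconds after BeginPlay, it checks local control once and destroys suppression, name text, first-person mesh, camera, lean and reference-point components.
; FreeAimSpringArm is detached rather than destroyed.
; Disconnected, never-run nodes would remove AI, inventory and movement components or show a watermark widget; Tick is disabled.
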(event Custom|StripComponents
  (Utilities|FlowControl|Delay 5.0)
  (if (not (Class|DFBlueprintFunctions|IsLocallyPlayerControlled))
    ;[1 1 1] XXX: get rid of stuff we can do without
    (Utilities|FlowControl|Sequence
      (:then_0
        (Components|DestroyComponent (Variables|Default|GetSuppression_A))
        (Components|DestroyComponent (Variables|Default|GetSuppression_B))
        (Components|DestroyComponent (Variables|Default|GetSuppression_R))
        (Components|DestroyComponent (Variables|Default|GetSuppression_L))
        (Components|DestroyComponent (Variables|Default|GetPlayerNameTextRender))
        (Components|DestroyComponent (Variables|Default|GetMesh1P))
        (Components|DestroyComponent (Variables|Default|GetCameraBoom))
        (Components|DestroyComponent (Variables|Default|GetLeanComponent))
        (Components|DestroyComponent (Variables|Default|GetRefPoint))
        (Components|DestroyComponent (Variables|Default|GetTargetCameraPoint))
        (Components|DestroyComponent (Variables|Default|GetCamera1P))
        (Components|DestroyComponent (Variables|Default|GetCamera))
        (Transformation|DetachFromComponent (Variables|Default|GetFreeAimSpringArm) "KeepRelative" "KeepRelative" "KeepRelative" true)
        (Components|DestroyComponent (Variables|Default|GetSpringArm))))))

(event EventBeginPlay
  (|CallParentFunction)
  (CallFunction|StripComponents))

(event Collision|EventActorBeginOverlap
  (params (OtherActor :type Actor%20Object%20Reference)))

(event EventTick
  (params (DeltaSeconds :type Float%20%28single-precision%29))
  (|CallParentFunction DeltaSeconds) ; This node is disabled and will not be called.\nDrag off pins to build functionality.
)

(fn ConstructionScript
  (|CallParentFunction))