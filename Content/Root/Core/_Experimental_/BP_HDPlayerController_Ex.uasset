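; Experimental player controller Blueprint that adds debug helpers for inspecting movement and killing bots.
; On BeginPlay it starts a looping one-second timer that prints the speed of player pawn 0.
; Alt+G calls OnServerKillBot, which applies a fixed 100 damage to the pawn of every BP_HDAIController, with that pawn as its own damage causer.
; An alternative path calling Die on DFBaseCharacter is left unconnected.
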(event Custom|OnServerKillBot
  (bind _outactors (Actor|GetAllActorsOfClass "/HDAssets/Core/BP_HDAIController.BP_HDAIController_C"))
  (for _array_element _outactors
    (Game|Damage|ApplyDamage (Pawn|GetControlledPawn _array_element) 1e+02 0 (Pawn|GetControlledPawn _array_element) "/CasualCQB/Root/Blueprints/BP_GenericDamageType.BP_GenericDamageType_C")))

(event Custom|CustomEvent_0
  (Development|PrintString (Utilities|String|ToString(Float) (Math|Vector|VectorLength (Transformation|GetVelocity (Game|Player|GetPlayerPawn 0))))))

(event EventBeginPlay
  (|CallParentFunction)
  (Utilities|Time|SetTimerbyEvent (delegate Custom|CustomEvent_0) 1.0 true))

(event EventTick
  (params (DeltaSeconds :type Float%20%28single-precision%29))
  (|CallParentFunction DeltaSeconds) ; This node is disabled and will not be called.\nDrag off pins to build functionality.
)

(event Input|KeyboardEvents|AltG
  (params (Key :type Key%20Structure :default "None"))
  (:Pressed
    (CallFunction|OnServerKillBot)))

(fn ConstructionScript
  (|CallParentFunction))