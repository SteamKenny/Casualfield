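; Player camera manager that blacks out the view and silences world audio until the player first spawns in.
; Its construction script calls StartCameraOverride, which sets a manual black fade and mutes the SFX and Voice sound classes through SM_Master mix overrides.
; StopCameraOverride clears the fade and restores both classes, but nothing in this Blueprint calls it.
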(event EventBeginPlay
  (|CallParentFunction))

(event Collision|EventActorBeginOverlap
  (params (OtherActor :type Actor%20Object%20Reference))
  (|CallParentFunction OtherActor) ; This node is disabled and will not be called.\nDrag off pins to build functionality.
)

(event EventTick
  (params (DeltaSeconds :type Float%20%28single-precision%29))
  (|CallParentFunction DeltaSeconds) ; This node is disabled and will not be called.\nDrag off pins to build functionality.
)

(fn ConstructionScript
  (|CallParentFunction)
  (Logic|StartCameraOverride))

(fn StopCameraOverride
  (CameraFades|StopCameraFade)
  (Audio|SetSoundMixClassOverride "/HDCore/Core/SoundMixes/SM_Master.SM_Master" "/Engine/EngineSounds/SFX.SFX" 1.0 1.0 0.0 true) ; Re-enable world SFX
  (Audio|SetSoundMixClassOverride "/HDCore/Core/SoundMixes/SM_Master.SM_Master" "/Engine/EngineSounds/Voice.Voice" 1.0 1.0 0.0 true) ; Re-enable world voice
)

(fn StartCameraOverride
  (Class|PlayerCameraManager|SetManualCameraFade :InFadeAmount 1.0)
  (Audio|SetSoundMixClassOverride "/HDCore/Core/SoundMixes/SM_Master.SM_Master" "/Engine/EngineSounds/SFX.SFX" 0.0 1.0 0.0 true) ; Disable world SFX till we spawn in for the first time
  (Audio|SetSoundMixClassOverride "/HDCore/Core/SoundMixes/SM_Master.SM_Master" "/Engine/EngineSounds/Voice.Voice" 0.0 1.0 0.0 true) ; Disable world voice til we spawn in for the first time
)