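; CQB player character that adds downed and revive states, death broadcasts and an optional death camera to the base HD character.
; Its damage component intercepts health changes, driving kill attribution, controller feedback and either death or downed with an attached resuscitator.
; Other components handle ragdoll, equipment, spawn logic and protection.
; Server config toggles suppression effects, and cosmetic components are stripped from non-local characters outside PIE.
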(event Custom|OnRequestUpdateEquipmentItems
  (CallFunction|UpdateEquipmentItems))

(event Custom|SpawnDeathCameraClient
  (params (TargetActor :type Actor%20Object%20Reference) (OwnerController :type Player%20Controller%20Object%20Reference) (CameraTransform :type Transform) (FarTransform :type Transform))
  (bind _returnvalue (Game|SpawnActorfromClass "/CasualCQB/Root/Blueprints/BP_DeathCamera.BP_DeathCamera_C" (Math|Transform|MakeTransform (Transformation|GetActorLocation)) "AlwaysSpawn" self CameraTransform FarTransform 0))
  (Default|Initialise _returnvalue TargetActor self OwnerController))

(event Custom|OnEnterDowned
  (Default|SetIsDowned (Variables|Default|GetCP_Character_RagDollControl)) ; We need to set the downed flag on the server IMMEDIATLEY\nfor logic that made test against this
  (Logic|UpdateScore (Variables|Logic|GetLastDamagePlayerState) (Variables|Default|GetPlayerState)) ; Credit +1Kill and Score to Killer
  (Logic|BroadcastPlayerDeath)
  (bind _returnvalue (Game|SpawnActorfromClass "/CasualCQB/Root/Blueprints/BP_Resuscitator.BP_Resuscitator_C" (Math|Conversions|ToTransform(Vector) (Transformation|GetActorLocation)) "Undefined" (Logic|GetReplicationOwner) self (Pawn|GetController) 0))
  (Transformation|AttachComponentToComponent _returnvalue (Variables|Character|GetMesh) "pelvis" "SnapToTarget" "SnapToTarget" "SnapToTarget" true)
  (Default|StartWait _returnvalue))

(event Custom|OnPlayerResuscitatedServer
  (Logic|ResetDamage)
  (Default|EnableDamage (Variables|Default|GetCP_Character_Damage) true))

(event Custom|OnDamage
  (params (Damage :type Float%20%28single-precision%29) (Health :type Float%20%28single-precision%29) (DamageInstigator :type Controller%20Object%20Reference) (DamageCauser :type Actor%20Object%20Reference) (HeadShot :type Boolean) (HealthZero :type Boolean) (IsDowned :type Boolean))
  (Logic|ProcessDamage DamageInstigator DamageCauser HeadShot HealthZero)
  (if HealthZero
    (if IsDowned
      (CallFunction|OnEnterDowned) ; Trigger "downed" state
      (else
        (Class|DFBaseCharacter|Die 0.0 (Utilities|Struct|MakeDamageEvent) DamageInstigator DamageCauser) ; Trigger "dead" state
      ))))

(event Custom|OnDamageBlocked
  (params (DamageInstigator :type Controller%20Object%20Reference) (DamageCauser :type Actor%20Object%20Reference))
  (Logic|ProcessDamageBlocked DamageInstigator DamageCauser))

(event Custom|OnHealthRefresh
  (bind _controller (Logic|GetMatchingController))
  (bind _health (Variables|Default|GetHealth))
  ;[1 1 1] For Player Controller
  (Utilities|IsValid _controller
    (:Is%20Valid
      (Utilities|FlowControl|Sequence
        (:then_0
          (Networking|SwitchHasAuthority
            (:Authority
              (Default|OnHealthUpdateServer _controller _health))))
        (:then_1
          (Networking|CanExecuteCosmeticEvents
            (:True
              (Default|OnHealthUpdateClient _controller _health))))))))

(event Custom|OnGameHasEnded
  (Default|EnableDamage (Variables|Default|GetCP_Character_Damage) false)
  (Variables|Logic|SetbGameHasEnded true))

(event Custom|OnCharacterDeathClient
  (params (PlayerController :type BP%20HD%20Player%20Controller%20CQB%20Object%20Reference) (InsitgatingPlayerState :type Player%20State%20Object%20Reference) (InstigatingPlayerName :type String) (InstigatingPlayerActor :type Actor%20Object%20Reference) (DamageCauserName :type String) (DamageCauserIcon :type Texture%202D%20Object%20Reference) (HeadShot :type Boolean))
  (Utilities|IsValid PlayerController
    (:Is%20Valid
      (Default|UpdateKilledbyClient PlayerController InsitgatingPlayerState InstigatingPlayerName DamageCauserName DamageCauserIcon HeadShot)
      (if (Variables|/CasualCQB/Root/Blueprints/Components/CP_GameState_Config.CP_GameState_Config_C|GetEnableDeathCamera (CallFunction|GetServerConfig))
        (CallFunction|SpawnDeathCameraClient InstigatingPlayerActor PlayerController (Transformation|GetWorldTransform (Variables|Default|GetCamera1P)) (Transformation|GetWorldTransform (Variables|Default|GetCamera))) ; XXX: probably should not do if death camera UI is not also enabled?
      ))))

(event EventOnEndViewTarget
  (params (PC :type Player%20Controller%20Object%20Reference))
  (bind _springarm (Variables|Default|GetSpringArm))
  ;[1 1 1] Prevent view target from changing to controller on death, if we are not using death-cam
  (if (not (or (Variables|/CasualCQB/Root/Blueprints/Components/CP_GameState_Config.CP_GameState_Config_C|GetEnableDeathCamera (CallFunction|GetServerConfig)) false))
    (|CallParentFunction PC)
    (Utilities|Casting|CastToController (Pawn|GetViewTarget PC))
    (Game|Player|SetViewTargetwithBlend PC self 0.0 "VTBlend_Linear" 0.0 false)
    (Variables|/Script/Engine.SpringArmComponent|SetbUsePawnControlRotation _springarm false)
    (Variables|/Script/Engine.SpringArmComponent|SetbDoCollisionTest _springarm true)
    (Variables|/Script/Engine.SpringArmComponent|SetProbeSize _springarm 1e+02) ; WARNING: HARD-CODES!
  ))

(event Collision|EventActorBeginOverlap
  (params (OtherActor :type Actor%20Object%20Reference))
  (|CallParentFunction OtherActor) ; This node is disabled and will not be called.\nDrag off pins to build functionality.
)

(event EventPossessed
  (params (NewController :type Controller%20Object%20Reference))
  (bind _controller (Logic|GetMatchingController))
  (|CallParentFunction NewController)
  (Utilities|IsValid _controller
    (:Is%20Valid
      (Default|OnReset _controller))))

(event EventBeginPlay
  (|CallParentFunction)
  (Default|Initialise (Variables|Default|GetCP_Actor_Basic_Cosmetics) (Variables|Default|GetCamera1P))
  (Logic|InitialiseSuppression)
  (Logic|UpdateSuppression)
  (Default|Initialise (Variables|Default|GetCP_Character_RagDollControl) (Variables|Character|GetMesh) (Variables|Default|GetMesh1P) (Variables|Default|GetCapsuleComponent) (Variables|Default|GetSpringArm) (Variables|Default|GetCP_Character_WC_PlayerTag))
  (Default|Initialise (Variables|Default|GetCP_Character_Damage) (Variables|Character|GetMesh))
  (EventDispatchers|BindEventtoOnDamage (Variables|Default|GetCP_Character_Damage) (delegate Custom|OnDamage))
  (EventDispatchers|BindEventtoOnDamageBlocked (Variables|Default|GetCP_Character_Damage) (delegate Custom|OnDamageBlocked))
  (EventDispatchers|BindEventtoOnHealthRefresh (Variables|Default|GetCP_Character_Damage) (delegate Custom|OnHealthRefresh))
  (Default|Initialise (Variables|Default|GetCP_Character_Movement) (Variables|Default|GetDFCharacterMovement) self)
  (CallFunction|StripComponents)
  (CallFunction|PeriodicStateCheck))

(event EventPlayHit
  (params (DamageTaken :type Float%20%28single-precision%29) (DamageEvent :type Damage%20Event%20Structure%20%28by%20ref%29) (PawnInstigator :type Pawn%20Object%20Reference) (DamageCauser :type Actor%20Object%20Reference) (bKilled :type Boolean))
  (if (> DamageTaken 0.0)
    (|CallParentFunction DamageTaken DamageEvent PawnInstigator DamageCauser bKilled)
    (Default|OnHitDamage (Variables|Default|GetCP_Character_Damage))))

(event EventOnDeath
  (params (KillingDamage :type Float%20%28single-precision%29) (DamageEvent :type Damage%20Event%20Structure%20%28by%20ref%29) (InstigatingPawn :type Pawn%20Object%20Reference) (DamageCauser :type Actor%20Object%20Reference))
  (|CallParentFunction KillingDamage DamageEvent InstigatingPawn DamageCauser)
  (if (and (not (Default|IsDownedorDead (Variables|Default|GetCP_Character_RagDollControl))) (not (Variables|Logic|GetbGameHasEnded))) ; Have we already run the broadcast for downed?
    (Logic|BroadcastPlayerDeath)))

(event EventCurrentLoadout
  (Default|OnLoadoutChanged (Variables|Default|GetCP_Character_Equipment)))

(event EventHealthChanged
  (params (NewHealthTotal :type Float%20%28single-precision%29) (PrevHealthTotal :type Float%20%28single-precision%29))
  ;[1 1 1] Take control of the health/damage systems by conditinoal blocking of the health mutation
  (if (not (Variables|Default|GetbDying)) ; Prevent health interception when character is dying
    (Default|InterceptHealthChanged (Variables|Default|GetCP_Character_Damage) NewHealthTotal PrevHealthTotal)))

(event EventOnPCFireReleased
  (Default|OnCharacterFireReleased (Variables|Default|GetCP_Character_Equipment))
  (|CallParentFunction))

(event EventOnPCFirePressed
  (Default|OnCharacterFirePressed (Variables|Default|GetCP_Character_Equipment))
  (|CallParentFunction))

(event Input|ActionEvents|InputActionReload
  (params (Key :type Key%20Structure :default "None"))
  (bind _cp_character_equipment (Variables|Default|GetCP_Character_Equipment))
  (:Pressed
    (Default|OnCharacterReloadPressed _cp_character_equipment))
  (:Released
    (Default|OnCharacterReloadReleased _cp_character_equipment)))

(event Custom|OnCheckState
  ;[1 1 1] Update Equipment Items for owning client
  (bind _result (Default|ValidateEquipment (Variables|Default|GetCP_Character_Equipment) (Variables|Default|GetCurrentLoadout) (Class|DFBaseCharacter|GetInventory)))
  (if (not _result)
    (Utilities|Time|ClearandInvalidateTimerbyHandle (stale Custom|CurrentLoadoutChangedEx _returnvalue))
    (CallFunction|CurrentLoadoutChangedEx)))

(event Custom|StripComponents
  (if (not (Class|DFBlueprintFunctions|IsPlayinEditor))
    (Utilities|IsValid (Variables|Default|GetPlayerState) :!label _label
      (:Is%20Valid
        (if (not (Class|DFBlueprintFunctions|IsLocallyPlayerControlled))
          ;[1 1 1] XXX: get rid of stuff we can do without
          (Utilities|FlowControl|Sequence
            (:then_0
              (Components|DestroyComponent (Variables|Default|GetSuppression_A))
              (Components|DestroyComponent (Variables|Default|GetSuppression_B))
              (Components|DestroyComponent (Variables|Default|GetSuppression_R))
              (Components|DestroyComponent (Variables|Default|GetSuppression_L))
              (Components|DestroyComponent (Variables|Default|GetPlayerNameTextRender))
              (Components|DestroyComponent (Variables|Default|GetCameraBoom))
              (Components|DestroyComponent (Variables|Default|GetLeanComponent))
              (Components|DestroyComponent (Variables|Default|GetRefPoint))
              (Components|DestroyComponent (Variables|Default|GetTargetCameraPoint))
              (Components|DestroyComponent (Variables|Default|GetCamera1P))
              (Components|DestroyComponent (Variables|Default|GetCamera))
              (Transformation|DetachFromComponent (Variables|Default|GetFreeAimSpringArm) "KeepRelative" "KeepRelative" "KeepRelative" true)
              (Transformation|DetachFromComponent (Variables|Default|GetSpringArm) "KeepRelative" "KeepRelative" "KeepRelative" true)
              (Transformation|DetachFromComponent (Variables|Default|GetMesh1P) "KeepRelative" "KeepRelative" "KeepRelative" true)))))
      (:Is%20Not%20Valid
        (Utilities|FlowControl|Delay 0.2)
        (goto _label)))))

(event Custom|PeriodicStateCheck)

(event Custom|CurrentLoadoutChangedEx
  ;[1 1 1] Update Equipment Items for owning client
  (Utilities|Time|ClearandInvalidateTimerbyHandle (stale _returnvalue))
  (if (Class|DFBlueprintFunctions|IsLocallyPlayerControlled)
    (Class|DFBlueprintFunctions|PrintStringtoLog "Current Loadout Changed" "VeryVerbose")
    (if (Class|DFBaseCharacter|IsAlive)
      (Class|DFBlueprintFunctions|PrintStringtoLog "IsAlive returned True, proceeding to update Equipment Items..." "VeryVerbose")
      (CallFunction|UpdateEquipmentItems)
      (bind _returnvalue (Utilities|Time|SetTimerbyEvent (delegate Custom|OnCheckState) 0.2 true 0.2))
      (else
        (Class|DFBlueprintFunctions|PrintStringtoLog "IsAlive returned False, no Equipment Items will be updated from the current loadout" "VeryVerbose")))))

(fn ConstructionScript
  (|CallParentFunction)
  (Logic|Construction))

(fn Construction
  (bind _cp_character_equipment (Variables|Default|GetCP_Character_Equipment))
  (EventDispatchers|BindEventtoOnRequestUpdateEquipmentItems _cp_character_equipment (EventDispatchers|CreateEvent :!event Custom|OnRequestUpdateEquipmentItems))
  (Variables|/CasualCQB/Root/Blueprints/Components/CP_Character_Equipment.CP_Character_Equipment_C|SetOwnerCharacter _cp_character_equipment self))

(fn GetPlayerNamefromPawn
  (params (Pawn :type Pawn%20Object%20Reference))
  (bind _playerstate (Variables|/Script/Engine.Pawn|GetPlayerState Pawn))
  (if (and (Utilities|IsValid Pawn) (Utilities|IsValid _playerstate))
    (return (PlayerState|GetPlayerName _playerstate))
    (else
      (return "?"))))

(fn GetPlayerKitNamefromPawn
  (params (Pawn :type Pawn%20Object%20Reference))
  (bind _playerstate (Variables|/Script/Engine.Pawn|GetPlayerState Pawn))
  (if (and (Utilities|IsValid Pawn) (Utilities|IsValid _playerstate))
    (bind _ashdplayer_state (Utilities|Casting|CastToHDPlayerState _playerstate))
    (return (Utilities|String|ToString(Text) (Variables|/Script/HDMain.HDKit|GetKitDisplayName (Variables|/Script/HDMain.HDPlayerState|GetSpawnLoadout _ashdplayer_state))))
    (else
      (return ""))))

(fn GetPlayerNamefromPlayerState
  (params (PlayerState :type Player%20State%20Object%20Reference))
  (if (Utilities|IsValid PlayerState)
    (return (PlayerState|GetPlayerName PlayerState))))

(fn UpdateSuppression
  (Utilities|FlowControl|Sequence
    (:then_0
      (if (Variables|/CasualCQB/Root/Blueprints/Components/CP_GameState_Config.CP_GameState_Config_C|GetEnableSuppressionEffect (CallFunction|GetServerConfig))
        (Variables|Default|SetSuppresionEffect (Variables|Logic|GetSuppressionEffectOriginal))
        (else
          (Variables|Default|SetSuppresionEffect (Utilities|Struct|MakeWeightedBlendable 0.0 "/HDCore/MaterialLibrary/ScreenEffects/MI_Suppresion_PostProcess_01.MI_Suppresion_PostProcess_01")))))
    (:then_1
      (if (Variables|/CasualCQB/Root/Blueprints/Components/CP_GameState_Config.CP_GameState_Config_C|GetEnableSuppressionMovement (CallFunction|GetServerConfig))
        (Variables|Default|SetSuppressionCameraShake (Variables|Logic|GetSuppressionCameraShakeOriginal))
        (else
          (Variables|Default|SetSuppressionCameraShake 0))))))

(fn InitialiseSuppression
  (Variables|Logic|SetSuppressionEffectOriginal (Variables|Default|GetSuppresionEffect))
  (Variables|Logic|SetSuppressionCameraShakeOriginal (Variables|Default|GetSuppressionCameraShake)))

(fn GetSpawnSave
  (bind (_transform _result) (Default|GetSpawnSave (Variables|Default|GetCP_Character_SpawnLogic) 1e+02)) ; Prefer a spawn save that isn't too close to the current Characters location
  (if _result
    (return _transform _result)
    (else
      (bind (_transform_2 _result_2) (Default|GetSpawnSave (Variables|Default|GetCP_Character_SpawnLogic) 0.0)) ; Fallback .. assuming that spawn logic will get us out of the do do
      (return _transform_2 _result_2))))

(fn UpdateScore
  (params (Killer :type Player%20State%20Object%20Reference) (Victim :type Player%20State%20Object%20Reference))
  (bind _asdfbase_player_state (Utilities|Casting|CastToDFBasePlayerState Killer))
  (bind _asdfbase_player_state_2 (Utilities|Casting|CastToDFBasePlayerState Victim))
  (Class|DFBasePlayerState|ScoreKillPlayer _asdfbase_player_state _asdfbase_player_state_2 1e+01) ; XXX: probably better to pull the points given from the ruleset
)

(fn GetReplicationOwner
  (bind _returnvalue (Pawn|GetController))
  (Utilities|Casting|CastToAIController _returnvalue
    (:then
      (bind _outactors (Actor|GetAllActorsOfClass "/Script/Engine.PlayerController"))
      (bind _result (Math|Integer|DecrementInt (Utilities|Array|Length _outactors))
        (:%20%20
          (return (Utilities|Array|Get(acopy) _outactors (Math|Random|RandomIntegerinRange 0 _result))))))
    (:CastFailed
      (return _returnvalue))))

(fn EquipSelectedItemfromInventory
  (params (bSwitchFireModeForSelected :type Boolean))
  (Default|EquipSelectedItemfromInventory (Variables|Default|GetCP_Character_Equipment) bSwitchFireModeForSelected))

(fn ResetDamage
  (Variables|Logic|SetLastDamagePlayerName "")
  (Variables|Logic|SetLastDamagePlayerState 0)
  (Variables|Logic|SetLastDamageWeaponName "")
  (Variables|Logic|SetLastDamageWeaponIcon 0)
  (Variables|Logic|SetLastDamageController 0)
  (Variables|Logic|SetLastDamageSelf false)
  (Variables|Logic|SetLastDamageHeadShot false))

(fn GetLastDamagePawn
  (bind _lastdamagecontroller (Variables|Logic|GetLastDamageController))
  (Utilities|IsValid _lastdamagecontroller
    (:Is%20Valid
      (return (Pawn|GetControlledPawn _lastdamagecontroller)))))

(fn BroadcastPlayerDeath
  (Networking|SwitchHasAuthority
    (:Authority
      (bind _outactors (Actor|GetAllActorsOfClass "/CasualCQB/Root/Core/BP_HDPlayerController_CQB.BP_HDPlayerController_CQB_C"))
      (for _array_element _outactors
        (Default|OnCharacterDeathAllServer _array_element (Variables|Logic|GetLastDamagePlayerState) (Variables|Logic|GetLastDamagePlayerName) self (CallFunction|GetPlayerNamefromPlayerState (Variables|Default|GetPlayerState)) (Variables|Logic|GetLastDamageWeaponName) (Variables|Logic|GetLastDamageHeadShot)))
      (CallFunction|OnCharacterDeathClient (Logic|GetMatchingController) (Variables|Logic|GetLastDamagePlayerState) (Variables|Logic|GetLastDamagePlayerName) (Logic|GetLastDamagePawn) (Variables|Logic|GetLastDamageWeaponName) (Variables|Logic|GetLastDamageWeaponIcon) (Variables|Logic|GetLastDamageHeadShot)))))

(fn GetMatchingController
  (bind _asbp_hdplayer_controller_cqb (Utilities|Casting|CastToBP_HDPlayerController_CQB (Pawn|GetController)))
  (return _asbp_hdplayer_controller_cqb))

(fn ProcessDamage
  (params (DamageInstigator :type Controller%20Object%20Reference) (DamageCauser :type Actor%20Object%20Reference) (HeadShot :type Boolean) (HealthZero :type Boolean))
  (bind _playerstate (Variables|/Script/Engine.Controller|GetPlayerState DamageInstigator))
  (Utilities|FlowControl|Sequence
    (:then_0
      (Utilities|IsValid DamageInstigator
        (:Is%20Valid
          (if (== (Variables|/Script/Engine.Controller|GetPlayerState DamageInstigator) (Variables|Default|GetPlayerState))
            (LocalVariables|SetMessageTarget (Logic|GetMatchingController))
            (else
              (Utilities|IsValid DamageInstigator
                (:Is%20Valid
                  (LocalVariables|SetMessageTarget DamageInstigator))))))))
    (:then_1
      (bind _asbp_hdplayer_controller_cqb (Utilities|Casting|CastToBP_HDPlayerController_CQB (LocalVariables|GetMessageTarget)))
      (Default|OnDamageCaused _asbp_hdplayer_controller_cqb))
    (:then_2
      (if HealthZero
        (Utilities|FlowControl|Sequence
          (:then_0
            (Utilities|IsValid DamageInstigator
              (:Is%20Valid
                (Variables|Logic|SetLastDamageController DamageInstigator)
                (bind _playername (Logic|GetPlayerNamefromPlayerState _playerstate))
                (Variables|Logic|SetLastDamagePlayerName _playername)
                (Variables|Logic|SetLastDamagePlayerState _playerstate))))
          (:then_1
            (Utilities|IsValid DamageCauser
              (:Is%20Valid
                (bind _itemutilcomponent (Class|IFGameStateCQB|GetItemUtil(Message) (Game|GetGameState)))
                (Utilities|IsValid _itemutilcomponent
                  (:Is%20Valid
                    (bind (_weaponname _weaponicon) (Default|GetWeaponNameandIconfromActor _itemutilcomponent DamageCauser))
                    (Variables|Logic|SetLastDamageWeaponName _weaponname)
                    (Variables|Logic|SetLastDamageWeaponIcon _weaponicon))
                  (:Is%20Not%20Valid
                    _))
                (Variables|Logic|SetLastDamageWeaponClass (Utilities|GetClass DamageCauser)))))
          (:then_2
            (Variables|Logic|SetLastDamageSelf (== (Logic|GetMatchingController) (LocalVariables|GetMessageTarget)))
            (Variables|Logic|SetLastDamageHeadShot HeadShot)))))))

(fn ProcessDamageBlocked
  (params (DamageInstigator :type Controller%20Object%20Reference) (DamageCauser :type Actor%20Object%20Reference))
  (Utilities|FlowControl|Sequence
    (:then_0
      (Utilities|IsValid DamageInstigator
        (:Is%20Valid
          (if (!= (Variables|/Script/Engine.Controller|GetPlayerState DamageInstigator) (Variables|Default|GetPlayerState))
            (LocalVariables|SetMessageTarget DamageInstigator)
            (else
              (LocalVariables|SetMessageTarget (Logic|GetMatchingController)))))))
    (:then_1
      (bind _asbp_hdplayer_controller_cqb (Utilities|Casting|CastToBP_HDPlayerController_CQB (LocalVariables|GetMessageTarget)))
      (Default|OnDamageBlocked _asbp_hdplayer_controller_cqb))))

(fn GetCameraLookat
  (return (Class|SkeletalMeshComponent|GetSkeletalCenterOfMass (Variables|Character|GetMesh)) true))

(fn GetRagDollControl
  (return (Variables|Default|GetCP_Character_RagDollControl)))

(fn GetSpawnProtection
  (return (Variables|Default|GetCP_Character_SpawnProtection)))

(fn OnApplyDamage
  (return (Default|IsinSafeZone (Variables|Default|GetCP_Character_SpawnProtection)) (Default|IsDownedorDead (Variables|Default|GetCP_Character_RagDollControl))))