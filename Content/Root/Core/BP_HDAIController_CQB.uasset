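; AI controller for CQB bots that wires GOAP and perception components into a shared utility and manages the downed, revive and respawn lifecycle.
; Downing freezes the bot and switches its voice profile; resuscitation restores both, notifies the character and leaves prone after a delay.
; Unpossessing records death time, which gates respawn by a server-configured or editor-only delay.
; Disconnected development test hooks remain in the Hacks graph.
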(event Custom|OnBotResuscitated
  (bind _character (Logic|GetMatchingCharacter))
  (bind _cp_aicontroller_util (Variables|Default|GetCP_AIController_Util))
  (Default|UnFreeze _cp_aicontroller_util)
  (Default|RevertVoiceProfile _cp_aicontroller_util)
  (Utilities|FlowControl|Sequence
    (:then_0
      (Utilities|IsValid _character
        (:Is%20Valid
          (Default|OnPlayerResuscitatedServer _character))))
    (:then_1
      (CallFunction|OnBotRevived))
    (:then_2
      (Utilities|FlowControl|Delay 5.0) ; Wait x seconds, then come out of prone
      (bind _asdfbase_character (Utilities|Casting|CastToDFBaseCharacter (Pawn|GetControlledPawn)))
      (Class|DFBaseCharacter|LeaveProne _asdfbase_character))))

(event Custom|OnBotDowned
  (bind _cp_aicontroller_util (Variables|Default|GetCP_AIController_Util))
  (Default|PlayDeathVocal _cp_aicontroller_util)
  (Default|Freeze _cp_aicontroller_util)
  (Default|UseVoiceProfile _cp_aicontroller_util))

(event Custom|OnBotAborted
  (bind _cp_aicontroller_util (Variables|Default|GetCP_AIController_Util))
  (Default|UnFreeze _cp_aicontroller_util)
  (Default|RevertVoiceProfile _cp_aicontroller_util))

(event EventBeginPlay
  (|CallParentFunction)
  (Default|Initialise (Variables|Default|GetCP_AIController_Util) (Variables|Default|GetGOAPComp) (Variables|Default|GetPerceptionComp))
  (CallFunction|OnBotInitialised))

(event EventUnPossess
  (params (UnpossessedPawn :type Pawn%20Object%20Reference))
  (|CallParentFunction UnpossessedPawn)
  (CallFunction|OnBotAborted)
  (Variables|Logic|SetLastDeathTimeSeconds (Utilities|Time|GetGameTimeinSeconds)))

(event Custom|OnBotInitialised)

(event Custom|OnBotRevived)

(fn ConstructionScript
  (|CallParentFunction))

(fn GetMatchingCharacter
  (bind _asbp_hdplayer_character_cqb (Utilities|Casting|CastToBP_HDPlayerCharacter_CQB (Pawn|GetControlledPawn)))
  (return _asbp_hdplayer_character_cqb))

(fn CanRestartPlayer
  (if (== (Variables|Logic|GetLastDeathTimeSeconds) 0.0)
    (return true)
    (else
      (return (>= (- (Utilities|Time|GetGameTimeinSeconds) (Variables|Logic|GetLastDeathTimeSeconds)) (Math|Float|SelectFloat (Variables|Logic-Config|GetEditorRespawnDelay) (Math|Conversions|ToFloat(Integer) (Variables|/CasualCQB/Root/Blueprints/Components/CP_GameState_Config.CP_GameState_Config_C|GetMinRespawnDelay (CallFunction|GetServerConfig))) (Class|DFBlueprintFunctions|IsPlayinEditor)))))))